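; BP_ArenaGuard is a trigger actor that starts the arena battle and handles the player's exit from it.
; When the player overlaps its box and IsEntering is false, it starts the Spawner, or pauses the game and shows WBP_EndArenaBattle if spawning is active.
; The widget's OnLeave stops the Spawner, then sequences Door and Marker with delays while moving the player to the spline location nearest a hardcoded exit point.
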(event OnComponentBeginOverlap(Box)
  (params (OverlappedComponent :type Primitive%20Component%20Object%20Reference) (OtherActor :type Actor%20Object%20Reference) (OtherComp :type Primitive%20Component%20Object%20Reference) (OtherBodyIndex :type Integer) (bFromSweep :type Boolean) (SweepResult :type Hit%20Result%20Structure%20%28by%20ref%29))
  (Utilities|Casting|CastToBP_PlayerCharacter OtherActor)
  (if (not (Variables|Default|GetIsEntering))
    (if (Variables|/Game/VikingMageProject/Core/Characters/NPC/WaveManagement/BP_NPC_Spawn.BP_NPC_Spawn_C|GetIsActive (Variables|Default|GetSpawner))
      (Game|SetGamePaused true)
      (bind _returnvalue (UserInterface|CreateWidget "/Game/VikingMageProject/Core/UI/WBP_EndArenaBattle.WBP_EndArenaBattle_C"))
      (EventDispatchers|AssignOnLeave _returnvalue (delegate Custom|OnLeave))
      (UserInterface|Viewport|AddtoViewport _returnvalue 0)
      (else
        (Default|ArenaStart (Variables|Default|GetSpawner))))))

(event Custom|OnLeave
  (bind _returnvalue (Game|GetPlayerCharacter 0))
  (bind _asbp_player_character (Utilities|Casting|CastToBP_PlayerCharacter _returnvalue))
  (Default|ArenaStop (Variables|Default|GetSpawner))
  (Default|OpenDoor (Variables|Default|GetDoor))
  (Utilities|FlowControl|Delay 2.0)
  (Default|MovetoLocation _asbp_player_character true (Spline|FindLocationClosesttoWorldLocation (Variables|/Game/VikingMageProject/Core/World/BP_MovementPathSpline.BP_MovementPathSpline_C|GetSpline (Variables|/Game/VikingMageProject/Core/Characters/BP_CharacterCustom.BP_CharacterCustom_C|GetMovementSpline _asbp_player_character)) (Math|Vector|MakeVector -2.58e+03 -2841.0 7e+02) "World") 2.0 false false)
  (Variables|/Game/VikingMageProject/Core/Interaction/BP_InteractionMarker.BP_InteractionMarker_C|SetIsActive (Variables|Default|GetMarker) false)
  (Utilities|FlowControl|Delay 1.0)
  (Default|CloseDoor (Variables|Default|GetDoor))
  (Utilities|FlowControl|Delay 1.5)
  (Variables|/Game/VikingMageProject/Core/Interaction/BP_InteractionMarker.BP_InteractionMarker_C|SetIsActive (Variables|Default|GetMarker) true))

(event EventBeginPlay)

(event Collision|EventActorBeginOverlap
  (params (OtherActor :type Actor%20Object%20Reference)))

(event EventTick
  (params (DeltaSeconds :type Float%20%28single-precision%29)))

(fn ConstructionScript)