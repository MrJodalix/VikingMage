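; BP_TorchFire is a placeable torch fire whose point light flickers at runtime.
; Each tick it picks a random intensity within a maximum step of the last value, bounded by configurable minimum and maximum, giving a random-walk flicker.
; The construction script positions the light at a configurable relative offset.
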(event EventBeginPlay)

(event EventTick
  (params (DeltaSeconds :type Float%20%28single-precision%29))
  (bind _output_get (Variables|Default|SetLastIntensity (Math|Random|RandomFloatinRange (Math|Float|Max(Float) (Variables|Default|GetMinIntesity) (- (Variables|Default|GetLastIntensity) (Variables|Default|GetMaxChangePerTick))) (Math|Float|Min(Float) (Variables|Default|GetMaxIntesity) (+ (Variables|Default|GetLastIntensity) (Variables|Default|GetMaxChangePerTick))))))
  (Rendering|Components|Light|SetIntensity (Variables|Default|GetPointLight) _output_get))

(event Collision|EventActorBeginOverlap
  (params (OtherActor :type Actor%20Object%20Reference)))

(fn ConstructionScript
  (Transformation|SetRelativeLocation (Variables|Default|GetPointLight) (Variables|Default|GetLightOffset) false false))