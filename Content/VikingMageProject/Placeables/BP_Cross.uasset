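; BP_Cross is an interactable cross placeable that toggles between active and inactive, sliding down when activated and back up when deactivated.
; Interact flips the state and runs a timeline that nudges the cross vertically by a fixed step per update, so travel distance depends on frame rate.
; Further interaction is blocked until the timeline finishes.
; ResetToDefault restores the location saved at BeginPlay and clears the active state.
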(event Collision|EventActorBeginOverlap
  (params (OtherActor :type Actor%20Object%20Reference)))

(event EventTick
  (params (DeltaSeconds :type Float%20%28single-precision%29)))

(event EventInteract
  (bind _cross (Variables|Default|GetCross))
  (if (Variables|Default|GetInteractable)
    (bind _output_get (Variables|Default|SetIsActiveCross (not (Variables|Default|GetIsActiveCross))))
    (if _output_get
      (Variables|Default|SetFactor -1.0)
      (else
        (Variables|Default|SetFactor 1.0)))
    (Variables|Default|SetInteractable false)
    (Timeline|Animation PlayFromStart
      (:Update
        (Transformation|SetWorldLocation _cross (+ (Transformation|GetWorldLocation _cross) (Math|Vector|MakeVector 0.0 0.0 (* (Variables|Default|GetFactor) 0.4))) false false))
      (:Finished
        (Variables|Default|SetInteractable true)))))

(event EventBeginPlay
  (Variables|Default|SetSafeLocation (Transformation|GetWorldLocation (Variables|Default|GetCross))))

(fn ConstructionScript)

(fn ResettoDefault
  (Variables|Default|SetIsActiveCross false)
  (Transformation|SetWorldLocation (Variables|Default|GetCross) (Variables|Default|GetSafeLocation) false false)
  (Variables|Default|SetFactor -1.0)
  (Variables|Default|SetInteractable true))