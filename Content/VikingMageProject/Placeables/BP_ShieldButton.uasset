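; BP_ShieldButton is an interactable puzzle button that opens a giant door when its linked props are correctly set.
; Interact checks that Cross and Chalice are interactable, then requires Torch and Chalice active with Cross inactive.
; Success shakes the camera and slides the door backward; failure damages the player and resets all three props.
; ResetToDefault restores the door's starting position but leaves DoorOpened set, as that clearing node is unconnected.
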(event Collision|EventActorBeginOverlap
  (params (OtherActor :type Actor%20Object%20Reference)))

(event EventTick
  (params (DeltaSeconds :type Float%20%28single-precision%29)))

(event EventInteract
  (bind _giantdoor (Variables|Default|GetGiantDoor))
  (bind _rootcomponent (Variables|/Script/Engine.Actor|GetRootComponent _giantdoor))
  (bind _returnvalue (Transformation|GetWorldLocation _rootcomponent))
  (if (not (Variables|Default|GetDoorOpened))
    (if (and (Variables|/Game/VikingMageProject/Placeables/BP_Cross.BP_Cross_C|GetInteractable (Variables|Default|GetCross)) (Variables|/Game/VikingMageProject/Placeables/BP_ChaliceAndSkull.BP_ChaliceAndSkull_C|GetInteractable (Variables|Default|GetChalice)))
      (bind _output_get (Variables|Default|SetOpenTheDoor (Math|Boolean|ANDBoolean (not (Variables|/Game/VikingMageProject/Placeables/BP_Cross.BP_Cross_C|GetIsActiveCross (Variables|Default|GetCross))) (Variables|/Game/VikingMageProject/Placeables/BP_Torch.BP_Torch_C|GetIsActiveTorch (Variables|Default|GetTorch)) (Variables|/Game/VikingMageProject/Placeables/BP_ChaliceAndSkull.BP_ChaliceAndSkull_C|GetIsActiveChalice (Variables|Default|GetChalice)))))
      (if _output_get
        (Variables|Default|SetDoorOpened true)
        (Camera|PlayWorldCameraShake "/Game/VikingMageProject/Cinematics/BP_DoorShake.BP_DoorShake_C" _returnvalue 0.0 1e+03 0.8)
        (Components|MoveComponentTo _rootcomponent (+ _returnvalue (* (* (Math|Vector|GetForwardVector _rootcomponent) -1.0) (Variables|Default|GetLength))) "0, 0, 0" true true 5.0 false)
        (else
          (Game|Damage|ApplyDamage (Game|GetPlayerCharacter 0) (Variables|Default|GetTrapDamage) 0 0)
          (Utilities|FlowControl|Sequence
            (:then_0
              (Default|ResettoDefault (Variables|Default|GetCross)))
            (:then_1
              (Default|ResettoDefault (Variables|Default|GetTorch)))
            (:then_2
              (Default|ResettoDefault (Variables|Default|GetChalice)))))))))

(event EventBeginPlay
  (Variables|Default|SetSafeLocation (Transformation|GetWorldLocation (Variables|/Script/Engine.Actor|GetRootComponent (Variables|Default|GetGiantDoor)))))

(fn ConstructionScript)

(fn ResettoDefault
  (Variables|Default|SetOpenTheDoor false)
  (Transformation|SetWorldLocation (Variables|/Script/Engine.Actor|GetRootComponent (Variables|Default|GetGiantDoor)) (Variables|Default|GetSafeLocation) false false))