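; BP_DownslideDoor is a placeable, interactable door that slides its Hitbox component to a final offset once activated.
; Interact sets an active flag and reports success.
; Tick then moves the Hitbox at constant speed with VInterpToConstant, teleporting without sweep, until the offset matches the target and a done flag stops updates.
; The file has no logic to reverse or reset the slide.
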(event EventTick
  (params (DeltaSeconds :type Float%20%28single-precision%29))
  (if (and (Variables|Default|GetIsActive) (not (Variables|Default|GetIsDone)))
    (Transformation|SetRelativeLocation (Variables|Default|GetHitbox) (Math|Interpolation|VInterptoConstant (Variables|Default|GetCurrentOffset) (Variables|Default|GetFinalOffset) DeltaSeconds (Variables|Default|GetSpeed)) false true)
    (Variables|Default|SetCurrentOffset (Math|Interpolation|VInterptoConstant (Variables|Default|GetCurrentOffset) (Variables|Default|GetFinalOffset) DeltaSeconds (Variables|Default|GetSpeed)))
    (Variables|Default|SetIsDone (Math|Vector|Equal(Vector) (Variables|Default|GetCurrentOffset) (Variables|Default|GetFinalOffset) 0.0001))))

(fn ConstructionScript)

(fn Interact
  (params (Interactor :type BP%20Player%20Character%20Object%20Reference))
  (Variables|Default|SetIsActive true)
  (return true))