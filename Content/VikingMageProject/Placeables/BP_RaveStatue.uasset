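; BP_RaveStatue is a placeable statue that reveals a collectible fire rune and activates a linked interactor, logged as a door, once the rune is collected.
; Finishing the assigned PuzzleObject, or interacting with the statue, triggers activation.
; Activation progress drives two lerps, moving the top cylinder and rune basket in staggered phases that overlap around BorderValue.
; The child-actor BP_Item's collected event calls Interact on SolvedInteractor.
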(event Custom|OnFinishedPuzzle
  (CallFunction|ActivationTriggered))

(event Custom|CollectedFireRune
  (Default|Interact (Variables|Default|GetSolvedInteractor))
  (Development|PrintString "Activated Door!" true true "(R=1.000000,G=0.000000,B=0.000000,A=1.000000)" 5e+01))

(event Collision|EventActorBeginOverlap
  (params (OtherActor :type Actor%20Object%20Reference)))

(event EventTick
  (params (DeltaSeconds :type Float%20%28single-precision%29)))

(event EventBeginPlay
  (EventDispatchers|AssignOnFinishedPuzzle (Variables|Default|GetPuzzleObject) (delegate Custom|OnFinishedPuzzle))
  (Variables|Default|SetActive false)
  (bind _asbp_item (Utilities|Casting|CastToBP_Item (Variables|/Script/Engine.ChildActorComponent|GetChildActor (Variables|Custom|GetChildActor))))
  (EventDispatchers|BindEventtoCollected _asbp_item (delegate Custom|CollectedFireRune)))

(event EventVisualizeTriggeredProgress
  (params (Progress :type Float%20%28single-precision%29))
  (bind _bordervalue (Variables|Default|GetBorderValue))
  (bind _bordervalueoverlap (Variables|Default|GetBorderValueOverlap))
  (Utilities|FlowControl|Sequence
    (:then_0
      (Transformation|SetRelativeLocation (Variables|Default|GetTopCylinder) (Math|Vector|Lerp(Vector) (Variables|Default|GetTopCylinderStart) (Variables|Default|GetTopCylinderEnd) (Math|Float|MapRangeClamped Progress 0.0 (+ _bordervalue _bordervalueoverlap) 0.0 1.0)) false false))
    (:then_1
      (Transformation|SetRelativeLocation (Variables|Default|GetRuneBasket) (Math|Vector|Lerp(Vector) (Variables|Default|GetBasketStart) (Variables|Default|GetBasketEnd) (Math|Float|MapRangeClamped Progress (- _bordervalue _bordervalueoverlap) 1.0 0.0 1.0)) false false))))

(fn ConstructionScript)

(fn Interact
  (params (Interactor :type BP%20Player%20Character%20Object%20Reference))
  (CallFunction|ActivationTriggered)
  (return false))