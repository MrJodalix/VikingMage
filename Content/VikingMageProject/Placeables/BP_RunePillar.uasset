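; Rune pillar puzzle placeable that rewards the player with an inventory item when interacted with after its dependencies complete.
; Full dependency progress from the parent class activates the interaction marker; triggered progress then lerps the pillar between active and finished positions.
; Interacting destroys the marker, hides the rune, adds the item and fires activation.
; Becoming active switches off the DisableOnSolved entries; success sound and spell granting remain TODOs.
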(event Custom|OnActivityChangedEvent
  (Development|PrintString "Changed Activity")
  (if (Variables|Default|GetActive)
    (for _array_element (Variables|Default|GetDisableOnSolved)
      (Variables|/Game/VikingMageProject/Core/Interaction/BP_InteractionMarker.BP_InteractionMarker_C|SetIsActive _array_element false))))

(event EventBeginPlay
  (|CallParentFunction)
  (Variables|/Game/VikingMageProject/Core/Interaction/BP_InteractionMarker.BP_InteractionMarker_C|SetIsActive (Variables|Default|GetInteractionMarker) false)
  (EventDispatchers|BindEventtoActivityChanged (delegate Custom|OnActivityChangedEvent)))

(event Collision|EventActorBeginOverlap
  (params (OtherActor :type Actor%20Object%20Reference))
  (|CallParentFunction OtherActor) ; This node is disabled and will not be called.\nDrag off pins to build functionality.
)

(event EventTick
  (params (DeltaSeconds :type Float%20%28single-precision%29))
  (|CallParentFunction DeltaSeconds) ; This node is disabled and will not be called.\nDrag off pins to build functionality.
)

(event EventVisualizeDependenciesProgress
  (params (Progress :type Float%20%28single-precision%29))
  (bind _returnvalue (== Progress 1.0))
  (bind _interactionmarker (Variables|Default|GetInteractionMarker))
  (|CallParentFunction Progress)
  (Utilities|IsValid _interactionmarker
    (:Is%20Valid
      (Variables|/Game/VikingMageProject/Core/Interaction/BP_InteractionMarker.BP_InteractionMarker_C|SetIsActive _interactionmarker _returnvalue)
      (bind _output_get (Variables|Default|SetPuzzleDone _returnvalue))
      (if _output_get
        _))))

(event EventVisualizeTriggeredProgress
  (params (Progress :type Float%20%28single-precision%29))
  (if (Variables|Default|GetPuzzleDone)
    (Transformation|SetWorldLocation (Variables|Default|GetDefaultSceneRoot) (Math|Vector|Lerp(Vector) (Variables|Default|GetActivePosition) (Variables|Default|GetFinishedPosition) Progress) false false)))

(fn ConstructionScript
  (|CallParentFunction))

(fn Interact
  (params (Interactor :type BP%20Player%20Character%20Object%20Reference))
  (Actor|DestroyActor (Variables|Default|GetInteractionMarker))
  (Rendering|SetVisibility (Variables|Default|GetRune) false false)
  ;[1 1 1] TODO: Add Spell to Character
  (Default|AddItemsfromInventory (Variables|/Game/VikingMageProject/Core/Characters/Player/BP_PlayerCharacter.BP_PlayerCharacter_C|GetInventory%20%28InventoryComponent%29 (.AsBP%20Player%20Character (Utilities|Casting|CastToBP_PlayerCharacter (Game|GetPlayerCharacter 0)))) 4 1)
  (CallFunction|ActivationTriggered)
  (return true))