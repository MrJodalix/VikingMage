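; Interactable chalice placeable that toggles an active state and slides a linked Skull actor back and forth along world X.
; Each accepted interaction flips the direction and plays a timeline, locking further input until it finishes.
; The timeline adds a fixed offset every update, so travel distance depends on update count.
; ResetToDefault returns the skull to its location cached at BeginPlay and restores the inactive, interactable state.
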(event Collision|EventActorBeginOverlap
  (params (OtherActor :type Actor%20Object%20Reference)))

(event EventTick
  (params (DeltaSeconds :type Float%20%28single-precision%29)))

(event EventBeginPlay
  (Variables|Default|SetSafeLocation (Transformation|GetWorldLocation (Variables|/Script/Engine.Actor|GetRootComponent (Variables|Default|GetSkull)))))

(event EventInteract
  (if (Variables|Default|GetInteractable)
    (bind _output_get (Variables|Default|SetIsActiveChalice (not (Variables|Default|GetIsActiveChalice))))
    (if _output_get
      (Variables|Default|SetFactor -1.0)
      (else
        (Variables|Default|SetFactor 1.0)))
    (Variables|Default|SetInteractable false)
    (Timeline|Timeline_0 PlayFromStart
      (:Update
        (Transformation|SetWorldLocation (Variables|/Script/Engine.Actor|GetRootComponent (Variables|Default|GetSkull)) (+ (Transformation|GetWorldLocation (Variables|/Script/Engine.Actor|GetRootComponent (Variables|Default|GetSkull))) (Math|Vector|MakeVector (* (Variables|Default|GetFactor) 4.0) 0.0 0.0)) false false))
      (:Finished
        (Variables|Default|SetInteractable true)))))

(fn ConstructionScript)

(fn ResettoDefault
  (Variables|Default|SetIsActiveChalice false)
  (Transformation|SetWorldLocation (Variables|/Script/Engine.Actor|GetRootComponent (Variables|Default|GetSkull)) (Variables|Default|GetSafeLocation) false false)
  (Variables|Default|SetFactor -1.0)
  (Variables|Default|SetInteractable true))