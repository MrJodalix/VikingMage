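; BP_RollingStone is a physics-driven rolling stone hazard that deals massive damage to the player character on hit.
; Hit events latch a contact flag for each of two stopping meshes, or apply damage to BP_PlayerCharacter while damage is enabled.
; Tick waits until both contacts are set and the stone's speed falls to the minimum, then turns off physics simulation and damage.
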(event EventBeginPlay)

(event Collision|EventActorBeginOverlap
  (params (OtherActor :type Actor%20Object%20Reference)))

(event EventTick
  (params (DeltaSeconds :type Float%20%28single-precision%29))
  (if (Math|Boolean|ANDBoolean (Variables|Default|GetContactMesh2) (Variables|Default|GetContactMesh1) (<= (Math|Vector|VectorLength (Transformation|GetComponentVelocity (Variables|Default|GetStone))) (Variables|Default|GetMinVelocity)))
    (Physics|SetSimulatePhysics (Variables|Default|GetStone) false)
    (Variables|Default|SetDealingDamage false)))

(event Collision|EventHit
  (params (MyComp :type Primitive%20Component%20Object%20Reference) (Other :type Actor%20Object%20Reference) (OtherComp :type Primitive%20Component%20Object%20Reference) (bSelfMoved :type Boolean) (HitLocation :type Vector :default "0, 0, 0") (HitNormal :type Vector :default "0, 0, 0") (NormalImpulse :type Vector :default "0, 0, 0") (Hit :type Hit%20Result%20Structure%20%28by%20ref%29))
  (if (== Other (Variables|Default|GetStoppingMesh1))
    (Variables|Default|SetContactMesh1 true)
    (elif (== Other (Variables|Default|GetStoppingMesh2))
      (Variables|Default|SetContactMesh2 true)
      (elif (Variables|Default|GetDealingDamage)
        (bind _asbp_player_character (Utilities|Casting|CastToBP_PlayerCharacter Other))
        (Game|Damage|ApplyDamage _asbp_player_character 1e+04 0 0)))))

(fn ConstructionScript)