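; Axe-wielding melee enemy NPC that attacks standing or running, depending on its velocity.
; Weapon overlaps during a swing damage characters of another faction once, then spawn a hit sound and blood splash at a sphere-traced point.
; Tick caches the weapon's last position, so the splash direction opposes its motion.
; Equipping sets the axe mesh and collision; death disables collision and drops the axe as a physics-simulated mesh actor.
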(event OnComponentBeginOverlap(Weapon)
  (params (OverlappedComponent :type Primitive%20Component%20Object%20Reference) (OtherActor :type Actor%20Object%20Reference) (OtherComp :type Primitive%20Component%20Object%20Reference) (OtherBodyIndex :type Integer) (bFromSweep :type Boolean) (SweepResult :type Hit%20Result%20Structure%20%28by%20ref%29))
  (bind _mesh (Variables|Character|GetMesh))
  (bind _weapon (Variables|Default|GetWeapon))
  (bind _returnvalue (Transformation|GetAttachSocketName _weapon))
  (bind _returnvalue_2 (Transformation|GetSocketTransform _mesh _returnvalue "RTS_World"))
  ;[1 1 1] Nur Schaden an anderen Charakteren einer anderen Fraktion
  (bind _asbp_character_custom (Utilities|Casting|CastToBP_CharacterCustom OtherActor))
  (if (and (Utilities|Enum|NotEqual(Enum) (Variables|/Game/VikingMageProject/Core/Characters/BP_CharacterCustom.BP_CharacterCustom_C|GetFaction _asbp_character_custom) (Variables|Default|GetFaction)) (Variables|Default|GetIsWeaponSwing))
    (Game|Damage|ApplyDamage OtherActor (Variables|/Game/VikingMageProject/Core/Characters/NPC/BP_NPCStats.BP_NPCStats_C|GetBaseDamage (Variables|Default|GetBP_NPCStats)) (Pawn|GetController) 0)
    (Variables|Default|SetIsWeaponSwing false)
    (Variables|Default|SetSplatterLocation (.location _returnvalue_2))
    (bind (_outhit _returnvalue_3) (Collision|SphereTraceByChannel (.location _returnvalue_2) (+ (.location _returnvalue_2) (* (Math|Vector|GetForwardVector (.rotation _returnvalue_2)) 5e+01)) (Variables|Default|GetSplatterTraceRadius) "TraceTypeQuery8" true 0 "None"))
    (if _returnvalue_3
      (Variables|Default|SetSplatterLocation (.location _outhit)))
    (bind _returnvalue_4 (Game|SpawnActorfromClass "/Game/VikingMageProject/VFX/Blood/BP_BloodSplashParticles.BP_BloodSplashParticles_C" (Math|Transform|MakeTransform (Variables|Default|GetSplatterLocation) "0, 0, 0" "1,1,1") "AlwaysSpawn" 0 0))
    (Default|InitSplash _returnvalue_4 (* (Math|Vector|Normalize (- (Transformation|GetWorldLocation (Variables|Default|GetWeapon)) (Variables|Default|GetLastWeaponPosition))) -1.0) 5e+02 3.5e+02 2e+01)
    (Default|Splash _returnvalue_4)
    (Audio|PlaySoundatLocation "/Game/VikingMageProject/Audio/Sounds/OneShots/MeleeWeapons/A_BloodyHit_Cue.A_BloodyHit_Cue" (Variables|Default|GetSplatterLocation) "0, 0, 0" 1.0 1.0 0.0 0 0 0)))

(event OnDeath(BP_NPCStats)
  (Collision|SetCollisionEnabled (Variables|Default|GetWeapon) "NoCollision")
  (CallFunction|DropRightHand))

(event EventTick
  (params (DeltaSeconds :type Float%20%28single-precision%29))
  (|CallParentFunction DeltaSeconds)
  (Variables|Default|SetLastWeaponPosition (Transformation|GetWorldLocation (Variables|Default|GetWeapon))))

(fn ConstructionScript
  (|CallParentFunction))

(fn PrimaryAttack
  (|CallParentFunction)
  (if (<= (Math|Vector|VectorLength (Variables|/Script/Engine.MovementComponent|GetVelocity (Variables|Character|GetCharacterMovement))) 0.2)
    ;[1 1 1] TODO: Prüfung, ob wir überhaupt angreifen können
    (Variables|Default|SetIsAttack true)
    (Development|PrintString "Standing Attack!")
    (else
      (Variables|Default|SetIsRunAttack true)
      (Development|PrintString "Running Attack"))))

(fn EquipRightHand
  (bind _weapon (Variables|Default|GetWeapon))
  (|CallParentFunction)
  (Components|StaticMesh|SetStaticMesh _weapon (Variables|Default|GetRightHandEquipmentMesh))
  (Collision|SetCollisionEnabled _weapon "QueryAndPhysics")
  (Development|PrintString "EquippedAxe"))

(fn DropRightHand
  (bind _weapon (Variables|Default|GetWeapon))
  (bind _returnvalue (Game|SpawnActorfromClass "/Script/Engine.StaticMeshActor" (Math|Transform|MakeTransform (Transformation|GetWorldLocation _weapon) (Transformation|GetWorldRotation _weapon) "1,1,1") "Undefined" 0 0))
  (Transformation|SetMobility _returnvalue "Movable")
  (Components|StaticMesh|SetStaticMesh (Variables|/Script/Engine.StaticMeshActor|GetStaticMeshComponent _returnvalue) (Variables|Default|GetRightHandEquipmentMesh))
  (Physics|SetSimulatePhysics (Variables|/Script/Engine.StaticMeshActor|GetStaticMeshComponent _returnvalue) true)
  (Development|PrintString "Dropped Weapon" true true "(R=0.000000,G=0.034078,B=1.000000,A=1.000000)" 2e+01)
  (Components|StaticMesh|SetStaticMesh (Variables|Default|GetWeapon) 0))