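; Axe thug enemy NPC Blueprint that adds a gathering state on top of its parent NPC behavior.
; On BeginPlay it writes the inverse of IsGathering to the AI controller's IsNotGathering blackboard key, if a controller is valid.
; Its StartFocusActor override runs the parent logic, then clears IsGathering without rewriting the blackboard key here.
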(event EventBeginPlay
  (bind _self self)
  (bind _returnvalue (AI|GetAIController _self))
  (|CallParentFunction)
  (Utilities|IsValid _returnvalue
    (:Is%20Valid
      (AI|Components|Blackboard|SetValueasBool (Variables|/Script/AIModule.AIController|GetBlackboard _returnvalue) (Utilities|Name|MakeLiteralName "IsNotGathering") (not (Variables|Custom|AttackTrigger|GetIsGathering))))))

(fn ConstructionScript
  (|CallParentFunction))

(fn StartFocusActor
  (params (Character :type BP%20Character%20Custom%20Object%20Reference))
  (|CallParentFunction Character)
  (Variables|Custom|AttackTrigger|SetIsGathering false))