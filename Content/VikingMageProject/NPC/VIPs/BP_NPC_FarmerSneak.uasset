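; BP_NPC_FarmerSneak is a stealth-section farmer NPC that catches the player and sends them back along their movement spline.
; PrimaryAttack runs the blackboard target to the spline point nearest SendBackLocation, toggles their AI detectability, and pauses its own sensing on a timer.
; Hearing noise while alerted focuses it on the instigator, otherwise the parent reaction runs.
; Tick flickers its offset point light with a clamped random walk.
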(event EventTick
  (params (DeltaSeconds :type Float%20%28single-precision%29))
  (bind _output_get (Variables|Default|SetLastIntensity (Math|Random|RandomFloatinRange (Math|Float|Max(Float) (Variables|Default|GetMinIntesity) (- (Variables|Default|GetLastIntensity) (Variables|Default|GetMaxChangePerTick))) (Math|Float|Min(Float) (Variables|Default|GetMaxIntesity) (+ (Variables|Default|GetLastIntensity) (Variables|Default|GetMaxChangePerTick))))))
  (Rendering|Components|Light|SetIntensity (Variables|Default|GetPointLight) _output_get))

(event EventBeginPlay
  (|CallParentFunction)
  (Variables|Default|SetStartPosition (Transformation|GetWorldLocation (Variables|Default|GetCapsuleComponent))))

(fn ConstructionScript
  (|CallParentFunction)
  (Transformation|SetRelativeLocation (Variables|Default|GetPointLight) (Variables|Default|GetLightOffset) false false))

(fn PrimaryAttack
  (bind _returnvalue (Utilities|Name|MakeLiteralName "TargetActor"))
  (bind _self self)
  (bind _returnvalue_2 (AI|GetAIController _self))
  (bind _returnvalue_3 (AI|GetBlackboard _returnvalue_2))
  (bind _returnvalue_4 (AI|Components|Blackboard|GetValueasObject _returnvalue_3 _returnvalue))
  (Development|PrintString "Hello Got you!" true true "(R=1.000000,G=0.000000,B=0.068582,A=1.000000)")
  (Class|PawnSensingComponent|SetSensingUpdatesEnabled (Variables|Default|GetPawnSensing) false)
  (Utilities|IsValid _returnvalue_4
    (:Is%20Valid
      (bind _asbp_player_character (Utilities|Casting|CastToBP_PlayerCharacter _returnvalue_4)
        (:then
          (bind _startsuccess (Default|MovetoLocation _asbp_player_character true (Spline|FindLocationClosesttoWorldLocation (Variables|/Game/VikingMageProject/Core/World/BP_MovementPathSpline.BP_MovementPathSpline_C|GetSpline (Variables|/Game/VikingMageProject/Core/Characters/BP_CharacterCustom.BP_CharacterCustom_C|GetMovementSpline _asbp_player_character)) (Transformation|GetActorLocation (Variables|Default|GetSendBackLocation)) "World") (Variables|/Game/VikingMageProject/Core/Characters/Player/BP_PlayerCharacter.BP_PlayerCharacter_C|GetRunSpeed _asbp_player_character) false false))
          (bind _output_get (Variables|/Game/VikingMageProject/Core/Characters/Player/BP_PlayerCharacter.BP_PlayerCharacter_C|SetCanBeSeenByAI _asbp_player_character (not _startsuccess)))
          (Variables|/Game/VikingMageProject/Core/Characters/Player/BP_PlayerCharacter.BP_PlayerCharacter_C|SetmakesNoiseForAI _asbp_player_character _output_get))
        (:CastFailed
          _)))
    (:Is%20Not%20Valid
      _))
  (CallFunction|StopFocusActor true)
  (Utilities|Time|SetTimerbyEvent (EventDispatchers|CreateEvent :!event ReenableSenses) 6.0))

(fn ReenableSenses
  (Class|PawnSensingComponent|SetSensingUpdatesEnabled (Variables|Default|GetPawnSensing) true))

(fn OnHearReaction
  (params (Instigator :type Pawn%20Object%20Reference) (Location :type Vector :default "0, 0, 0") (Volume :type Float%20%28single-precision%29))
  (Development|PrintString "OnHearReaction Sneaki Farmer" true true "(R=0.000000,G=1.000000,B=0.008149,A=1.000000)" 4.0)
  (if (Variables|Default|GetIsAlerted)
    (bind _asbp_character_custom (Utilities|Casting|CastToBP_CharacterCustom Instigator))
    (CallFunction|StartFocusActor _asbp_character_custom)
    (Development|PrintString "Heared Second Time" true true "(R=0.886643,G=0.000000,B=1.000000,A=1.000000)" 1e+01)
    (else
      (|CallParentFunction Instigator Location Volume))))