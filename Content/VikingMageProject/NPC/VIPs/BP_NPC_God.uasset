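; God NPC Blueprint that appears with particle and light effects when dialog begins.
; SaySomeDialog calls Spawn and waits five seconds if no valid DialogInstigator exists, then runs the parent dialog logic.
; Spawn reveals the mesh, raises the ambient light and toggles the spawn particles.
; Despawn triggers a delayed event that swaps in despawn particles, then hides the mesh and zeroes the light.
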(event Custom|DelayedDespawn
  (bind _particlesystem (Variables|Default|GetParticleSystem))
  (Utilities|FlowControl|Delay 1.0)
  (Effects|Components|ParticleSystem|SetTemplate _particlesystem (Variables|Default|GetDespawnParticles))
  (Components|Activation|ToggleActive _particlesystem)
  (Utilities|FlowControl|Delay 0.1)
  (Development|SetHiddeninGame (Variables|Character|GetMesh) true false)
  (Rendering|Components|Light|SetIntensity (Variables|Default|GetAmbientLight) 0.0))

(event EventBeginPlay
  (|CallParentFunction) ; This node is disabled and will not be called.\nDrag off pins to build functionality.
)

(event Collision|EventActorBeginOverlap
  (params (OtherActor :type Actor%20Object%20Reference))
  (|CallParentFunction OtherActor) ; This node is disabled and will not be called.\nDrag off pins to build functionality.
)

(event EventTick
  (params (DeltaSeconds :type Float%20%28single-precision%29))
  (|CallParentFunction DeltaSeconds) ; This node is disabled and will not be called.\nDrag off pins to build functionality.
)

(event EventSaySomeDialog
  (params (Node :type Dlg%20Node%20Object%20Reference) (Instigator :type BP%20Bubble%20Dialog%20Trigger%20Object%20Reference))
  (Utilities|IsValid (Variables|Default|GetDialogInstigator)
    (:Is%20Valid
      _)
    (:Is%20Not%20Valid
      (CallFunction|Spawn)
      (Utilities|FlowControl|Delay 5.0)))
  (|CallParentFunction Node Instigator))

(fn ConstructionScript
  (|CallParentFunction))

(fn Spawn
  (bind _particlesystem (Variables|Default|GetParticleSystem))
  (Development|SetHiddeninGame (Variables|Character|GetMesh) false false)
  (Rendering|Components|Light|SetIntensity (Variables|Default|GetAmbientLight) (Variables|Default|GetLightIntensity))
  (Effects|Components|ParticleSystem|SetTemplate _particlesystem (Variables|Default|GetSpawnParticles))
  (Components|Activation|ToggleActive _particlesystem))

(fn Despawn
  (CallFunction|DelayedDespawn))