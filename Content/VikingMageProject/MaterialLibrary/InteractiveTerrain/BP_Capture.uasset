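; Scene capture actor that follows the player and maintains persistent render targets, apparently for interactive terrain.
; Each tick it snaps to the player's position in texel-sized steps to avoid swimming, publishing location to MPC_Capture, which also receives capture size at BeginPlay.
; The normalized move offset feeds a material drawn into RT_Persistent to compensate for movement, then a second material draws RT_Persistent_Blurred.
; All three render targets are cleared at BeginPlay.
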(event EventBeginPlay
  (Rendering|Material|SetScalarParameterValue "/Game/VikingMageProject/MaterialLibrary/InteractiveTerrain/MPC_Capture.MPC_Capture" "CaptureSize" (Variables|/Script/Engine.SceneCaptureComponent2D|GetOrthoWidth (Variables|Default|GetSceneCaptureComponent2D)) :!class /Script/Engine.KismetMaterialLibrary)
  (bind _returnvalue (Rendering|Material|CreateDynamicMaterialInstance "/Game/VikingMageProject/MaterialLibrary/InteractiveTerrain/M_DrawToPersistent.M_DrawToPersistent" "None" "None" :!class /Script/Engine.KismetMaterialLibrary))
  (Variables|Default|SetDrawMaterial _returnvalue)
  (bind _returnvalue_2 (Rendering|Material|CreateDynamicMaterialInstance "/Game/VikingMageProject/MaterialLibrary/InteractiveTerrain/M_DrawToPersistentBlurred.M_DrawToPersistentBlurred" "None" "None" :!class /Script/Engine.KismetMaterialLibrary))
  (Variables|Default|SetBlurredMaterial _returnvalue_2)
  (Rendering|ClearRenderTarget2D "/Game/VikingMageProject/MaterialLibrary/InteractiveTerrain/RenderTargets/RT_Capture.RT_Capture")
  (Rendering|ClearRenderTarget2D "/Game/VikingMageProject/MaterialLibrary/InteractiveTerrain/RenderTargets/RT_Persistent.RT_Persistent")
  (Rendering|ClearRenderTarget2D "/Game/VikingMageProject/MaterialLibrary/InteractiveTerrain/RenderTargets/RT_Persistent_Blurred.RT_Persistent_Blurred"))

(event EventTick
  (params (DeltaSeconds :type Float%20%28single-precision%29))
  (CallFunction|MoveCapture)
  (CallFunction|DrawtoPersistent))

(fn ConstructionScript)

(fn DrawtoPersistent
  (bind _scenecapturecomponent2d (Variables|Default|GetSceneCaptureComponent2D))
  (bind _moveoffset (Variables|Default|GetMoveOffset))
  (bind _orthowidth (Variables|/Script/Engine.SceneCaptureComponent2D|GetOrthoWidth _scenecapturecomponent2d))
  (bind _returnvalue (/ _moveoffset _orthowidth))
  (Rendering|Material|SetVectorParameterValue (Variables|Default|GetDrawMaterial) "Offset" (Utilities|Struct|MakeLinearColor (.x _returnvalue) (.y _returnvalue) 0.0 1.0) :!class /Script/Engine.MaterialInstanceDynamic)
  (Rendering|DrawMaterialtoRenderTarget "/Game/VikingMageProject/MaterialLibrary/InteractiveTerrain/RenderTargets/RT_Persistent.RT_Persistent" (Variables|Default|GetDrawMaterial))
  (Rendering|DrawMaterialtoRenderTarget "/Game/VikingMageProject/MaterialLibrary/InteractiveTerrain/RenderTargets/RT_Persistent_Blurred.RT_Persistent_Blurred" (Variables|Default|GetBlurredMaterial)))

(fn MoveCapture
  (bind _returnvalue (Game|Player|GetPlayerPawn 0))
  (bind _returnvalue_2 (Transformation|GetActorLocation))
  (bind _scenecapturecomponent2d (Variables|Default|GetSceneCaptureComponent2D))
  (bind _rtexresolution (Variables|Default|GetRTexResolution))
  (bind _returnvalue_3 (Transformation|GetActorLocation _returnvalue))
  (bind _returnvalue_4 (/ 1.0 _rtexresolution))
  (bind _orthowidth (Variables|/Script/Engine.SceneCaptureComponent2D|GetOrthoWidth _scenecapturecomponent2d))
  (bind _returnvalue_5 (* _orthowidth _returnvalue_4))
  (bind _returnvalue_6 (Utilities|SnaptoPixelWorldSize (.x _returnvalue_3) (.y _returnvalue_3) _returnvalue_5))
  (bind _returnvalue_7 (- _returnvalue_6 _returnvalue_2))
  (bind _output_get (Variables|Default|SetMoveOffset (Math|Vector2D|MakeVector2D (.x _returnvalue_7) (.y _returnvalue_7))))
  (Transformation|AddActorWorldOffset (Math|Vector|MakeVector (.x _output_get) (.y _output_get) 0.0))
  (Rendering|Material|SetVectorParameterValue "/Game/VikingMageProject/MaterialLibrary/InteractiveTerrain/MPC_Capture.MPC_Capture" "CaptureLocation" (Math|Conversions|ToLinearColor(Vector) (Transformation|GetActorLocation)) :!class /Script/Engine.KismetMaterialLibrary))