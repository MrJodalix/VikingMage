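; Blood splash actor that plays a Niagara effect and leaves blood decals where its particles collide.
; InitSplash feeds direction, velocity range and angle to the system, and Splash activates it.
; The actor registers as the Niagara export callback, then line-traces along each reported particle's velocity.
; Each trace spawns a random, randomly sized and rotated decal attached to the hit component or bone, with randomized lifespan for bone hits.
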(event EventBeginPlay
  (Niagara|SetNiagaraVariable(Object) (Variables|Default|GetBloodSplash) "User.BPCallback" self))

(event EventParticleData
  (params (Data :type Array%20of%20Basic%20Particle%20Data%20Structures) (NiagaraSystem :type Niagara%20System%20Object%20Reference))
  (CallFunction|HandleParticleCollision Data))

(fn ConstructionScript)

(fn HandleParticleCollision
  (params (ParticleData :type Array%20of%20Basic%20Particle%20Data%20Structures))
  (for _array_element ParticleData
    (bind _outhit (Collision|LineTraceByChannel (.Position (Utilities|Struct|BreakBasicParticleData _array_element)) (+ (.Position (Utilities|Struct|BreakBasicParticleData _array_element)) (* (Math|Vector|Normalize (.Velocity (Utilities|Struct|BreakBasicParticleData _array_element))) 1e+02)) "TraceTypeQuery8" true 0 "None"))
    (LocalVariables|SetBloodDecal (Utilities|Array|Get(acopy) (Variables|Default|GetBloodDecals) (Math|Random|RandomIntegerinRange 0 (- (Utilities|Array|Length (Variables|Default|GetBloodDecals)) 1))))
    (LocalVariables|SetRandSize (Math|Random|RandomFloatinRange (Variables|Default|GetMinSize) (Variables|Default|GetMaxSize)))
    (LocalVariables|SetSurfaceRot (Math|Rotator|MakeRotator (Math|Random|RandomFloatinRange 0.0 3.6e+02) (.pitch (Math|Rotator|MakeRotfromX (* (.normal _outhit) -1.0))) (.yaw (Math|Rotator|MakeRotfromX (* (.normal _outhit) -1.0)))))
    (if (Utilities|Name|NotEqual(Name) (.hitbonename _outhit) "None")
      (LocalVariables|SetDecalLifeSpan (Math|Random|RandomFloatinRange 1e+01 2e+01)))
    (Class|GameplayStatics|SpawnDecalAttached (LocalVariables|GetBloodDecal) (Math|Vector|MakeVector 1e+01 (LocalVariables|GetRandSize) (LocalVariables|GetRandSize)) (.hitcomponent _outhit) (.hitbonename _outhit) (.location _outhit) (LocalVariables|GetSurfaceRot) "KeepWorldPosition" (LocalVariables|GetDecalLifeSpan))))

(fn InitSplash
  (params (Direction :type Vector :default "0.900000,0,0.400000") (MaxVelocity :type Float%20%28single-precision%29) (MinVelocity :type Float%20%28single-precision%29) (SplatAngle :type Float%20%28single-precision%29))
  (bind _bloodsplash (Variables|Default|GetBloodSplash))
  (Niagara|SetNiagaraVariable(Float) _bloodsplash "User.SplatAngle" SplatAngle)
  (Niagara|SetNiagaraVariable(Float) _bloodsplash "User.MaxSplatVelocity" MaxVelocity)
  (Niagara|SetNiagaraVariable(Float) _bloodsplash "User.MinSplatVelocity" MinVelocity)
  (Class|NiagaraComponent|SetNiagaraVariableVec3 _bloodsplash "User.SplatDirection" Direction))

(fn Splash
  (Components|Activation|SetActive (Variables|Default|GetBloodSplash) true false))