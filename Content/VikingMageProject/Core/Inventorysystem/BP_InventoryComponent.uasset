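; Inventory component for the player and other actors such as chests or NPCs, holding ItemID/amount stacks.
; Pickups and transfers merge into stacks using DT_Items limits or fill free slots, then refresh the player HUD and notify the owner's quest log.
; Interacting opens this inventory beside the player's.
; Mouse drops spawn physics items by projecting the cursor onto the movement spline's plane, clamped near the player.
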(event Custom|Interact_1_1
  (params (Interactor :type BP%20Character%20Custom%20Object%20Reference))
  (bind _asbp_player_character (Utilities|Casting|CastToBP_PlayerCharacter (Game|GetPlayerCharacter 0)))
  (CallFunction|OpenOtherInventory (Variables|/Game/VikingMageProject/Core/Characters/Player/BP_PlayerCharacter.BP_PlayerCharacter_C|GetInventory%20%28InventoryComponent%29 _asbp_player_character) self))

(fn DropItem
  (params (IndexInInventory :type Integer))
  (bind _returnvalue (Game|Player|GetPlayerPawn 0))
  (bind _rootcomponent (Variables|/Script/Engine.Actor|GetRootComponent _returnvalue))
  ;[1 1 1] Lässt ein Item in der Welt fallen (es wird aus dem Inventar entfernt)
  (bind _returnvalue_2 (Game|SpawnActorfromClass "/Game/VikingMageProject/Core/Inventorysystem/Items/BP_Item.BP_Item_C" (Math|Transform|MakeTransform (+ (Transformation|GetWorldLocation _rootcomponent) (* (Math|Vector|GetForwardVector _rootcomponent) 25))) "Undefined" 0 0))
  (Default|Dropped _returnvalue_2 (.ItemID (Utilities|Struct|BreakSInventory (Utilities|Array|Get(acopy) (Variables|Default|GetItems) IndexInInventory))))
  (Physics|SetSimulatePhysics (Variables|/Game/VikingMageProject/Core/Inventorysystem/Items/BP_Item.BP_Item_C|GetItemMesh _returnvalue_2) true)
  (CallFunction|ConsumeItems IndexInInventory 1))

(fn ConsumeItems
  (params (Index :type Integer) (Amount :type Integer))
  (bind _items (Variables|Default|GetItems))
  (bind _items_2 (Variables|Default|GetItems))
  (bind _output (Utilities|Array|Get(acopy) _items Index))
  (bind (_itemid _amount) (Utilities|Struct|BreakSInventory _output))
  (bind _returnvalue (- _amount Amount))
  ;[1 1 1] Ein Item wird mit einer bestimmten Anzahl aus dem Spielerinventar entfernt
  (if (== _returnvalue 0)
    (Utilities|Array|RemoveIndex _items_2 Index)
    (else
      (Utilities|Array|SetArrayElem _items_2 Index (Utilities|Struct|MakeSInventory _itemid _returnvalue))))
  (CallFunction|RefreshPlayerInventory))

(fn EatItem
  (params (IdexInInv :type Integer))
  ;[1 1 1] Isst ein Item
  (CallFunction|ConsumeItems IdexInInv 1))

(fn AddItemfromWorld
  (params (HitActor :type Actor%20Object%20Reference))
  (bind _returnvalue (Components|GetOwner))
  (bind _returnvalue_2 (Actor|GetComponentbyClass _returnvalue "/Game/VikingMageProject/Core/QuestSystemInterface/BP_QuestLogComponent.BP_QuestLogComponent_C"))
  ;[1 1 1] Fügt dem Spielerinventar ein Item aus der Welt hinzu
  (Utilities|IsValid HitActor
    (:Is%20Valid
      (bind (_itemid _canbepickedup _amount) (Class|BIItemInterface|PickUp(Message) HitActor))
      (LocalVariables|SetItemFound false)
      (if _canbepickedup
        (for (_array_element _array_index) (Variables|Default|GetItems)
          (bind _returnvalue_3 (Utilities|GetDataTableRow "/Game/VikingMageProject/Core/Inventorysystem/Items/DT_Items.DT_Items" (Utilities|String|StringToName (Utilities|String|ToString(Integer) (.ItemID (Utilities|Struct|BreakSInventory _array_element)))))
            (:then
              (if (Math|Boolean|ANDBoolean (== (.ItemID (Utilities|Struct|BreakSInventory _array_element)) _itemid) (< (+ (.Amount (Utilities|Struct|BreakSInventory _array_element)) _amount) (.MaxAmountPerStack (Utilities|Struct|BreakSItemData _returnvalue_3))) (not (LocalVariables|GetItemFound)))
                (LocalVariables|SetItemFound true)
                (Utilities|Array|SetArrayElem (Variables|Default|GetItems) _array_index (Utilities|Struct|MakeSInventory _itemid (+ (.Amount (Utilities|Struct|BreakSInventory _array_element)) _amount)))
                (Actor|DestroyActor HitActor)
                (Default|RenewInventory (Variables|/Game/VikingMageProject/Core/UI/WBP_PlayerHUD.WBP_PlayerHUD_C|GetWBP_Inventory_Players (Variables|/Game/VikingMageProject/Core/Characters/Player/BP_PlayerCharacter.BP_PlayerCharacter_C|GetWBP_PlayerHUD (.AsBP%20Player%20Character (Utilities|Casting|CastToBP_PlayerCharacter (Game|GetPlayerCharacter 0))))))
                (if (Utilities|IsValid _returnvalue_2)
                  (Default|ItemCollected _returnvalue_2 _itemid (CallFunction|GetItemAmount _itemid)))))))
        (if (and (not (LocalVariables|GetItemFound)) (< (Utilities|Array|Length (Variables|Default|GetItems)) (Variables|Default|GetMaxItemInInv)))
          (Utilities|Array|Add (Variables|Default|GetItems) (Utilities|Struct|MakeSInventory _itemid _amount))
          (Actor|DestroyActor HitActor)
          (Default|RenewInventory (Variables|/Game/VikingMageProject/Core/UI/WBP_PlayerHUD.WBP_PlayerHUD_C|GetWBP_Inventory_Players (Variables|/Game/VikingMageProject/Core/Characters/Player/BP_PlayerCharacter.BP_PlayerCharacter_C|GetWBP_PlayerHUD (.AsBP%20Player%20Character (Utilities|Casting|CastToBP_PlayerCharacter (Game|GetPlayerCharacter 0))))))
          (if (Utilities|IsValid _returnvalue_2)
            (Default|ItemCollected _returnvalue_2 _itemid (CallFunction|GetItemAmount _itemid))))))))

(fn AddItemsfromInventory
  (params (Item%20ID :type Integer) (Amount :type Integer))
  (bind _returnvalue (Game|GetPlayerCharacter 0))
  (bind _returnvalue_2 (Components|GetOwner))
  (bind _items (Variables|Default|GetItems))
  (bind _returnvalue_3 (Utilities|Array|Length _items))
  (bind _returnvalue_4 (Actor|GetComponentbyClass _returnvalue_2 "/Game/VikingMageProject/Core/QuestSystemInterface/BP_QuestLogComponent.BP_QuestLogComponent_C"))
  (bind _asbp_player_character (Utilities|Casting|CastToBP_PlayerCharacter _returnvalue))
  (bind _returnvalue_5 (Utilities|IsValid _returnvalue_4))
  (bind _wbp_playerhud (Variables|/Game/VikingMageProject/Core/Characters/Player/BP_PlayerCharacter.BP_PlayerCharacter_C|GetWBP_PlayerHUD _asbp_player_character))
  (bind _wbp_inventory_players (Variables|/Game/VikingMageProject/Core/UI/WBP_PlayerHUD.WBP_PlayerHUD_C|GetWBP_Inventory_Players _wbp_playerhud))
  (bind _wbp_inventory_other_actor (Variables|/Game/VikingMageProject/Core/Inventorysystem/Widgets/WBP_Inventory_Players.WBP_Inventory_Players_C|GetWBP_Inventory_Other_Actor _wbp_inventory_players))
  ;[1 1 1] Fügt dem Spielerinventar ein Item mit einer gewissen Anzahl aus einem anderen Inventar hinzu
  (LocalVariables|SetFoundItem false)
  (for (_array_element _array_index) (Variables|Default|GetItems)
    (bind _returnvalue_6 (Utilities|GetDataTableRow "/Game/VikingMageProject/Core/Inventorysystem/Items/DT_Items.DT_Items" (Utilities|String|StringToName (Utilities|String|ToString(Integer) (.ItemID (Utilities|Struct|BreakSInventory _array_element)))))
      (:then
        (if (Math|Boolean|ANDBoolean (== (.ItemID (Utilities|Struct|BreakSInventory _array_element)) Item%20ID) (not (LocalVariables|GetFoundItem)) (<= (+ (.Amount (Utilities|Struct|BreakSInventory _array_element)) Amount) (.MaxAmountPerStack (Utilities|Struct|BreakSItemData _returnvalue_6))))
          (LocalVariables|SetFoundItem true)
          (Utilities|Array|SetArrayElem (Variables|Default|GetItems) _array_index (Utilities|Struct|MakeSInventory (.ItemID (Utilities|Struct|BreakSInventory _array_element)) (+ (.Amount (Utilities|Struct|BreakSInventory _array_element)) Amount)))
          (Default|RenewInventory _wbp_inventory_players)
          (Default|RenewInventory _wbp_inventory_other_actor)
          (if _returnvalue_5
            (Default|ItemCollected _returnvalue_4 Item%20ID (CallFunction|GetItemAmount Item%20ID)))))))
  (Development|PrintString (Utilities|String|Append (Utilities|String|ToString(Integer) _returnvalue_3) (Utilities|String|ToString(Boolean) (LocalVariables|GetFoundItem))) true true "(R=0.000000,G=0.000000,B=0.000000,A=1.000000)" 4.0)
  (if (and (not (LocalVariables|GetFoundItem)) (< _returnvalue_3 (Variables|Default|GetMaxItemInInv)))
    (Utilities|Array|Add (Variables|Default|GetItems) (Utilities|Struct|MakeSInventory Item%20ID Amount))
    (Default|RenewInventory _wbp_inventory_players)
    (Default|RenewInventory _wbp_inventory_other_actor)
    (if _returnvalue_5
      (Default|ItemCollected _returnvalue_4 Item%20ID (CallFunction|GetItemAmount Item%20ID)))
    (return true)
    (else
      (return (LocalVariables|GetFoundItem)))))

(fn MoveItemstoOtherInventory
  (params (Other%20Inventory :type BP%20Inventory%20Component%20Object%20Reference) (Item%20ID :type Integer) (Amount :type Integer))
  ;[1 1 1] Entfernt ein Item (Anzahl) aus dem Spielerinventar und fügt es einem Actorinventar hinzu
  (for _array_element (Variables|Default|GetItems)
    (if (== (.ItemID (Utilities|Struct|BreakSInventory _array_element)) Item%20ID)
      (if (< (.Amount (Utilities|Struct|BreakSInventory _array_element)) Amount)
        (CallFunction|AddItemsfromInventory Other%20Inventory (.ItemID (Utilities|Struct|BreakSInventory _array_element)) (.Amount (Utilities|Struct|BreakSInventory _array_element)))
        (CallFunction|ConsumeItems (.ItemID (Utilities|Struct|BreakSInventory _array_element)) (.Amount (Utilities|Struct|BreakSInventory _array_element)))
        (else
          (CallFunction|AddItemsfromInventory Other%20Inventory (.ItemID (Utilities|Struct|BreakSInventory _array_element)) Amount)
          (CallFunction|ConsumeItems (.ItemID (Utilities|Struct|BreakSInventory _array_element)) Amount))))))

(fn CheckifItemsAreinInventory
  (params (Item%20ID :type Integer) (Amount :type Integer))
  ;[1 1 1] Prüft, ob ein Item im Inventar des Spielers in einer bestimmten Anzahl vorliegt
  (LocalVariables|SetAmountFound 0)
  (for _array_element (Variables|Default|GetItems)
    (if (== (.ItemID (Utilities|Struct|BreakSInventory _array_element)) Item%20ID)
      (LocalVariables|SetAmountFound (+ (.Amount (Utilities|Struct|BreakSInventory _array_element)) (LocalVariables|GetAmountFound)))))
  (return (>= (LocalVariables|GetAmountFound) Amount) (LocalVariables|GetAmountFound)))

(fn OpenOtherInventory
  (params (OtherInventory :type BP%20Inventory%20Component%20Object%20Reference))
  ;[1 1 1] Öffnet das Inventar eines anderen Actors (z.B. eine Kiste, NPC, etc.) und das eigene
  (bind _asbp_player_character (Utilities|Casting|CastToBP_PlayerCharacter (Game|GetPlayerCharacter 0)))
  (Default|OpenOtherInventory (Variables|/Game/VikingMageProject/Core/UI/WBP_PlayerHUD.WBP_PlayerHUD_C|GetWBP_Inventory_Players (Variables|/Game/VikingMageProject/Core/Characters/Player/BP_PlayerCharacter.BP_PlayerCharacter_C|GetWBP_PlayerHUD _asbp_player_character)) OtherInventory)
  (Default|TriggerMenu (Variables|/Game/VikingMageProject/Core/Characters/Player/BP_PlayerCharacter.BP_PlayerCharacter_C|GetWBP_PlayerHUD _asbp_player_character) "NewEnumerator6" false))

(fn CloseOtherInventory
  ;[1 1 1] Schließt das Inventar eines anderen Actors (z.B. eine Kiste, NPC, etc.) und das eigene
  (bind _asbp_player_character (Utilities|Casting|CastToBP_PlayerCharacter (Game|GetPlayerCharacter 0)))
  (if (and (Utilities|Enum|Equal(Enum) (Variables|/Game/VikingMageProject/Core/UI/WBP_PlayerHUD.WBP_PlayerHUD_C|GetCurrentMenu (Variables|/Game/VikingMageProject/Core/Characters/Player/BP_PlayerCharacter.BP_PlayerCharacter_C|GetWBP_PlayerHUD _asbp_player_character)) "NewEnumerator6") (Default|IsOtherInventoryOpened (Variables|/Game/VikingMageProject/Core/UI/WBP_PlayerHUD.WBP_PlayerHUD_C|GetWBP_Inventory_Players (Variables|/Game/VikingMageProject/Core/Characters/Player/BP_PlayerCharacter.BP_PlayerCharacter_C|GetWBP_PlayerHUD _asbp_player_character))))
    (Default|TriggerMenu (Variables|/Game/VikingMageProject/Core/Characters/Player/BP_PlayerCharacter.BP_PlayerCharacter_C|GetWBP_PlayerHUD _asbp_player_character) "NewEnumerator6" false)))

(fn GetItemAmount
  (params (ItemID :type Integer))
  (LocalVariables|SetAmountFound 0)
  (for _array_element (Variables|Default|GetItems)
    (if (== (.ItemID (Utilities|Struct|BreakSInventory _array_element)) ItemID)
      (LocalVariables|SetAmountFound (+ (.Amount (Utilities|Struct|BreakSInventory _array_element)) (LocalVariables|GetAmountFound)))))
  (return (LocalVariables|GetAmountFound)))

(fn RefreshPlayerInventory
  (Default|RenewInventory (Variables|/Game/VikingMageProject/Core/UI/WBP_PlayerHUD.WBP_PlayerHUD_C|GetWBP_Inventory_Players (Variables|/Game/VikingMageProject/Core/Characters/Player/BP_PlayerCharacter.BP_PlayerCharacter_C|GetWBP_PlayerHUD (.AsBP%20Player%20Character (Utilities|Casting|CastToBP_PlayerCharacter (Game|GetPlayerCharacter 0)))))))

(fn RemoveItembyID
  (params (ItemID :type Integer) (ItemAmount :type Integer))
  (for (_array_element _array_index) (Variables|Default|GetItems)
    (if (== (.itemid _array_element) ItemID)
      (CallFunction|ConsumeItems _array_index ItemAmount))))

(fn DropIteminScreen
  (params (IndexInInventory :type Integer))
  (bind _returnvalue (Game|GetPlayerCharacter 0))
  (bind _returnvalue_2 (Game|GetPlayerCharacter 0))
  (bind _asbp_player_character (Utilities|Casting|CastToBP_PlayerCharacter _returnvalue))
  (bind _asbp_player_character_2 (Utilities|Casting|CastToBP_PlayerCharacter _returnvalue_2))
  (bind _capsulecomponent (Variables|/Script/Engine.Character|GetCapsuleComponent _asbp_player_character_2))
  (bind _capsulecomponent_2 (Variables|/Script/Engine.Character|GetCapsuleComponent _asbp_player_character))
  (bind _returnvalue_3 (Transformation|GetWorldLocation _capsulecomponent_2))
  (bind _returnvalue_4 (Transformation|GetWorldLocation _capsulecomponent))
  (if true
    (bind _returnvalue_5 (Class|WidgetLayoutLibrary|GetMousePositiononViewport))
    (bind _returnvalue_6 (Game|SpawnActorfromClass "/Game/VikingMageProject/Core/Inventorysystem/Items/BP_Item.BP_Item_C" (Math|Transform|MakeTransform (+ (Math|Vector|MakeVector (.x (Math|Vector|ClampVectorSize (- (.Intersection (Class|KismetMathLibrary|LinePlaneIntersectionOriginNormal (.WorldPosition (Class|GameplayStatics|DeprojectScreentoWorld (Game|GetPlayerController 0) (* (Math|Vector2D|MakeVector2D (.x _returnvalue_5) (.y _returnvalue_5)) (Class|WidgetLayoutLibrary|GetViewportScale)))) (+ (.WorldPosition (Class|GameplayStatics|DeprojectScreentoWorld (Game|GetPlayerController 0) (* (Math|Vector2D|MakeVector2D (.x _returnvalue_5) (.y _returnvalue_5)) (Class|WidgetLayoutLibrary|GetViewportScale)))) (* (.WorldDirection (Class|GameplayStatics|DeprojectScreentoWorld (Game|GetPlayerController 0) (* (Math|Vector2D|MakeVector2D (.x _returnvalue_5) (.y _returnvalue_5)) (Class|WidgetLayoutLibrary|GetViewportScale)))) 1e+03)) _returnvalue_4 (Class|SplineComponent|FindRightVectorClosesttoWorldLocation (Variables|/Game/VikingMageProject/Core/World/BP_MovementPathSpline.BP_MovementPathSpline_C|GetSpline (Variables|/Game/VikingMageProject/Core/Characters/BP_CharacterCustom.BP_CharacterCustom_C|GetMovementSpline _asbp_player_character_2)) _returnvalue_4 "World"))) _returnvalue_3) 0.0 (Variables|Default|GetMaxItemSpawnDistance))) (.y (Math|Vector|ClampVectorSize (- (.Intersection (Class|KismetMathLibrary|LinePlaneIntersectionOriginNormal (.WorldPosition (Class|GameplayStatics|DeprojectScreentoWorld (Game|GetPlayerController 0) (* (Math|Vector2D|MakeVector2D (.x _returnvalue_5) (.y _returnvalue_5)) (Class|WidgetLayoutLibrary|GetViewportScale)))) (+ (.WorldPosition (Class|GameplayStatics|DeprojectScreentoWorld (Game|GetPlayerController 0) (* (Math|Vector2D|MakeVector2D (.x _returnvalue_5) (.y _returnvalue_5)) (Class|WidgetLayoutLibrary|GetViewportScale)))) (* (.WorldDirection (Class|GameplayStatics|DeprojectScreentoWorld (Game|GetPlayerController 0) (* (Math|Vector2D|MakeVector2D (.x _returnvalue_5) (.y _returnvalue_5)) (Class|WidgetLayoutLibrary|GetViewportScale)))) 1e+03)) _returnvalue_4 (Class|SplineComponent|FindRightVectorClosesttoWorldLocation (Variables|/Game/VikingMageProject/Core/World/BP_MovementPathSpline.BP_MovementPathSpline_C|GetSpline (Variables|/Game/VikingMageProject/Core/Characters/BP_CharacterCustom.BP_CharacterCustom_C|GetMovementSpline _asbp_player_character_2)) _returnvalue_4 "World"))) _returnvalue_3) 0.0 (Variables|Default|GetMaxItemSpawnDistance))) (Math|Float|Max(Float) (.z (Math|Vector|ClampVectorSize (- (.Intersection (Class|KismetMathLibrary|LinePlaneIntersectionOriginNormal (.WorldPosition (Class|GameplayStatics|DeprojectScreentoWorld (Game|GetPlayerController 0) (* (Math|Vector2D|MakeVector2D (.x _returnvalue_5) (.y _returnvalue_5)) (Class|WidgetLayoutLibrary|GetViewportScale)))) (+ (.WorldPosition (Class|GameplayStatics|DeprojectScreentoWorld (Game|GetPlayerController 0) (* (Math|Vector2D|MakeVector2D (.x _returnvalue_5) (.y _returnvalue_5)) (Class|WidgetLayoutLibrary|GetViewportScale)))) (* (.WorldDirection (Class|GameplayStatics|DeprojectScreentoWorld (Game|GetPlayerController 0) (* (Math|Vector2D|MakeVector2D (.x _returnvalue_5) (.y _returnvalue_5)) (Class|WidgetLayoutLibrary|GetViewportScale)))) 1e+03)) _returnvalue_4 (Class|SplineComponent|FindRightVectorClosesttoWorldLocation (Variables|/Game/VikingMageProject/Core/World/BP_MovementPathSpline.BP_MovementPathSpline_C|GetSpline (Variables|/Game/VikingMageProject/Core/Characters/BP_CharacterCustom.BP_CharacterCustom_C|GetMovementSpline _asbp_player_character_2)) _returnvalue_4 "World"))) _returnvalue_3) 0.0 (Variables|Default|GetMaxItemSpawnDistance))) 0.0)) _returnvalue_3)) "AdjustIfPossibleButDontSpawnIfColliding" 0 0))
    (Default|Dropped _returnvalue_6 (.ItemID (Utilities|Struct|BreakSInventory (Utilities|Array|Get(acopy) (Variables|Default|GetItems) IndexInInventory))))
    (Physics|SetSimulatePhysics (Variables|/Game/VikingMageProject/Core/Inventorysystem/Items/BP_Item.BP_Item_C|GetItemMesh _returnvalue_6) true)
    (CallFunction|ConsumeItems IndexInInventory 1)))

(fn Interact
  (params (Interactor :type BP%20Player%20Character%20Object%20Reference))
  (return false))