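; A level-up rune item that drops with physics, hovers once settled, and is picked up into the player's rune list.
; Tick waits until velocity falls below a threshold, then disables physics, enables a custom-depth outline, raises the mesh and spins it.
; Cursor hover shows the name and outline.
; AddLevelUPRune inserts the EXP cost before the first lower-or-equal entry, adding nothing if none qualifies in a non-empty list, then destroys the actor.
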(event EventBeginPlay
  (Components|StaticMesh|SetStaticMesh (Variables|Default|GetRune) (Variables|Default|GetRuneMesh))
  (Physics|SetSimulatePhysics (Variables|Default|GetRune) true)
  (Utilities|FlowControl|Delay 0.1)
  (Actor|Tick|SetActorTickEnabled true))

(event EventTick
  (params (DeltaSeconds :type Float%20%28single-precision%29))
  (bind _rune (Variables|Default|GetRune))
  (bind _rune_2 (Variables|Default|GetRune))
  (bind _rune_3 (Variables|Default|GetRune))
  (bind _returnvalue (Transformation|GetWorldLocation _rune))
  (bind _returnvalue_2 (Transformation|GetWorldRotation _rune_2))
  (if (<= (Math|Vector|VectorLength (Transformation|GetComponentVelocity (Variables|Default|GetRune))) (Variables|Default|GetMovementThreshold))
    (if (not (Variables|Default|GetHoverPositionReached))
      (Rendering|SetRenderCustomDepth _rune_3 true)
      (Rendering|SetCustomDepthStencilValue _rune_3 (Variables|Default|GetOutlineColorType))
      (Physics|SetSimulatePhysics _rune false)
      (Variables|Default|SetHoverPositionReached true)
      (Components|MoveComponentTo _rune (Math|Vector|MakeVector (.x _returnvalue) (.y _returnvalue) (+ (.z _returnvalue) (Variables|Default|GetHoverHeight))) "0, 0, 0" false false 1.0 false)
      (else
        (Transformation|SetWorldRotation _rune_2 (Math|Rotator|MakeRotator (.roll _returnvalue_2) (.pitch _returnvalue_2) (+ (.yaw _returnvalue_2) (* DeltaSeconds (Variables|Default|GetRotationSpeed)))) false false)))))

(event MouseInput|EventActorBeginCursorOver
  (bind _rune (Variables|Default|GetRune))
  (Rendering|SetRenderCustomDepth _rune true)
  (Rendering|SetCustomDepthStencilValue _rune (Variables|Default|GetOutlineColorType))
  (CallFunction|SetNameVisibility true))

(event MouseInput|EventActorEndCursorOver
  (if (not (<= (Math|Vector|VectorLength (Transformation|GetComponentVelocity (Variables|Default|GetRune))) (Variables|Default|GetMovementThreshold)))
    (Rendering|SetRenderCustomDepth (Variables|Default|GetRune) false))
  (CallFunction|SetNameVisibility false))

(fn ConstructionScript)

(fn AddLevelUPRune
  (params (PlayerCharackter :type BP%20Player%20Character%20Object%20Reference))
  (bind _leveluprunes (Variables|/Game/VikingMageProject/Core/Characters/Player/BP_PlayerCharacter.BP_PlayerCharacter_C|GetLevelUpRunes PlayerCharackter))
  (Development|PrintString "Add Level UP ruen" true true "(R=1.000000,G=0.321939,B=0.000000,A=1.000000)")
  (if (== (Utilities|Array|Length _leveluprunes) 0)
    (Utilities|Array|Add _leveluprunes (Variables|Default|GetEXP_Cost))
    (CallFunction|PickUp)
    (else
      (bind (_array_element _array_index) (Utilities|Array|ForEachLoopwithBreak _leveluprunes :!label _label)
        (:LoopBody
          (if (<= _array_element (Variables|Default|GetEXP_Cost))
            (Utilities|Array|Insert _leveluprunes (Variables|Default|GetEXP_Cost) _array_index)
            (goto _label Break)))
        (:Completed
          (CallFunction|PickUp))))))

(fn PickUp
  (Development|PrintString "Pickup Rune")
  (Actor|DestroyActor)
  (return 0 false 0))