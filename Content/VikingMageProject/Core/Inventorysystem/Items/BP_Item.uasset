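; BP_Item is a world pickup item in the inventory system, whose mesh comes from DT_Items by ItemID at construction or when dropped.
; Player overlap and cursor hover drive a custom-depth outline.
; While hovered, Tick compares player distance to PickUpDist, switching outline stencil color and showing the name widget only when in range.
; PickUp fires CallCollected and returns the ID, pickup flag and an amount of one.
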(event EventDropped
  (params (Item%20ID :type Integer))
  (bind _output_get (Variables|Default|SetItemID Item%20ID))
  (bind _returnvalue (Utilities|GetDataTableRow "/Game/VikingMageProject/Core/Inventorysystem/Items/DT_Items.DT_Items" (Utilities|String|StringToName (Utilities|String|ToString(Integer) _output_get)))
    (:then
      (if (== (.ItemID (Utilities|Struct|BreakSItemData _returnvalue)) (Variables|Default|GetItemID))
        (Components|StaticMesh|SetStaticMesh (Variables|Default|GetItemMesh) (.Mesh (Utilities|Struct|BreakSItemData _returnvalue)))))))

(event EventOnBecomeViewTarget
  (params (PC :type Player%20Controller%20Object%20Reference))
  (CallFunction|SetNameVisibility true))

(event EventBeginPlay
  (Physics|SetSimulatePhysics (Variables|Default|GetItemMesh) (Variables|Default|GetShouldHavePhysics))
  (Transformation|SetMobility (Variables|Default|GetItemNameWidget) "Movable"))

(event EventSetNameVisibility
  (params (Visibility :type Boolean))
  (bind _aswbp_item_name (Utilities|Casting|CastToWBP_ItemName (UserInterface|GetWidget (Variables|Default|GetItemNameWidget))))
  (Variables|/Game/VikingMageProject/Core/Inventorysystem/Items/WBP_ItemName.WBP_ItemName_C|SetItemName _aswbp_item_name (Utilities|Text|ToText(Name) (Variables|Default|GetItemName)))
  (Rendering|SetVisibility (Variables|Default|GetItemNameWidget) Visibility true))

(event EventTick
  (params (DeltaSeconds :type Float%20%28single-precision%29))
  (bind _itemmesh (Variables|Default|GetItemMesh))
  (if (Variables|Default|GetIsCursorOver)
    (bind _asbp_player_character (Utilities|Casting|CastToBP_PlayerCharacter (Game|GetPlayerCharacter 0)))
    (if (<= (Math|Vector|VectorLength (- (Transformation|GetActorLocation) (Transformation|GetWorldLocation (Variables|/Script/Engine.Character|GetCapsuleComponent _asbp_player_character)))) (Variables|/Game/VikingMageProject/Core/Characters/Player/BP_PlayerCharacter.BP_PlayerCharacter_C|GetPickUpDist _asbp_player_character))
      (Rendering|SetCustomDepthStencilValue _itemmesh (Variables|Default|GetOutlineColorType))
      (CallFunction|SetNameVisibility true)
      (else
        (Rendering|SetCustomDepthStencilValue _itemmesh (Variables|Default|GetOutlineColorTypeTooFar))
        (CallFunction|SetNameVisibility false)))))

(event MouseInput|EventActorBeginCursorOver
  (Utilities|IsValid (Game|GetPlayerCharacter 0)
    (:Is%20Valid
      (Variables|Default|SetIsCursorOver true)
      (Rendering|SetRenderCustomDepth (Variables|Default|GetItemMesh) true))))

(event MouseInput|EventActorEndCursorOver
  (bind _itemmesh (Variables|Default|GetItemMesh))
  (Variables|Default|SetIsCursorOver false)
  (Rendering|SetRenderCustomDepth (Variables|Default|GetItemMesh) false)
  (CallFunction|SetNameVisibility false)
  (if (Variables|Default|GetIsActorOverlapping)
    (Rendering|SetRenderCustomDepth _itemmesh true)
    (Rendering|SetCustomDepthStencilValue _itemmesh (Variables|Default|GetOutlineColorTypeTooFar))))

(event Collision|EventActorBeginOverlap
  (params (OtherActor :type Actor%20Object%20Reference))
  (bind _itemmesh (Variables|Default|GetItemMesh))
  (Utilities|Casting|CastToBP_PlayerCharacter OtherActor)
  (Variables|Default|SetIsActorOverlapping true)
  (if (not (Variables|Default|GetIsCursorOver))
    (Rendering|SetRenderCustomDepth _itemmesh true)
    (Rendering|SetCustomDepthStencilValue _itemmesh (Variables|Default|GetOutlineColorTypeTooFar))))

(event Collision|EventActorEndOverlap
  (params (OtherActor :type Actor%20Object%20Reference))
  (Utilities|Casting|CastToBP_PlayerCharacter OtherActor)
  (Variables|Default|SetIsActorOverlapping false)
  (if (not (Variables|Default|GetIsCursorOver))
    (Rendering|SetRenderCustomDepth (Variables|Default|GetItemMesh) false)))

(fn ConstructionScript
  (CallFunction|Dropped (Variables|Default|GetItemID)))

(fn PickUp
  (Default|CallCollected)
  (return (Variables|Default|GetItemID) (Variables|Default|GetCanBePickedUp) 1))