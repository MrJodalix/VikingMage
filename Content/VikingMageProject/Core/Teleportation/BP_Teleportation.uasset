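; Teleporter trigger that moves the player to its Target after they stay overlapping for TimeTillTeleportation seconds.
; Overlap starts a timer and fades out via a level sequence and the player HUD; leaving early cancels and reverses the fade.
; Tick polls the timer, then assigns the Target's spline as the player's MovementSpline, teleports the capsule to the Target and fades back in.
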(event EventBeginPlay
  (bind _returnvalue (Sequencer|Player|CreateLevelSequencePlayer "/Game/VikingMageProject/Cinematics/FadeOut.FadeOut"))
  (Variables|Default|SetSequenzPlayer _returnvalue))

(event Collision|EventActorBeginOverlap
  (params (OtherActor :type Actor%20Object%20Reference))
  (bind _returnvalue (Utilities|Time|GetTimeSeconds))
  (Utilities|Casting|CastToBP_PlayerCharacter OtherActor)
  (Variables|Default|SetActorOverlaps true)
  (Variables|Default|SetTimer _returnvalue)
  (Development|PrintString (Utilities|String|ToString(Float) _returnvalue) true true "(R=0.000000,G=0.660000,B=1.000000,A=1.000000)" 4.0)
  (CallFunction|Fade false 0.5))

(event Collision|EventActorEndOverlap
  (params (OtherActor :type Actor%20Object%20Reference))
  (Utilities|Casting|CastToBP_PlayerCharacter OtherActor)
  (if (< (- (Utilities|Time|GetTimeSeconds) (Variables|Default|GetTimer)) (Variables|Default|GetTimeTillTeleportation))
    (Development|PrintString "Leave under 2 Sec" true true "(R=0.000000,G=0.660000,B=1.000000,A=1.000000)" 4.0)
    (Variables|Default|SetTimer 0.0)
    (Variables|Default|SetActorOverlaps false)
    (CallFunction|Fade true 0.5)))

(event EventTick
  (params (DeltaSeconds :type Float%20%28single-precision%29))
  (bind _target (Variables|Default|GetTarget))
  (if (and (Variables|Default|GetActorOverlaps) (>= (- (Utilities|Time|GetTimeSeconds) (Variables|Default|GetTimer)) (Variables|Default|GetTimeTillTeleportation)))
    (Development|PrintString "Stayed 2 Sec")
    (Variables|Default|SetTimer 0.0)
    (Variables|Default|SetActorOverlaps false)
    (bind _asbp_player_character (Utilities|Casting|CastToBP_PlayerCharacter (Game|GetPlayerCharacter 0)))
    (Variables|/Game/VikingMageProject/Core/Characters/Player/BP_PlayerCharacter.BP_PlayerCharacter_C|SetMovementSpline _asbp_player_character (Variables|/Game/VikingMageProject/Core/Teleportation/BP_TargetTeleportation.BP_TargetTeleportation_C|GetTargetSpline _target))
    (Transformation|SetWorldLocation (Variables|/Script/Engine.Character|GetCapsuleComponent _asbp_player_character) (Transformation|GetWorldLocation (Variables|/Game/VikingMageProject/Core/Teleportation/BP_TargetTeleportation.BP_TargetTeleportation_C|GetDefaultSceneRoot _target)) false true)
    (CallFunction|Fade true 0.25)))

(fn ConstructionScript)

(fn Fade
  (params (Fade%20In :type Boolean) (Speed :type Float%20%28single-precision%29))
  (bind _sequenzplayer (Variables|Default|GetSequenzPlayer))
  (if Fade%20In
    (Class|MovieSceneSequencePlayer|PlayReverse _sequenzplayer)
    (else
      (Sequencer|Player|Play _sequenzplayer :!class /Script/MovieScene.MovieSceneSequencePlayer)))
  (Default|FadePlayerUI (Variables|/Game/VikingMageProject/Core/Characters/Player/BP_PlayerCharacter.BP_PlayerCharacter_C|GetWBP_PlayerHUD (.AsBP%20Player%20Character (Utilities|Casting|CastToBP_PlayerCharacter (Game|GetPlayerCharacter 0)))) Fade%20In Speed))