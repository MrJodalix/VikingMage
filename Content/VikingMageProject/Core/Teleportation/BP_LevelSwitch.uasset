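; Level-switch trigger that sends the player to a configured level and destination tag after they stay inside for a set time.
; Overlap starts a level-sequence and HUD fade-out, unless a focused player is disallowed; leaving early reverses it.
; Tick checks the dwell time, then writes player data and spawn info to the game instance's save, saves the level and calls the player's Respawn rather than opening the level directly.
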(event EventBeginPlay
  (bind _returnvalue (Sequencer|Player|CreateLevelSequencePlayer "/Game/VikingMageProject/Cinematics/FadeOut.FadeOut"))
  (Variables|Default|SetSequenzPlayer _returnvalue))

(event Collision|EventActorBeginOverlap
  (params (OtherActor :type Actor%20Object%20Reference))
  (bind _returnvalue (Utilities|Time|GetTimeSeconds))
  (bind _asbp_player_character (Utilities|Casting|CastToBP_PlayerCharacter OtherActor))
  (Variables|Default|SetPlayerChar _asbp_player_character)
  (Variables|Default|SetActorOverlaps true)
  (Variables|Default|SetTimer _returnvalue)
  (Development|PrintString (Utilities|String|ToString(Float) _returnvalue) true true "(R=0.000000,G=0.660000,B=1.000000,A=1.000000)" 4.0)
  (if (or (Variables|Default|GetCanUseFocused) (not (Variables|/Game/VikingMageProject/Core/Characters/BP_CharacterCustom.BP_CharacterCustom_C|GetIsFocused (Variables|Default|GetPlayerChar))))
    (CallFunction|Fade false 0.5)
    (Variables|Default|SetStartedFade true)))

(event Collision|EventActorEndOverlap
  (params (OtherActor :type Actor%20Object%20Reference))
  (Utilities|Casting|CastToBP_PlayerCharacter OtherActor)
  (Variables|Default|SetPlayerChar 0)
  (if (< (- (Utilities|Time|GetTimeSeconds) (Variables|Default|GetTimer)) (Variables|Default|GetTimeTillTeleportation))
    (Development|PrintString "Leave under 2 Sec" true true "(R=0.000000,G=0.660000,B=1.000000,A=1.000000)" 4.0)
    (Variables|Default|SetTimer 0.0)
    (Variables|Default|SetActorOverlaps false)
    (if (Variables|Default|GetStartedFade)
      (CallFunction|Fade true 0.5)
      (Variables|Default|SetStartedFade false))))

(event EventTick
  (params (DeltaSeconds :type Float%20%28single-precision%29))
  (bind _returnvalue (Game|GetGameInstance))
  (bind _playerchar (Variables|Default|GetPlayerChar))
  (bind _asbp_game_instance (Utilities|Casting|CastToBP_GameInstance _returnvalue))
  (bind _playersavegame (Variables|/Game/VikingMageProject/Core/Characters/Player/BP_GameInstance.BP_GameInstance_C|GetPlayerSaveGame _asbp_game_instance))
  (Utilities|IsValid _playerchar
    (:Is%20Valid
      (if (and (and (Variables|Default|GetActorOverlaps) (or (Variables|Default|GetCanUseFocused) (not (Variables|/Game/VikingMageProject/Core/Characters/BP_CharacterCustom.BP_CharacterCustom_C|GetIsFocused _playerchar)))) (>= (- (Utilities|Time|GetTimeSeconds) (Variables|Default|GetTimer)) (Variables|Default|GetTimeTillTeleportation)))
        (Development|PrintString "Stayed 2 Sec")
        (Variables|Default|SetTimer 0.0)
        (Variables|Default|SetActorOverlaps false)
        (bind _asbp_player_character (Utilities|Casting|CastToBP_PlayerCharacter (Game|GetPlayerCharacter 0)))
        (Default|WriteDatatoGameInstance _asbp_player_character)
        (Variables|/Game/VikingMageProject/Core/Characters/Player/BP_GameInstance.BP_GameInstance_C|SetIsRespawning _asbp_game_instance true)
        (bind _output_get (Variables|/Game/VikingMageProject/Core/SaveData/BP_PlayerSaveGame.BP_PlayerSaveGame_C|SetSpawnInfo _playersavegame (Utilities|Struct|MakeSSpawnInfo (.level (Variables|Default|GetSpawnInfo)) (.destinationtag (Variables|Default|GetSpawnInfo)) (.playerstart (Variables|/Game/VikingMageProject/Core/SaveData/BP_PlayerSaveGame.BP_PlayerSaveGame_C|GetSpawnInfo _playersavegame)) (.spawnposition (Variables|/Game/VikingMageProject/Core/SaveData/BP_PlayerSaveGame.BP_PlayerSaveGame_C|GetSpawnInfo _playersavegame)) (.hasloadedgame (Variables|/Game/VikingMageProject/Core/SaveData/BP_PlayerSaveGame.BP_PlayerSaveGame_C|GetSpawnInfo _playersavegame)) (.movementspline (Variables|/Game/VikingMageProject/Core/SaveData/BP_PlayerSaveGame.BP_PlayerSaveGame_C|GetSpawnInfo _playersavegame)))))
        (Default|SaveCurrentLevel (.AsBP%20Game%20Instance (Utilities|Casting|CastToBP_GameInstance (Game|GetGameInstance))))
        (Default|Respawn (Variables|Default|GetPlayerChar))))))

(fn ConstructionScript)

(fn Fade
  (params (Fade%20In :type Boolean) (Speed :type Float%20%28single-precision%29))
  (bind _sequenzplayer (Variables|Default|GetSequenzPlayer))
  (if Fade%20In
    (Class|MovieSceneSequencePlayer|PlayReverse _sequenzplayer)
    (else
      (Sequencer|Player|Play _sequenzplayer :!class /Script/MovieScene.MovieSceneSequencePlayer)))
  (Default|FadePlayerUI (Variables|/Game/VikingMageProject/Core/Characters/Player/BP_PlayerCharacter.BP_PlayerCharacter_C|GetWBP_PlayerHUD (.AsBP%20Player%20Character (Utilities|Casting|CastToBP_PlayerCharacter (Game|GetPlayerCharacter 0)))) Fade%20In Speed))