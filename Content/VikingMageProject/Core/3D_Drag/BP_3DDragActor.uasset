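; Draggable physics puzzle piece that registers with a parent puzzle and reports whether it is correctly attached.
; While grabbed, Tick springs it toward the mouse ray's intersection with the drag plane, and Rotate turns it in steps.
; Attach3DComponent overlaps snap it onto fixed or attached pieces; pulling past DetachmentFriction frees single-connection pieces, and negative friction means fixed.
; A looping timer returns unattached, unrendered pieces to spawn.
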(event Custom|ColliderOverlap
  (params (OverlappedComponent :type Primitive%20Component%20Object%20Reference) (OtherActor :type Actor%20Object%20Reference) (OtherComp :type Primitive%20Component%20Object%20Reference) (OtherBodyIndex :type Integer) (bFromSweep :type Boolean) (SweepResult :type Hit%20Result%20Structure%20%28by%20ref%29))
  (CallFunction|CollisionReaction OverlappedComponent OtherComp OtherActor))

(event Custom|Grab
  (params (PlaneOrigin :type Vector) (PlaneNormal :type Vector) (Player :type Player%20Controller%20Object%20Reference))
  (bind _rotationstep (Variables|Options|GetRotationStep))
  (bind _staticmesh (Variables|Default|GetStaticMesh))
  (Variables|Default|SetPlaneOrigin PlaneOrigin)
  (Variables|Default|SetPlaneNormal PlaneNormal)
  (Variables|Default|SetDraggingPlayer Player)
  (Actor|Tick|SetActorTickEnabled true)
  (if (and (== (Variables|Default|GetAttachedPoints) 0) (> (Variables|Default|GetDetachmentFriction) 0.0))
    (Class|PrimitiveComponent|SetLinearDamping _staticmesh 7.0)
    (Class|PrimitiveComponent|SetAngularDamping _staticmesh 9.999999980506448e+18)
    (Class|PrimitiveComponent|SetPhysicsAngularVelocityinDegrees _staticmesh "0, 0, 0" false "None")
    (Utilities|FlowControl|Sequence
      (:then_0
        (Utilities|FlowControl|DoOnce false ; Initialize Rotation on first Grab
          (:Completed
            (Variables|Default|SetCurrentManualRotation (Math|Rotator|MakeRotator (* (Math|Random|RandomIntegerinRange 0 (Math|Float|Truncate (/ 3.6e+02 _rotationstep))) _rotationstep) 0.0 (.Yaw (Math|Rotator|BreakRotator (Math|Rotator|MakeRotfromX (Variables|Default|GetPlaneNormal)))))))))
      (:then_1
        (CallFunction|PlayRotateAnim)))))

(event Custom|ResetPos
  (bind _staticmesh (Variables|Default|GetStaticMesh))
  (bind _staticmesh_2 (Variables|Default|GetStaticMesh))
  (Development|PrintString (Utilities|String|Append (Utilities|GetDisplayName self) " Resetted") true true "(R=1.000000,G=0.021536,B=0.000000,A=1.000000)" 5e+01)
  (Variables|Default|SetCanNotSnap true)
  (Physics|SetSimulatePhysics _staticmesh false)
  (Collision|SetCollisionEnabled _staticmesh "NoCollision")
  (Class|VectorBlueprintLibrary|CustomMoveComponentto (Variables|Default|GetStaticMesh) (Variables|Default|GetSpawnPoint) true "0, 0, 0" false true false 0.5 false)
  (Physics|SetSimulatePhysics _staticmesh_2 true)
  (Collision|SetCollisionEnabled _staticmesh_2 "QueryAndPhysics")
  (Variables|Default|SetCanNotSnap false))

(event Custom|CheckReachable
  (if (not (CallFunction|IsAttached)) ; Never Respawn, when attached
    (if (not (Class|PrimitiveComponent|WasRecentlyRendered (Variables|Default|GetStaticMesh) 0.5))
      (CallFunction|ResetPos))))

(event Custom|PlayAttachAnim
  (params (OtherComponent :type Primitive%20Component%20Object%20Reference) (ThisComponent :type Primitive%20Component%20Object%20Reference))
  (bind _staticmesh (Variables|Default|GetStaticMesh))
  (bind _outrotation (Utilities|GetAttachRotation)
    (:%20
      (Class|VectorBlueprintLibrary|CustomMoveComponentto _staticmesh "0, 0, 0" false _outrotation true false false 0.2 true)
      (Class|VectorBlueprintLibrary|CustomMoveComponentto _staticmesh (CallFunction|CalcRelativeforWorldLocation _staticmesh (+ (Transformation|GetWorldLocation _staticmesh) (- (Transformation|GetWorldLocation OtherComponent) (Transformation|GetWorldLocation ThisComponent)))) true "0, 0, 0" false false false 0.2 false))))

(event Custom|DetachEvent
  (bind _staticmesh (Variables|Default|GetStaticMesh))
  (Utilities|FlowControl|Sequence
    (:then_0
      (Class|VectorBlueprintLibrary|CustomMoveComponentto _staticmesh "0, 0, 0" false (stale Custom|PlayAttachAnim _outrotation) true false false 0.2 true) ; enters at Stop
    )
    (:then_1
      (Class|VectorBlueprintLibrary|CustomMoveComponentto _staticmesh (CallFunction|CalcRelativeforWorldLocation _staticmesh (+ (Transformation|GetWorldLocation _staticmesh) (- (Transformation|GetWorldLocation (stale Custom|PlayAttachAnim OtherComponent)) (Transformation|GetWorldLocation (stale Custom|PlayAttachAnim ThisComponent))))) true "0, 0, 0" false false false 0.2 false) ; enters at Stop
    )))

(event Custom|PlayRotateAnim
  (Variables|Default|SetCanNotSnap true)
  (Class|VectorBlueprintLibrary|CustomMoveComponentto (Variables|Default|GetStaticMesh) "0, 0, 0" false (Variables|Default|GetCurrentManualRotation) true true false 0.2 true)
  (Variables|Default|SetCanNotSnap false))

(event EventBeginPlay
  (bind _parentpuzzle (Variables|Default|GetParentPuzzle))
  (bind _output (Utilities|ResolveSoftReference _parentpuzzle))
  (Utilities|IsValid _output
    (:Is%20Valid
      (Default|AddPuzzleActor _output self)
      (Variables|Default|SetSpawnPoint (Transformation|GetActorLocation))
      (Physics|SetSimulatePhysics (Variables|Default|GetStaticMesh) (>= (Variables|Default|GetDetachmentFriction) 0.0))
      (Utilities|Time|SetTimerbyEvent (delegate Custom|CheckReachable) 2.0 true)
      (for _array_element (Components|GetChildrenComponents (Variables|Default|GetStaticMesh) true)
        (bind _asattach_3dcomponent (Utilities|Casting|CastToAttach3DComponent _array_element))
        (Collision|AssignOnComponentBeginOverlap _asattach_3dcomponent (delegate Custom|ColliderOverlap))
        (Utilities|Array|Add (Variables|Default|GetColliders) _asattach_3dcomponent)))
    (:Is%20Not%20Valid
      (Class|VectorBlueprintLibrary|PrintStringErrorLog "No valid parent puzzle asigned."))))

(event EventTick
  (params (DeltaSeconds :type Float%20%28single-precision%29))
  (bind _draggingplayer (Variables|Default|GetDraggingPlayer))
  (bind _staticmesh (Variables|Default|GetStaticMesh))
  (bind _planenormal (Variables|Default|GetPlaneNormal))
  (bind _springstrength (Variables|Options|GetSpringStrength))
  (bind _tracedepth (Variables|Default|GetTraceDepth))
  (bind _planeorigin (Variables|Default|GetPlaneOrigin))
  (bind _returnvalue (Transformation|GetWorldLocation _staticmesh))
  (bind (_worldlocation _worlddirection) (Game|Player|ConvertMouseLocationToWorldSpace _draggingplayer))
  (bind _returnvalue_2 (* _worlddirection _tracedepth))
  (bind _returnvalue_3 (+ _worldlocation _returnvalue_2))
  (bind _intersection (Class|KismetMathLibrary|LinePlaneIntersectionOriginNormal _worldlocation _returnvalue_3 _planeorigin _planenormal))
  (bind _returnvalue_4 (- _intersection _returnvalue))
  (bind _returnvalue_5 (* _returnvalue_4 _springstrength))
  (switch int (Variables|Default|GetAttachedPoints)
    (:0
      (Physics|SetPhysicsLinearVelocity (Variables|Default|GetStaticMesh) (* _returnvalue_5 DeltaSeconds) true "None" :!label _label))
    (:1
      (bind (_detachable _attachedcollider) (CallFunction|CanActorDetach))
      (if _detachable
        (if (> (* (Math|Vector|VectorLength _returnvalue_5) (Utilities|CalcDetachStrengthFactor (Math|Vector|DotProduct (Math|Vector|Normalize _returnvalue_5) (Math|Vector|GetUpVector _attachedcollider)))) (Variables|Default|GetDetachmentFriction)) ; Overcome Friction, when attached
          (Actions|Detach)
          (goto _label))))))

(fn ConstructionScript)

(fn Attach
  (params (This :type Primitive%20Component%20Object%20Reference%20%28by%20ref%29) (Other :type Primitive%20Component%20Object%20Reference%20%28by%20ref%29) (OtherActor :type Actor%20Object%20Reference))
  (bind _asattach_3dcomponent (Utilities|Casting|CastToAttach3DComponent This))
  (LocalVariables|SetLocalThis _asattach_3dcomponent)
  (bind _asattach_3dcomponent_2 (Utilities|Casting|CastToAttach3DComponent Other))
  (LocalVariables|SetLocalOther _asattach_3dcomponent_2)
  (bind _asbp_3ddrag_actor (Utilities|Casting|CastToBP_3DDragActor OtherActor))
  (bind _output_get (LocalVariables|SetLocalOtherActor _asbp_3ddrag_actor))
  (if (or (> (Variables|BP_3DDragActor_C|GetAttachedPoints _output_get) 0) (< (Variables|BP_3DDragActor_C|GetDetachmentFriction _output_get) 0.0))
    ;[1 1 1] Do not attach to an Actor we are already attached to
    (if (not (Utilities|Array|ContainsItem (Variables|Default|GetAttachedActors) (LocalVariables|GetLocalOtherActor)))
      (bind _returnvalue (Class|Attach3DComponent|Attach (LocalVariables|GetLocalThis) (LocalVariables|GetLocalOther)))
      (if _returnvalue
        ;[1 0.1768 0] The Actual Attachment
        (Transformation|AttachComponentToComponent (Variables|Default|GetStaticMesh) (LocalVariables|GetLocalOther) "None" "KeepWorld" "KeepWorld" "KeepWorld" true)
        (CallFunction|ReevaluateAttachPoints)
        (CallFunction|ReevaluateAttachPoints (LocalVariables|GetLocalOtherActor))
        (CallFunction|PlayAttachAnim (LocalVariables|GetLocalOther) (LocalVariables|GetLocalThis))
        (Physics|SetSimulatePhysics (Variables|Default|GetStaticMesh) false)
        (Utilities|FlowControl|Sequence)))
    (else
      ;[1 1 1] Cannot attach to detached Actors
      (Development|PrintString "Not Attached")
      (return))))

(fn Detach
  (bind _staticmesh (Variables|Default|GetStaticMesh))
  (bind (_detachable _attachedcollider) (CallFunction|CanActorDetach))
  (if _detachable
    (bind _returnvalue (Class|Attach3DComponent|Detach _attachedcollider))
    (bind _asbp_3ddrag_actor (Utilities|Casting|CastToBP_3DDragActor _returnvalue)
      (:then
        (CallFunction|ReevaluateAttachPoints _asbp_3ddrag_actor))
      (:CastFailed
        _))
    (CallFunction|ReevaluateAttachPoints)
    ;[1 0.1768 0] The Actual Detachment
    (Transformation|AttachComponentToComponent _staticmesh (Variables|Default|GetDefaultSceneRoot) "None" "KeepWorld" "KeepWorld" "KeepWorld" true)
    (Physics|SetSimulatePhysics _staticmesh true)
    (Class|PrimitiveComponent|SetLinearDamping _staticmesh 7.0)
    (Class|PrimitiveComponent|SetAngularDamping _staticmesh 9.999999980506448e+18)
    (Class|PrimitiveComponent|SetPhysicsAngularVelocityinDegrees _staticmesh "0, 0, 0" false "None")
    (CallFunction|DetachEvent)))

(fn Drop
  (bind _staticmesh (Variables|Default|GetStaticMesh))
  (Variables|Default|SetDraggingPlayer 0)
  (Class|PrimitiveComponent|SetLinearDamping _staticmesh 0.1)
  (Class|PrimitiveComponent|SetAngularDamping _staticmesh 0.0)
  (Actor|Tick|SetActorTickEnabled false))

(fn Rotate
  (params (Steps :type Integer))
  (if (and (== (Variables|Default|GetAttachedPoints) 0) (>= (Variables|Default|GetDetachmentFriction) 0.0))
    (Variables|Default|SetCurrentManualRotation (Math|Rotator|CombineRotators (Variables|Default|GetCurrentManualRotation) (Math|Vector|RotatorfromAxisandAngle (Variables|Default|GetPlaneNormal) (* Steps (Variables|Options|GetRotationStep)))))
    (Class|PrimitiveComponent|SetPhysicsAngularVelocityinDegrees (Variables|Default|GetStaticMesh) "0, 0, 0" false "None")
    (CallFunction|PlayRotateAnim)))

(fn CalcRelativeforWorldLocation
  (params (Component :type Primitive%20Component%20Object%20Reference) (WorldLocation :type Vector))
  (LocalVariables|SetOldRelative (Variables|/Script/Engine.SceneComponent|GetRelativeLocation Component))
  (Transformation|SetWorldLocation Component WorldLocation false true)
  (LocalVariables|SetNewRelative (Variables|/Script/Engine.SceneComponent|GetRelativeLocation Component))
  (Transformation|SetRelativeLocation Component (LocalVariables|GetOldRelative) false true)
  (return (LocalVariables|GetNewRelative)))

(fn ReevaluateAttachPoints
  (Utilities|Array|Clear (Variables|Default|GetAttachedActors))
  (bind _colliders (Utilities|GetAttachedColliders)
    (:Out
      (for _array_element _colliders
        (bind _asbp_3ddrag_actor (Utilities|Casting|CastToBP_3DDragActor (Components|GetOwner (Variables|/Script/VikingMage.Attach3DComponent|GetAttachedTo _array_element))))
        (Utilities|Array|Add (Variables|Default|GetAttachedActors) _asbp_3ddrag_actor))
      (bind _output_get (Variables|Default|SetAttachedPoints (Utilities|Array|Length _colliders)))
      (Development|PrintString (Utilities|String|Append (Utilities|GetDisplayName self) " Attachments: " (Utilities|String|ToString(Integer) _output_get))))))

(fn CollisionReaction
  (params (OverlappedComponent :type Primitive%20Component%20Object%20Reference) (OtherComp :type Primitive%20Component%20Object%20Reference) (OtherActor :type Actor%20Object%20Reference))
  (if (not (Variables|Default|GetCanNotSnap))
    (if (Utilities|IsValid (Variables|Default|GetDraggingPlayer))
      (Actions|Attach OverlappedComponent OtherComp OtherActor))))

(fn CanActorDetach
  (if (> (Variables|Default|GetDetachmentFriction) 0.0)
    (bind _colliders (Utilities|GetAttachedColliders)
      (:Out
        (return (== (Utilities|Array|Length _colliders) 1) (Utilities|Array|Get(acopy) _colliders))))
    (else
      (Development|PrintString "Friction too high")
      (return false 0))))

(fn IsCorrectlyAttached
  (bind _staticmesh (Variables|Default|GetStaticMesh))
  (bind _rotationtolerance (LocalVariables|GetRotationTolerance))
  (bind _returnvalue (Transformation|GetWorldRotation _staticmesh))
  (if (< (Variables|Default|GetDetachmentFriction) 0.0)
    (return true) ; permanently attached Actors are considered correct
    (else
      (for _array_element (Variables|Default|GetColliders)
        (bind _returnvalue_2 (Class|Attach3DComponent|IsCorrectlyAttached _array_element))
        (Development|PrintString (Utilities|String|Append "Collider correct: " (Utilities|String|ToString(Boolean) _returnvalue_2)))
        (if (not _returnvalue_2)
          (return false)))
      (return (Math|Boolean|ANDBoolean (Math|Float|NearlyEqual(Float) (.roll _returnvalue) 0.0 _rotationtolerance) (Math|Float|NearlyEqual(Float) (.pitch _returnvalue) 0.0 _rotationtolerance) (Math|Float|NearlyEqual(Float) (.yaw _returnvalue) (.yaw (Math|Rotator|MakeRotfromX (Variables|Default|GetPlaneNormal))) _rotationtolerance))))))

(fn IsAttached
  (return (or (!= (Variables|Default|GetAttachedPoints) 0) (< (Variables|Default|GetDetachmentFriction) 0.0))))