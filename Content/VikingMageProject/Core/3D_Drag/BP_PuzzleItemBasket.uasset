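; A puzzle item basket Blueprint that turns an attached item ID into a spawned 3D actor.
; Attach runs the parent logic, then Drop looks up the actor class in DT_ItemID_To_3DClass using an "Item"+ID row name.
; Drop spawns it near SpawnPoint with a random offset and rotation, then registers it with PuzzlePawn when valid.
; SetHighlight simply defers to the parent.
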(fn ConstructionScript)

(fn Drop
  (params (ItemID :type Integer))
  (bind _returnvalue (Utilities|GetDataTableRow "/Game/VikingMageProject/Core/3D_Drag/DT_ItemID_To_3DClass.DT_ItemID_To_3DClass" (Utilities|String|StringToName (Utilities|String|Append "Item" (Utilities|String|ToString(Integer) ItemID))))
    (:then
      (bind _returnvalue_2 (Game|SpawnActorfromClass (.class _returnvalue) (Math|Transform|MakeTransform (+ (Transformation|GetWorldLocation (Variables|Default|GetSpawnPoint)) (* (Math|Random|RandomUnitVector) (Math|Random|RandomFloatinRange 0.0 2e+02))) (Math|Random|RandomRotator true) (Variables|Default|GetSpawn%20Scale)) "AdjustIfPossibleButAlwaysSpawn" 0 0))
      (bind _puzzlepawn (Variables|Default|GetPuzzlePawn)
        (:then
          (Default|AddPuzzleActor _puzzlepawn _returnvalue_2))
        (:else)))))

(fn SetHighlight
  (params (Highlight :type EAttachHighlight%20Enum :default "NewEnumerator0"))
  (|CallParentFunction Highlight))

(fn Attach
  (params (ItemID :type Integer))
  (|CallParentFunction ItemID)
  (CallFunction|Drop ItemID))