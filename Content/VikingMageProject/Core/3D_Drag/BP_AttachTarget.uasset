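; BP_AttachTarget is a drop target for the 3D drag system that accepts items by ID and previews where they can attach.
; CanAttach rejects already dropped items and treats the list as a whitelist, or as a blacklist when AcceptAll is set.
; SetHighlight tints a hologram mesh through custom primitive data, falling back to custom-depth stencil outlines when no hologram mesh is set.
; Attach records the item and reveals the attached mesh.
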(fn ConstructionScript)

(fn CanAttach
  (params (ItemID :type Integer))
  (bind _droppeditems (Variables|Default|GetDroppedItems))
  (bind _returnvalue (Utilities|Array|ContainsItem _droppeditems ItemID))
  (bind _returnvalue_2 (not _returnvalue))
  (if (Variables|Default|GetAcceptAll)
    (return (and (not (Utilities|Array|ContainsItem (Variables|Default|GetList) ItemID)) _returnvalue_2))
    (else
      (return (and _returnvalue_2 (Utilities|Array|ContainsItem (Variables|Default|GetList) ItemID))))))

(fn SetHighlight
  (params (Highlight :type EAttachHighlight%20Enum :default "NewEnumerator0"))
  (bind _staticmesh (Variables|Default|GetStaticMesh))
  (if (Utilities|IsValid (Variables|/Script/Engine.StaticMeshComponent|GetStaticMesh (Variables|Default|GetHoloObjectMesh)))
    (if (not (Variables|/Script/Engine.SceneComponent|GetbVisible (Variables|Default|GetAttachedObjectMesh)))
      (switch Utilities|FlowControl|Switch|SwitchonEAttachHighlight Highlight
        (:NewEnumerator0
          (Rendering|SetVisibility (Variables|Default|GetHoloObjectMesh) false true)
          (Development|PrintString "Should be hidden"))
        (:NewEnumerator1
          (Rendering|SetVisibility (Variables|Default|GetHoloObjectMesh) true true)
          (Rendering|Material|SetCustomPrimitiveDataVector4 (Variables|Default|GetHoloObjectMesh) 0 (Variables|Default|GetDefaultHoloColor)))
        (:NewEnumerator2
          (Rendering|SetVisibility (Variables|Default|GetHoloObjectMesh) true true)
          (Rendering|Material|SetCustomPrimitiveDataVector4 (Variables|Default|GetHoloObjectMesh) 0 (Variables|Default|GetHoverHoloColor)))))
    (else
      (switch Utilities|FlowControl|Switch|SwitchonEAttachHighlight Highlight
        (:NewEnumerator0
          ;[1 1 1] Outline
          (Rendering|SetRenderCustomDepth _staticmesh false))
        (:NewEnumerator1
          (Rendering|SetRenderCustomDepth _staticmesh true)
          (Rendering|SetCustomDepthStencilValue _staticmesh (Variables|Default|GetPossibleOutlineType)))
        (:NewEnumerator2
          (Rendering|SetRenderCustomDepth _staticmesh true)
          (Rendering|SetCustomDepthStencilValue _staticmesh (Variables|Default|GetHoveredOutlineType)))))))

(fn Attach
  (params (ItemID :type Integer))
  (Utilities|Array|Add (Variables|Default|GetDroppedItems) ItemID)
  (Rendering|SetVisibility (Variables|Default|GetAttachedObjectMesh) true false))