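; Player save game that records per-level world state, such as destroyed, moved and instanced actors, NPCs, attachables, doors and interaction markers.
; LevelDataMap maps each level name to a BP_LevelSaveData object, where save functions store state keyed by actor, or transforms grouped by class for instanced actors.
; Only the destroyed and instanced saves create missing level data through CheckLevelDataMap; the others assume the entry exists.
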(fn SaveDestroyedActor
  (params (DestroyedActor :type Actor%20Object%20Reference) (LevelName :type String))
  (CallFunction|CheckLevelDataMap LevelName)
  (Utilities|Array|AddUnique (Variables|/Game/VikingMageProject/Core/SaveData/BP_LevelSaveData.BP_LevelSaveData_C|GetDestroyedActors (.Value (Utilities|Map|Find (Variables|Default|GetLevelDataMap) LevelName))) (Utilities|ResolveSoftReference DestroyedActor)))

(fn CheckLevelDataMap
  (params (LevelName :type String))
  (if (not (Utilities|Map|Contains (Variables|Default|GetLevelDataMap) LevelName))
    ;[1 1 1] Add new LevelData if not exists
    (bind _returnvalue (Game|ConstructObjectfromClass "/Game/VikingMageProject/Core/SaveData/BP_LevelSaveData.BP_LevelSaveData_C" self))
    (Utilities|Map|Add (Variables|Default|GetLevelDataMap) LevelName _returnvalue)))

(fn SaveMovableActor
  (params (MovableActor :type Actor%20Object%20Reference) (LevelName :type String))
  (Utilities|Map|Add (Variables|/Game/VikingMageProject/Core/SaveData/BP_LevelSaveData.BP_LevelSaveData_C|GetMovableActors (.Value (Utilities|Map|Find (Variables|Default|GetLevelDataMap) LevelName))) (Utilities|ResolveSoftReference MovableActor) (Transformation|GetActorTransform MovableActor)))

(fn SaveInstancedActor
  (params (InstancedActor :type Actor%20Object%20Reference) (LevelName :type String))
  (bind _returnvalue (Utilities|GetClass InstancedActor))
  (bind _leveldatamap (Variables|Default|GetLevelDataMap))
  (bind _value (Utilities|Map|Find _leveldatamap LevelName))
  (bind _instancedactors (Variables|/Game/VikingMageProject/Core/SaveData/BP_LevelSaveData.BP_LevelSaveData_C|GetInstancedActors _value))
  (bind (_value_2 _returnvalue_2) (Utilities|Map|Find _instancedactors _returnvalue))
  (CallFunction|CheckLevelDataMap LevelName)
  (if _returnvalue_2
    (Utilities|Array|Add (Utilities|Struct|BreakS_InstancedObjectInfo _value_2) (Transformation|GetActorTransform InstancedActor))
    (else
      (Utilities|Map|Add _instancedactors _returnvalue (Utilities|Struct|MakeS_InstancedObjectInfo (Utilities|Array|MakeArray (Transformation|GetActorTransform InstancedActor)))))))

(fn SaveNPC
  (params (NPC :type BP%20NPC%20Object%20Reference) (LevelName :type String))
  (bind _bp_npcstats (Variables|/Game/VikingMageProject/Core/Characters/NPC/BP_NPC.BP_NPC_C|GetBP_NPCStats NPC))
  (Utilities|Map|Add (Variables|/Game/VikingMageProject/Core/SaveData/BP_LevelSaveData.BP_LevelSaveData_C|GetNPCs (.Value (Utilities|Map|Find (Variables|Default|GetLevelDataMap) LevelName))) (Utilities|ResolveSoftReference NPC) (Utilities|Struct|MakeS_NPCSaveStats (Variables|/Game/VikingMageProject/Core/Characters/NPC/BP_NPCStats.BP_NPCStats_C|GetcurrHealth _bp_npcstats) (Variables|/Game/VikingMageProject/Core/Characters/NPC/BP_NPCStats.BP_NPCStats_C|GetmaxHealth _bp_npcstats) (Variables|/Game/VikingMageProject/Core/Characters/NPC/BP_NPCStats.BP_NPCStats_C|GetisDead _bp_npcstats) (Variables|/Game/VikingMageProject/Core/Characters/NPC/BP_NPC.BP_NPC_C|GetIsArmed NPC))))

(fn SaveAttachable
  (params (AttachTarget :type BP%20Attach%20Target%20Object%20Reference) (LevelName :type String))
  (Utilities|Map|Add (Variables|/Game/VikingMageProject/Core/SaveData/BP_LevelSaveData.BP_LevelSaveData_C|GetAttachables (.Value (Utilities|Map|Find (Variables|Default|GetLevelDataMap) LevelName))) (Utilities|ResolveSoftReference AttachTarget) (Utilities|Struct|MakeS_AttachablesStats (Variables|/Script/Engine.SceneComponent|GetbVisible (Variables|/Game/VikingMageProject/Core/3D_Drag/BP_AttachTarget.BP_AttachTarget_C|GetAttachedObjectMesh AttachTarget)))))

(fn SaveDownslideDoor
  (params (DownslideDoor :type BP%20Downslide%20Door%20Object%20Reference) (LevelName :type String))
  (Utilities|Map|Add (Variables|/Game/VikingMageProject/Core/SaveData/BP_LevelSaveData.BP_LevelSaveData_C|GetDownslideDoors (.Value (Utilities|Map|Find (Variables|Default|GetLevelDataMap) LevelName))) (Utilities|ResolveSoftReference DownslideDoor) (Utilities|Struct|MakeS_DownslideDoorsStats (Variables|/Game/VikingMageProject/Placeables/BP_DownslideDoor.BP_DownslideDoor_C|GetIsDone DownslideDoor))))

(fn SaveInteractionMarker
  (params (InteractionMarker :type BP%20Interaction%20Marker%20Object%20Reference) (LevelName :type String))
  (Utilities|Map|Add (Variables|/Game/VikingMageProject/Core/SaveData/BP_LevelSaveData.BP_LevelSaveData_C|GetInteractionMarker (.Value (Utilities|Map|Find (Variables|Default|GetLevelDataMap) LevelName))) (Utilities|ResolveSoftReference InteractionMarker) (Utilities|Struct|MakeS_InteractionMarkerInfo (Variables|/Game/VikingMageProject/Core/Interaction/BP_InteractionMarker.BP_InteractionMarker_C|GetIsActive InteractionMarker) (Variables|/Game/VikingMageProject/Core/Interaction/BP_InteractionMarker.BP_InteractionMarker_C|GetAutoInteract InteractionMarker) (Variables|/Game/VikingMageProject/Core/Interaction/BP_InteractionMarker.BP_InteractionMarker_C|GetAutoInteractOnlyOnce InteractionMarker) (Variables|/Script/Engine.Actor|GetbAutoDestroyWhenFinished InteractionMarker))))