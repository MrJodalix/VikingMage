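; BP_Trigger_Sphere is a trigger actor, spherical by its name, that relays overlaps to event actors attached to it.
; On BeginPlay it gathers its attached actors that cast to BP_TriggerEvent into EventInstances.
; Actor begin and end overlaps call Enter and Exit on each stored event, passing the other actor without filtering.
; Attachment serves as the wiring, so the trigger holds no response logic of its own.
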(event Collision|EventActorEndOverlap
  (params (OtherActor :type Actor%20Object%20Reference))
  (for _array_element (Variables|Default|GetEventInstances)
    (Default|Exit _array_element OtherActor)))

(event Collision|EventActorBeginOverlap
  (params (OtherActor :type Actor%20Object%20Reference))
  (for _array_element (Variables|Default|GetEventInstances)
    (Default|Enter _array_element OtherActor)))

(event EventBeginPlay
  (for _array_element (Actor|GetAttachedActors true)
    (bind _asbp_trigger_event (Utilities|Casting|CastToBP_TriggerEvent _array_element))
    (Utilities|Array|Add (Variables|Default|GetEventInstances) _asbp_trigger_event)))

(fn ConstructionScript)