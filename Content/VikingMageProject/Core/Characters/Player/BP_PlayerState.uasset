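; Player state for the Viking mage that holds and updates health, mana, experience, level and level-up points.
; While alive, Tick regenerates health (passively only below a threshold) and mana, adding queued over-time amounts from healing and mana finishers.
; Passive regen switches to a faster rate after the player character stays unfocused for a delay; focusing resets this.
; A visual experience value climbs toward actual experience to animate gains.
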(event EventBeginPlay
  (Variables|Stats|Exp|SetexpCurrVisual (Variables|Stats|Exp|Getexperience)))

(event EventTick
  (params (DeltaSeconds :type Float%20%28single-precision%29))
  (CallFunction|VisualizeExpGain DeltaSeconds)
  (if (not (Variables|Stats|Health|GetIsDead))
    (CallFunction|UpdateSpeedupTime DeltaSeconds)
    (Stats|Health|RegainHealth DeltaSeconds)
    (Stats|Mana|RegainMana DeltaSeconds)))

(fn ConstructionScript)

(fn IncPlayerHealth
  (params (amount :type Float%20%28single-precision%29))
  (Variables|Stats|Health|SetcurrHealth (Math|Float|Max(Float) (Math|Float|Min(Float) (+ amount (Variables|Stats|Health|GetcurrHealth)) (Variables|Stats|Health|GetmaxHealth)) 0.0)))

(fn DecPlayerHealth
  (params (Amount :type Float%20%28single-precision%29))
  (bind _output_get (Variables|Stats|Health|SetcurrHealth (Math|Float|Min(Float) (Math|Float|Max(Float) (- (Variables|Stats|Health|GetcurrHealth) Amount) 0.0) (Variables|Stats|Health|GetmaxHealth))))
  (return _output_get))

(fn IncPlayerMana
  (params (amount :type Float%20%28single-precision%29))
  (Variables|Stats|Mana|SetcurrMana (Math|Float|Min(Float) (+ amount (Variables|Stats|Mana|GetcurrMana)) (Variables|Stats|Mana|GetmaxMana))))

(fn DecPlayerMana
  (params (amount :type Float%20%28single-precision%29))
  (Variables|Stats|Mana|SetcurrMana (Math|Float|Max(Float) (- (Variables|Stats|Mana|GetcurrMana) amount) 0.0)))

(fn VisualizeExpGain
  (params (deltaSeconds :type Float%20%28single-precision%29))
  (if (< (Variables|Stats|Exp|GetexpCurrVisual) (Variables|Stats|Exp|Getexperience))
    (Variables|Stats|Exp|SetexpCurrVisual (+ (* deltaSeconds (Variables|Stats|Exp|GetexpVisualSpeed)) (Variables|Stats|Exp|GetexpCurrVisual)))
    (else
      (Variables|Stats|Exp|SetexpCurrVisual (Variables|Stats|Exp|Getexperience)))))

(fn AddExperience
  (params (addedExp :type Float%20%28single-precision%29))
  (bind _output_get (Variables|Stats|Exp|Setexperience (+ addedExp (Variables|Stats|Exp|Getexperience))))
  (Development|PrintString (Utilities|String|ToString(Float) _output_get)))

(fn RegainMana
  (params (DeltaSeconds :type Float%20%28single-precision%29))
  (Utilities|FlowControl|Sequence
    (:then_0
      ;[1 1 1] Passive Regeneration
      (if (<= (Variables|Stats|Mana|GetcurrMana) (Variables|Stats|Mana|GetmaxMana))
        (if (Variables|Stats|Mana|GetManaSpeedUpRegain)
          (LocalVariables|SetManaAmount (* (/ (Variables|Stats|Mana|GetmaxMana) (Variables|Stats|Mana|GetManaSpeedUpTime)) DeltaSeconds))
          (else
            (LocalVariables|SetManaAmount (* (Variables|Stats|Mana|GetBasePassiveManaRegen) DeltaSeconds))))))
    (:then_1
      ;[1 1 1] Finisher Regeneration
      (if (> (Variables|Stats|Mana|OverTime|GetManaToAddOverTime) 0.0)
        (LocalVariables|SetRestManaToAdd (Math|Float|Max(Float) (- (Variables|Stats|Mana|OverTime|GetManaToAddOverTime) (* (Variables|Stats|Mana|OverTime|GetManaAddSpeed) DeltaSeconds)) 0.0))
        (LocalVariables|SetFinisherAmount (- (Variables|Stats|Mana|OverTime|GetManaToAddOverTime) (LocalVariables|GetRestManaToAdd)))
        (Variables|Stats|Mana|OverTime|SetManaToAddOverTime (LocalVariables|GetRestManaToAdd))))
    (:then_2
      (Stats|Mana|IncPlayerMana (+ (LocalVariables|GetManaAmount) (LocalVariables|GetFinisherAmount))))))

(fn RegainHealth
  (params (DeltaSeconds :type Float%20%28single-precision%29))
  (Utilities|FlowControl|Sequence
    (:then_0
      ;[1 1 1] Passive Regeneration
      (if (< (Variables|Stats|Health|GetcurrHealth) (Math|Conversions|ToFloat(Integer) (Math|Float|Floor (* (Variables|Stats|Health|GetmaxHealth) (Variables|Stats|Health|GetHealthRegenThreshold)))))
        (if (Variables|Stats|Health|GetHealthSpeedUpRegain)
          (LocalVariables|SetHealAmount (* (/ (Variables|Stats|Health|GetmaxHealth) (Variables|Stats|Health|GetHealthSpeedUpTime)) DeltaSeconds))
          (else
            (LocalVariables|SetHealAmount (* (Variables|Stats|Health|GetBasePassivHealthRegen) DeltaSeconds))))))
    (:then_1
      ;[1 1 1] Finisher Regeneration
      (if (> (Variables|Stats|Health|OverTime|GetHealthToAddOverTime) 0.0)
        (LocalVariables|SetRestHealthToAdd (Math|Float|Max(Float) (- (Variables|Stats|Health|OverTime|GetHealthToAddOverTime) (* (Variables|Stats|Health|OverTime|GetHealthAddSpeed) DeltaSeconds)) 0.0))
        (LocalVariables|SetFinisherAmount (- (Variables|Stats|Health|OverTime|GetHealthToAddOverTime) (LocalVariables|GetRestHealthToAdd)))
        (Variables|Stats|Health|OverTime|SetHealthToAddOverTime (LocalVariables|GetRestHealthToAdd))))
    (:then_2
      (Stats|Health|IncPlayerHealth (+ (LocalVariables|GetHealAmount) (LocalVariables|GetFinisherAmount))))))

(fn UpdateSpeedupTime
  (params (DeltaTime :type Float%20%28single-precision%29))
  (bind _asbp_player_character (Utilities|Casting|CastToBP_PlayerCharacter (Game|GetPlayerCharacter 0)))
  (if (not (Variables|/Game/VikingMageProject/Core/Characters/BP_CharacterCustom.BP_CharacterCustom_C|GetIsFocused _asbp_player_character))
    (Utilities|FlowControl|Sequence
      (:then_0
        ;[1 1 1] Health Speedup Counter
        (if (< (Variables|Stats|Health|GetHealthSpeedUpCount) (Variables|Stats|Health|GetHealthSpeedUpRegainDelay))
          (Variables|Stats|Health|SetHealthSpeedUpCount (+ (Variables|Stats|Health|GetHealthSpeedUpCount) DeltaTime))
          (else
            (Variables|Stats|Health|SetHealthSpeedUpRegain true))))
      (:then_1
        ;[1 1 1] Mana Speedup Counter
        (if (< (Variables|Stats|Mana|GetManaSpeedUpCount) (Variables|Stats|Mana|GetManaSpeedUpRegainDelay))
          (Variables|Stats|Mana|SetManaSpeedUpCount (+ (Variables|Stats|Mana|GetManaSpeedUpCount) DeltaTime))
          (else
            (Variables|Stats|Mana|SetManaSpeedUpRegain true)))))
    (else
      (Variables|Stats|Health|SetHealthSpeedUpCount 0.0)
      (Variables|Stats|Health|SetHealthSpeedUpRegain false)
      (Variables|Stats|Mana|SetManaSpeedUpCount 0.0)
      (Variables|Stats|Mana|SetManaSpeedUpRegain false))))

(fn AddFinisherMana
  (params (InstantAmount :type Float%20%28single-precision%29) (OverTimeAmount :type Float%20%28single-precision%29))
  ;[1 1 1] Instant Mana Boost
  (Stats|Mana|IncPlayerMana InstantAmount)
  ;[1 1 1] Over Time Mana Boost
  (Variables|Stats|Mana|OverTime|SetManaToAddOverTime (+ (Variables|Stats|Mana|OverTime|GetManaToAddOverTime) OverTimeAmount)))

(fn AddHealing
  (params (InstantAmount :type Float%20%28single-precision%29) (OverTimeAmount :type Float%20%28single-precision%29))
  ;[1 1 1] Instant Heal
  (Stats|Health|IncPlayerHealth InstantAmount)
  ;[1 1 1] Over Time Heal
  (Variables|Stats|Health|OverTime|SetHealthToAddOverTime (+ (Variables|Stats|Health|OverTime|GetHealthToAddOverTime) OverTimeAmount)))

(fn AddLevel
  (Math|Integer|IncrementInt (Variables|Stats|Getlevel)
    (:%20%20
      (Variables|Stats|SetLevelUpPoints (+ (Variables|Stats|GetLevelUpPoints) 2)))))