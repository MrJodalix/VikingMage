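; Fireball spell for the player that overrides CastSpell to launch a damaging projectile toward the aim target.
; After the parent cast logic, it spawns the spell actor through the player character, slightly ahead of the capsule and rotated along the aim direction.
; The projectile is initialized with base damage and gets the cast sound attached, faded in from partway through the clip.
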(fn CastSpell
  (params (playerState :type BP%20Player%20State%20Object%20Reference) (playerChar :type BP%20Player%20Character%20Object%20Reference))
  (bind _capsulecomponent (Variables|/Script/Engine.Character|GetCapsuleComponent playerChar))
  (bind _returnvalue (Transformation|GetWorldLocation _capsulecomponent))
  (|CallParentFunction playerState playerChar)
  (bind _directiontotarget (Default|GetDirectiontoAimTarget playerChar _returnvalue))
  (bind _newactor (Default|CharacterSpawnActor playerChar (Variables|Default|GetspellActor) (+ _returnvalue (* (Math|Vector|Normalize _directiontotarget) 5e+01)) (Math|Rotator|FindLookatRotation _returnvalue (+ _returnvalue (* (Math|Vector|Normalize _directiontotarget) 5e+01))) (Variables|Default|GetactorScale)))
  (bind _asbp_4e_base_projectile_alt (Utilities|Casting|CastToBP_4E_Base_ProjectileAlt _newactor))
  (Default|Initialize _asbp_4e_base_projectile_alt (Variables|Default|GetbaseDmg))
  (Development|PrintString 0 "Cast Fireball")
  (bind _returnvalue_2 (Audio|SpawnSoundAttached (Variables|Default|GetCastSound) (Variables|/Script/Engine.Actor|GetRootComponent _asbp_4e_base_projectile_alt) "None" "0, 0, 0" "0, 0, 0" "KeepRelativeOffset" true 1.0 1.0 0.0 0 0))
  (Audio|Components|Audio|FadeIn _returnvalue_2 0.2 1.0 0.9 "Linear" :!class /Script/Engine.AudioComponent))