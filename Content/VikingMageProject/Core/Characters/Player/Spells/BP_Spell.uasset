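; BP_Spell is a base spell Blueprint for the player character's spellcasting.
; CanCastSpell allows a cast only when current mana covers ManaCost and CooldownTimeLeft has run out.
; CastSpell deducts the mana cost through the player state and restarts the cooldown timer at CooldownTime.
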(fn CanCastSpell
  (params (currentMana :type Float%20%28single-precision%29))
  (return (and (>= currentMana (Variables|Default|GetmanaCost)) (<= (Variables|Default|GetcooldownTimeLeft) 0.0))))

(fn CastSpell
  (params (playerState :type BP%20Player%20State%20Object%20Reference) (playerChar :type BP%20Player%20Character%20Object%20Reference))
  (Default|DecPlayerMana playerState (Variables|Default|GetmanaCost))
  (Variables|Default|SetcooldownTimeLeft (Variables|Default|GetcooldownTime)))