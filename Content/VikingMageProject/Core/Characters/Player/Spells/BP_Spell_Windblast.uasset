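; Windblast spell that blasts physics objects and actors in a cone along the player's aim.
; A multi-sphere trace sized from field of effect and range gathers hits, which are filtered by angle and distance from the player.
; A power-curve distance falloff scales impulses on simulating components, damage and the NPC windblast reaction.
; If the caster is falling, the spell also launches them opposite the aim direction.
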(fn CastSpell
  (params (playerState :type BP%20Player%20State%20Object%20Reference) (playerChar :type BP%20Player%20Character%20Object%20Reference))
  (|CallParentFunction playerState playerChar)
  (bind _returnvalue (Audio|SpawnSoundAttached (Variables|Default|GetCastSound) (Variables|/Script/Engine.Actor|GetRootComponent playerChar) "None" "0, 0, 0" "0, 0, 0" "KeepRelativeOffset" false 1.0 1.0 0.0 0 0))
  (Audio|Components|Audio|FadeIn _returnvalue 0.0 1.0 0.0 "Linear" :!class /Script/Engine.AudioComponent)
  (bind (_outhits _resultlookdirection) (CallFunction|GetEffectedActors playerChar))
  (CallFunction|ApplyEffectsonActors _outhits playerChar _resultlookdirection)
  (CallFunction|ApplyPushBack playerChar _resultlookdirection)
  (Development|PrintString 0 "Cast Windblast"))

(fn GetEffectedActors
  (params (playerChar :type BP%20Player%20Character%20Object%20Reference))
  (LocalVariables|SetplayerLocation (Transformation|GetWorldLocation (Variables|/Script/Engine.Character|GetCapsuleComponent playerChar)))
  (bind _directiontotarget (Default|GetDirectiontoAimTarget playerChar (LocalVariables|GetplayerLocation)))
  (LocalVariables|SetlookDirection (Math|Vector|Normalize _directiontotarget))
  (bind _radius (CallFunction|CalcSphereCastRadius (LocalVariables|GetlookDirection) (LocalVariables|GetplayerLocation) playerChar))
  (bind _outhits (CallFunction|CastMultiSphereTracefromActor playerChar _radius (LocalVariables|GetlookDirection) "TraceTypeQuery5"))
  (bind _output_get (LocalVariables|SetresultHits _outhits))
  (for (_array_element _array_index) _output_get
    (Utilities|Array|SetArrayElem (LocalVariables|GetresultHits) _array_index (Collision|MakeHitResult (.bBlockingHit (Collision|BreakHitResult _array_element)) (.bInitialOverlap (Collision|BreakHitResult _array_element)) (.Time (Collision|BreakHitResult _array_element)) (Math|Vector|VectorLength (- (.ImpactPoint (Collision|BreakHitResult _array_element)) (LocalVariables|GetplayerLocation))) (.Location (Collision|BreakHitResult _array_element)) (.ImpactPoint (Collision|BreakHitResult _array_element)) (.Normal (Collision|BreakHitResult _array_element)) (.ImpactNormal (Collision|BreakHitResult _array_element)) (.PhysMat (Collision|BreakHitResult _array_element)) (.HitActor (Collision|BreakHitResult _array_element)) (.HitComponent (Collision|BreakHitResult _array_element)) (.HitBoneName (Collision|BreakHitResult _array_element)) (.HitItem (Collision|BreakHitResult _array_element)) (.FaceIndex (Collision|BreakHitResult _array_element)) (.TraceStart (Collision|BreakHitResult _array_element)) (.TraceEnd (Collision|BreakHitResult _array_element)))))
  (return (LocalVariables|GetresultHits) (LocalVariables|GetlookDirection)))

(fn CalcSphereCastRadius
  (params (lookDirection :type Vector) (startPosition :type Vector) (playerChar :type BP%20Player%20Character%20Object%20Reference))
  (bind _returnvalue (Transformation|GetActorRightVector playerChar))
  (bind _fieldofeffect (Variables|Default|GetfieldOfEffect))
  (bind _returnvalue_2 (Math|Vector|CrossProduct lookDirection _returnvalue))
  (bind _returnvalue_3 (/ _fieldofeffect 2.0))
  (Variables|Default|Setgamma (- 9e+01 _returnvalue_3))
  (bind _output_get (Variables|Default|SetsiteLength (* (Variables|Default|GetmaxDist) (/ 1.0 (Math|Trig|Sin(Degrees) (Variables|Default|Getgamma))))))
  (Default|DrawDebugSpherefromChar playerChar (+ startPosition (* (Math|Vector|RotateVectorAroundAxis lookDirection (* -1 _returnvalue_3) _returnvalue_2) _output_get)) "(R=0.101961,G=1.000000,B=0.113725,A=1.000000)" 5.0)
  (Default|DrawDebugSpherefromChar playerChar (+ startPosition (* (Math|Vector|RotateVectorAroundAxis lookDirection _returnvalue_3 _returnvalue_2) _output_get)) "(R=0.101961,G=1.000000,B=0.113725,A=1.000000)" 5.0)
  (return (/ (Math|Vector|VectorLength (- (+ startPosition (* (Math|Vector|RotateVectorAroundAxis lookDirection (* -1 _returnvalue_3) _returnvalue_2) _output_get)) (+ startPosition (* (Math|Vector|RotateVectorAroundAxis lookDirection _returnvalue_3 _returnvalue_2) _output_get)))) 2.0)))

(fn CastMultiSphereTracefromActor
  (params (playerChar :type BP%20Player%20Character%20Object%20Reference) (radius :type Float%20%28single-precision%29) (lookDirection :type Vector) (TraceChannel :type ETraceTypeQuery%20Enum :default "TraceTypeQuery1"))
  (bind _capsulecomponent (Variables|/Script/Engine.Character|GetCapsuleComponent playerChar))
  (bind _returnvalue (Transformation|GetWorldLocation _capsulecomponent))
  (bind (_outhits _hashit) (Default|CharacterMultiSphereTrace playerChar _returnvalue (+ _returnvalue (* lookDirection (Variables|Default|GetmaxDist))) radius TraceChannel))
  (return _outhits _hashit))

(fn ApplyEffectsonActors
  (params (hitResults :type Array%20of%20Hit%20Result%20Structures) (playerChar :type BP%20Player%20Character%20Object%20Reference) (lookDirection :type Vector))
  (LocalVariables|SetplayerLocation (Transformation|GetWorldLocation (Variables|/Script/Engine.Character|GetCapsuleComponent playerChar)))
  (for _array_element hitResults
    (bind _output_get (LocalVariables|SetdirToObject (- (.impactpoint _array_element) (LocalVariables|GetplayerLocation))))
    (bind _result (CallFunction|IsEffected lookDirection _output_get (.distance _array_element)))
    (if _result
      (Utilities|FlowControl|Sequence
        (:then_0
          (bind _distmodifier (CallFunction|CalcDistModifier (.distance _array_element)))
          ;[1 1 1] Physik-Effekte hinzufügen
          (Variables|Default|SetDist%20Modifier _distmodifier)
          (if (Physics|IsSimulatingPhysics (.hitcomponent _array_element) (.hitbonename _array_element))
            (Physics|AddImpulse (.hitcomponent _array_element) (* (* (.normal _array_element) -1.0) (* (Variables|Default|GetDist%20Modifier) (Variables|Default|GetimpulseStrength))) (.hitbonename _array_element) false)))
        (:then_1
          (Game|Damage|ApplyDamage (.hitactor _array_element) (* (Variables|Default|GetbaseDmg) (Variables|Default|GetDist%20Modifier)) (Pawn|GetController playerChar) 0 "/Game/VikingMageProject/Core/Characters/Player/Spells/BP_WindBlastDamage.BP_WindBlastDamage_C")
          (bind _asbp_npc (Utilities|Casting|CastToBP_NPC (.hitactor _array_element)))
          (Default|ReacttoWindblast _asbp_npc 0.3 (* (* (.normal _array_element) -1.0) (* (Variables|Default|GetDist%20Modifier) (Variables|Default|GetimpulseStrength))) (Variables|Default|GetDist%20Modifier)))))))

(fn CalcDistModifier
  (params (dist :type Float%20%28single-precision%29))
  (return (+ (* (Math|Float|Power (/ dist (Variables|Default|GetmaxDist)) 1.25) -1.0) 1.0)))

(fn IsEffected
  (params (lookDirection :type Vector) (directionToObject :type Vector) (distToObject :type Float%20%28single-precision%29))
  (bind _returnvalue (Class|VectorBlueprintLibrary|CalcAngleBetweenVectors lookDirection directionToObject))
  (LocalVariables|SetangleBetweenLookAndObj _returnvalue)
  (return (and (and (> (Math|Vector|DotProduct lookDirection directionToObject) 0.0) (<= distToObject (Variables|Default|GetmaxDist))) (< (LocalVariables|GetangleBetweenLookAndObj) (/ (Variables|Default|GetfieldOfEffect) 2.0)))))

(fn ApplyPushBack
  (params (playerChar :type BP%20Player%20Character%20Object%20Reference) (lookDirection :type Vector))
  (bind _returnvalue (* lookDirection -1.0))
  (bind (_x _y _z) (Math|Vector|BreakVector _returnvalue))
  (if (AI|Components|NavMovement|IsFalling (Variables|/Script/Engine.Character|GetCharacterMovement playerChar))
    (Character|LaunchCharacter playerChar (Math|Vector|MakeVector (* _x (Variables|Repulsion|GetpushBackStrengthXY)) (* _y (Variables|Repulsion|GetpushBackStrengthXY)) (* _z (Variables|Repulsion|GetpushBackStrengthZ))) (Variables|Repulsion|GetoverrideXY) (Variables|Repulsion|GetoverrideZ))))