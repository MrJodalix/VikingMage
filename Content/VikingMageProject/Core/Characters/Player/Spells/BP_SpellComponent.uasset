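; Player spell component that holds the spell inventory, tracks the selected slot and casts the current spell.
; StarterSpells classes are instantiated into SpellInventory objects, all rebuilt on each slot swap or removal.
; Casting checks mana, cooldown and player state unless the SpellOverload cheat is set, then plays the attack montage and delegates to the spell object.
; Tick counts down cooldowns, and the component pushes cooldowns, icons and selection to the player HUD.
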(event EventBeginPlay
  (CallFunction|UpdateSpellInventory))

(event EventTick
  (params (DeltaSeconds :type Float%20%28single-precision%29))
  (CallFunction|DecreaseSpellCooldownTime DeltaSeconds))

(fn SetCurrentSpellIdx
  (params (CurrentSpellIdx :type Integer))
  (Variables|Default|SetCurrentSpellIdx (Math|Integer|Max(Integer) (Math|Integer|Min(Integer) CurrentSpellIdx (Utilities|Array|Length (Variables|Default|GetSpellInventory)))))
  (CallFunction|UpdateActiveSpellonHUD))

(fn CanCastSpell
  (params (currMana :type Float%20%28single-precision%29))
  (bind _spellinventory (Variables|Default|GetSpellInventory))
  (bind _currentspellidx (Variables|Default|GetCurrentSpellIdx))
  (bind _output (Utilities|Array|Get(acopy) _spellinventory _currentspellidx))
  (Utilities|IsValid _output
    (:Is%20Valid
      (bind _cancastspell (Default|CanCastSpell _output currMana))
      (return (and _cancastspell (Variables|Default|GetCanCastSpells))))
    (:Is%20Not%20Valid
      (Development|PrintString "Kein Zauber selektiert.")
      (return false))))

(fn ScrollCurrentSpellIdx
  (params (isScrollUp :type Boolean))
  (if isScrollUp
    (if (>= (+ (Variables|Default|GetCurrentSpellIdx) 1) (Utilities|Array|Length (Variables|Default|GetSpellInventory)))
      (Variables|Default|SetCurrentSpellIdx 0)
      (else
        (Variables|Default|SetCurrentSpellIdx (+ (Variables|Default|GetCurrentSpellIdx) 1))))
    (elif (< (- (Variables|Default|GetCurrentSpellIdx) 1) 0)
      (Variables|Default|SetCurrentSpellIdx (- (Utilities|Array|Length (Variables|Default|GetSpellInventory)) 1))
      (else
        (Variables|Default|SetCurrentSpellIdx (- (Variables|Default|GetCurrentSpellIdx) 1)))))
  (CallFunction|UpdateActiveSpellonHUD))

(fn GetCurrentSpell
  (return (Utilities|Array|Get(acopy) (Variables|Default|GetSpellInventory) (Variables|Default|GetCurrentSpellIdx))))

(fn DecreaseSpellCooldownTime
  (params (deltaTime :type Float%20%28single-precision%29))
  (for (_array_element _array_index) (Variables|Default|GetSpellInventory)
    (Utilities|IsValid _array_element
      (:Is%20Valid
        (if (> (Variables|/Game/VikingMageProject/Core/Characters/Player/Spells/BP_Spell.BP_Spell_C|GetcooldownTimeLeft _array_element) 0.0)
          (bind _output_get (Variables|/Game/VikingMageProject/Core/Characters/Player/Spells/BP_Spell.BP_Spell_C|SetcooldownTimeLeft _array_element (- (Variables|/Game/VikingMageProject/Core/Characters/Player/Spells/BP_Spell.BP_Spell_C|GetcooldownTimeLeft _array_element) deltaTime)))
          (Default|UpdateCooldownAbilities (Variables|/Game/VikingMageProject/Core/Characters/Player/BP_PlayerCharacter.BP_PlayerCharacter_C|GetWBP_PlayerHUD (.AsBP%20Player%20Character (Utilities|Casting|CastToBP_PlayerCharacter (Components|GetOwner)))) _array_index (/ _output_get (Variables|/Game/VikingMageProject/Core/Characters/Player/Spells/BP_Spell.BP_Spell_C|GetcooldownTime _array_element)))
          (Development|PrintString (Utilities|String|Append (Utilities|String|ToString(Object) _array_element) "Time Left" (Utilities|String|ToString(Float) (- (Variables|/Game/VikingMageProject/Core/Characters/Player/Spells/BP_Spell.BP_Spell_C|GetcooldownTimeLeft _array_element) deltaTime))) false))))))

(fn CastSpell
  (params (PlayerState :type BP%20Player%20State%20Object%20Reference) (PlayerChar :type BP%20Player%20Character%20Object%20Reference) (SpellOverload :type Boolean))
  (bind _playerchar (LocalVariables|GetplayerChar))
  (bind _playerchar_2 (LocalVariables|GetplayerChar))
  (Variables|/Game/VikingMageProject/Core/Characters/Player/BP_PlayerState.BP_PlayerState_C|SetManaSpeedUpRegain PlayerState false)
  (Variables|/Game/VikingMageProject/Core/Characters/Player/BP_PlayerState.BP_PlayerState_C|SetManaSpeedUpCount PlayerState 0.0)
  (if SpellOverload
    ;[1 1 1] Cheat erlaubt Zaubern ohne Prüfung und Einschränkung
    (bind _currentspell (CallFunction|GetCurrentSpell))
    (Utilities|IsValid _currentspell
      (:Is%20Valid
        _))
    (else
      (bind _cancastspell (CallFunction|CanCastSpell (Variables|/Game/VikingMageProject/Core/Characters/Player/BP_PlayerState.BP_PlayerState_C|GetcurrMana (Variables|/Game/VikingMageProject/Core/Characters/Player/BP_PlayerCharacter.BP_PlayerCharacter_C|GetCustomPlayerState (LocalVariables|GetplayerChar)))))
      (if (Math|Boolean|ANDBoolean _cancastspell (not (Variables|/Game/VikingMageProject/Core/Characters/Player/BP_PlayerCharacter.BP_PlayerCharacter_C|GetIsClimbing _playerchar_2)) (not (Variables|/Game/VikingMageProject/Core/Characters/Player/BP_PlayerCharacter.BP_PlayerCharacter_C|GetIsMenuOpen _playerchar_2)) (not (Variables|/Game/VikingMageProject/Core/Characters/Player/BP_PlayerState.BP_PlayerState_C|GetIsDead PlayerState)))
        _
        (else
          (Development|PrintString "Nicht genug Mana, Cooldown läuft noch oder Zaubern verboten")
          (return false)))))
  (Default|StartFightMode _playerchar)
  (bind _returnvalue (Animation|PlayAnimMontage _playerchar "/Game/VikingMageProject/Characters/Common/Animations/Mage/AM_SpellAttack.AM_SpellAttack" 1.8 "None"))
  (Default|PauseHandsIKforSeconds PlayerChar _returnvalue)
  (bind _currentspell_2 (CallFunction|GetCurrentSpell))
  (Utilities|IsValid _currentspell_2
    (:Is%20Valid
      (Default|CastSpell _currentspell_2 PlayerState PlayerChar)
      (return true))))

(fn UpdateIconsonPlayerHUD
  (bind _asbp_player_character (Utilities|Casting|CastToBP_PlayerCharacter (Components|GetOwner)))
  (LocalVariables|SetPlayerChar _asbp_player_character)
  (for (_array_element _array_index) (Variables|Default|GetSpellInventory)
    (Utilities|IsValid _array_element
      (:Is%20Valid
        (Default|UpdateIconAbilities (Variables|/Game/VikingMageProject/Core/Characters/Player/BP_PlayerCharacter.BP_PlayerCharacter_C|GetWBP_PlayerHUD (LocalVariables|GetPlayerChar)) _array_index (Variables|/Game/VikingMageProject/Core/Characters/Player/Spells/BP_Spell.BP_Spell_C|GetspellIcon _array_element)))
      (:Is%20Not%20Valid
        (Default|UpdateIconAbilities (Variables|/Game/VikingMageProject/Core/Characters/Player/BP_PlayerCharacter.BP_PlayerCharacter_C|GetWBP_PlayerHUD (LocalVariables|GetPlayerChar)) _array_index (Variables|Default|GetTEmptyIcon))))))

(fn UpdateActiveSpellonHUD
  (bind _asbp_player_character (Utilities|Casting|CastToBP_PlayerCharacter (Components|GetOwner)))
  (Default|UpdateActiveAbilities (Variables|/Game/VikingMageProject/Core/Characters/Player/BP_PlayerCharacter.BP_PlayerCharacter_C|GetWBP_PlayerHUD _asbp_player_character) (Variables|Default|GetCurrentSpellIdx)))

(fn SwapSpellat
  (params (Spell :type BP%20Spell%20Class%20Reference) (Index :type Integer))
  (bind _starterspells (Variables|Default|GetstarterSpells))
  (LocalVariables|SetOldSpell (Utilities|Array|Get(acopy) _starterspells Index))
  (Utilities|Array|SetArrayElem _starterspells Index Spell)
  (CallFunction|UpdateSpellInventory)
  (CallFunction|UpdateIconsonPlayerHUD)
  (return (LocalVariables|GetOldSpell)))

(fn RemoveSpellat
  (params (Index :type Integer))
  (bind _swappedspell (CallFunction|SwapSpellat 0 Index))
  (return _swappedspell))

(fn UpdateSpellInventory
  (for (_array_element _array_index) (Variables|Default|GetStarterSpells)
    (bind _returnvalue (Game|ConstructObjectfromClass _array_element self))
    (Utilities|Array|SetArrayElem (Variables|Default|GetSpellInventory) _array_index _returnvalue)))