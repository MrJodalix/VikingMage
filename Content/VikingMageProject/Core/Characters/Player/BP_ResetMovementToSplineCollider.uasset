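; BP_ResetMovementToSplineCollider is a trigger actor that ends the player character's off-spline walking state.
; A sphere overlap stores the BP_PlayerCharacter reference, which Tick then polls until its XY position is within a small tolerance of the actor's own, ignoring height.
; On a match it clears IsWalkingOffSpline, re-enables spell casting on the player's spell component and destroys itself.
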(event OnComponentBeginOverlap(Sphere)
  (params (OverlappedComponent :type Primitive%20Component%20Object%20Reference) (OtherActor :type Actor%20Object%20Reference) (OtherComp :type Primitive%20Component%20Object%20Reference) (OtherBodyIndex :type Integer) (bFromSweep :type Boolean) (SweepResult :type Hit%20Result%20Structure%20%28by%20ref%29))
  (bind _asbp_player_character (Utilities|Casting|CastToBP_PlayerCharacter OtherActor))
  (Variables|Default|SetPlayerChar _asbp_player_character))

(event EventTick
  (params (DeltaSeconds :type Float%20%28single-precision%29))
  (bind _self self)
  (bind _playerchar (Variables|Default|GetPlayerChar))
  (bind _playerchar_2 (Variables|Default|GetPlayerChar))
  (bind _returnvalue (Transformation|GetActorLocation _playerchar_2))
  (bind _returnvalue_2 (Transformation|GetActorLocation _self))
  (if (Utilities|IsValid (Variables|Default|GetPlayerChar))
    (if (Math|Vector|Equal(Vector) (Math|Vector2D|MakeVector2D (.x _returnvalue) (.y _returnvalue)) (Math|Vector2D|MakeVector2D (.x _returnvalue_2) (.y _returnvalue_2)) 1.0)
      (Variables|/Game/VikingMageProject/Core/Characters/Player/BP_PlayerCharacter.BP_PlayerCharacter_C|SetIsWalkingOffSpline _playerchar false)
      (Variables|/Game/VikingMageProject/Core/Characters/Player/Spells/BP_SpellComponent.BP_SpellComponent_C|SetCanCastSpells (Variables|/Game/VikingMageProject/Core/Characters/Player/BP_PlayerCharacter.BP_PlayerCharacter_C|GetCharacter%20Spells%20%28SpellComponent%29 _playerchar) true)
      (Actor|DestroyActor))))

(fn ConstructionScript)