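; Arena wave spawner that spawns enemy waves focused on the player, with difficulty selection and arena start triggered by dialogue events.
; Each wave's power budget grows with the squared index over a difficulty divisor, then gets spent on random EnemyPool units by PowerLevel.
; Units spawn at the spawner with death bindings, and when none remain the next wave follows after a delay.
; ArenaStop clears enemies, player focus and the wave index.
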(event Custom|ArenaStart
  (bind _waveindex (Variables|Default|GetWaveIndex))
  (Variables|Default|SetIsActive true)
  (Development|PrintString (Utilities|String|Append "Spawning Wave " (Utilities|String|ToString(Integer) _waveindex)))
  (bind _wave (CallFunction|GenerateWave _waveindex))
  (bind _waveactors (CallFunction|SpawnWave _wave))
  (bind _output_get (Variables|Default|SetWaveActors _waveactors))
  (Variables|Default|SetRemainingActors (Utilities|Array|Length _output_get)))

(event Custom|ArenaStop
  (Variables|Default|SetIsActive false)
  (Default|StopAllFocus (.AsBP%20Player%20Character (Utilities|Casting|CastToBP_PlayerCharacter (Game|GetPlayerCharacter 0))))
  (CallFunction|DestroyAllWaveActors)
  (Variables|Default|SetWaveIndex 0))

(event Custom|ActorDied
  (bind _result (Math|Integer|DecrementInt (Variables|Default|GetRemainingActors))
    (:%20%20
      (if (== _result 0)
        (Utilities|FlowControl|Delay (Variables|Default|GetTimeBetweenWaves))
        (CallFunction|NextWave)))))

(event Custom|NextWave
  (bind _waveindex (Variables|Default|GetWaveIndex))
  (CallFunction|DestroyAllWaveActors)
  (Math|Integer|IncrementInt (Variables|Default|GetWaveIndex)
    (:%20%20
      (Development|PrintString (Utilities|String|Append "Spawning Wave " (Utilities|String|ToString(Integer) _waveindex)))
      (bind _wave (CallFunction|GenerateWave _waveindex))
      (bind _waveactors (CallFunction|SpawnWave _wave))
      (bind _output_get (Variables|Default|SetWaveActors _waveactors))
      (Variables|Default|SetRemainingActors (Utilities|Array|Length _output_get)))))

(event EventBeginPlay
  (bind _minpower (CallFunction|GetMinUnitPower))
  (Variables|Default|SetMin%20Power _minpower)
  (EventDispatchers|BindEventtoOnRespawnDispatcher (.AsBP%20Player%20Character (Utilities|Casting|CastToBP_PlayerCharacter (Game|GetPlayerCharacter 0))) (EventDispatchers|CreateEvent :!event Custom|ArenaStop)))

(fn ConstructionScript)

(fn GenerateWave
  (params (WaveIndex :type Integer))
  (bind _enemypool (Variables|Default|GetEnemyPool))
  (bind _wavepower (CallFunction|CalculateWavePower (Variables|Default|GetDifficulty) WaveIndex))
  (bind _output_get (LocalVariables|SetCurrentWavePower _wavepower))
  (while (>= _output_get (Variables|Default|GetMin%20Power))
    (bind _output_get_2 (LocalVariables|SetCurrentUnit (Utilities|Array|Get(acopy) _enemypool (Math|Random|RandomInteger (Utilities|Array|Length _enemypool)))))
    (if (>= (LocalVariables|GetCurrentWavePower) (.PowerLevel (Utilities|GetClassDefaults _output_get_2)))
      (Utilities|Array|Add (LocalVariables|GetCurrentWaveUnits) (LocalVariables|GetCurrentUnit))
      (LocalVariables|SetCurrentWavePower (- (LocalVariables|GetCurrentWavePower) (.PowerLevel (Utilities|GetClassDefaults (LocalVariables|GetCurrentUnit)))))
      (Development|PrintString (Utilities|GetClassDisplayName (LocalVariables|GetCurrentUnit)))))
  (return (LocalVariables|GetCurrentWaveUnits)))

(fn CalculateWavePower
  (params (Difficulty :type EDifficulty%20Enum :default "NewEnumerator0") (Index :type Integer))
  (switch Utilities|FlowControl|Switch|SwitchonEDifficulty Difficulty
    (:NewEnumerator0
      (LocalVariables|SetFlatter (Variables|Default|GetEasyFlatter)))
    (:NewEnumerator1
      (LocalVariables|SetFlatter (Variables|Default|GetMediumFlatter)))
    (:NewEnumerator2
      (LocalVariables|SetFlatter (Variables|Default|GetHardFlatter))))
  (return (+ (/ (* Index Index) (LocalVariables|GetFlatter)) (Variables|Default|GetStartStrength))))

(fn SpawnWave
  (params (Wave :type Array%20of%20BP%20NPC%20Class%20References))
  (for _array_element Wave
    (bind _returnvalue (Game|SpawnActorfromClass _array_element (Math|Transform|MakeTransform (Transformation|GetActorLocation) "0, 0, 0" "1,1,1") "AdjustIfPossibleButAlwaysSpawn" 0 0))
    (Pawn|SpawnDefaultController _returnvalue)
    (Default|StartFocusActor _returnvalue (.AsBP%20Character%20Custom (Utilities|Casting|CastToBP_CharacterCustom (Game|GetPlayerCharacter 0))))
    (EventDispatchers|BindEventtoOnDeath (Variables|/Game/VikingMageProject/Core/Characters/NPC/BP_NPC.BP_NPC_C|GetBP_NPCStats _returnvalue) (EventDispatchers|CreateEvent :!event Custom|ActorDied))
    (Utilities|Array|Add (LocalVariables|GetActors) _returnvalue))
  (return (LocalVariables|GetActors)))

(fn GetMinUnitPower
  (bind _enemypool (Variables|Default|GetEnemyPool))
  (LocalVariables|SetMin (.PowerLevel (Utilities|GetClassDefaults (Utilities|Array|Get(acopy) _enemypool))))
  (for _index (range 1 (- (Utilities|Array|Length _enemypool) 1))
    (LocalVariables|SetMin (Math|Integer|Min(Integer) (LocalVariables|GetMin) (.PowerLevel (Utilities|GetClassDefaults (Utilities|Array|Get(acopy) _enemypool _index))))))
  (return (LocalVariables|GetMin)))

(fn DestroyAllWaveActors
  (for _array_element (Variables|Default|GetWaveActors)
    (Actor|DestroyActor _array_element)))

(fn CheckCondition
  (params (Context :type Dlg%20Context%20Object%20Reference) (ConditionName :type Name :default "None"))
  (return false))

(fn GetBoolValue
  (params (ValueName :type Name :default "None"))
  (return false))

(fn GetFloatValue
  (params (ValueName :type Name :default "None"))
  (return 0.0))

(fn GetIntValue
  (params (ValueName :type Name :default "None"))
  (return 0))

(fn GetNameValue
  (params (ValueName :type Name :default "None"))
  (return "None"))

(fn GetParticipantDisplayName
  (params (ActiveSpeaker :type Name :default "None"))
  (return ""))

(fn GetParticipantGender
  (return "Masculine"))

(fn GetParticipantIcon
  (params (ActiveSpeaker :type Name :default "None") (ActiveSpeakerState :type Name :default "None"))
  (return 0))

(fn GetParticipantName
  (return (Variables|Default|GetDlgRefName)))

(fn ModifyBoolValue
  (params (ValueName :type Name :default "None") (bNewValue :type Boolean))
  (return false))

(fn ModifyFloatValue
  (params (ValueName :type Name :default "None") (bDelta :type Boolean) (Value :type Float%20%28single-precision%29))
  (return false))

(fn ModifyIntValue
  (params (ValueName :type Name :default "None") (bDelta :type Boolean) (Value :type Integer))
  (return false))

(fn ModifyNameValue
  (params (ValueName :type Name :default "None") (NameValue :type Name :default "None"))
  (return false))

(fn OnDialogueEvent
  (params (Context :type Dlg%20Context%20Object%20Reference) (EventName :type Name :default "None"))
  (|SwitchDialogueCallbackEvent EventName
    (:Default
      (return false))
    (:SetDifficultyEasy
      (Variables|Default|SetDifficulty "NewEnumerator0"))
    (:SetDifficultyHard
      (Variables|Default|SetDifficulty "NewEnumerator2"))
    (:SetDifficultyMedium
      (Variables|Default|SetDifficulty "NewEnumerator1"))
    (:StartArena
      (CallFunction|ArenaStart)))
  (return true))