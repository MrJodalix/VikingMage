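; NPC character Blueprint that adds sight and hearing reactions through PawnSensing, feeding the AI controller's Blackboard.
; Seen enemy-faction characters are passed to StartFocusActor when no valid TargetActor exists, with players also requiring CanBeSeenByAI.
; Heard noises store their location as LastKnownTargetLocation, and both reactions print debug messages.
; Sensing updates switch off when the stats component reports death.
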(event OnSeePawn(PawnSensing)
  (params (Pawn :type Pawn%20Object%20Reference))
  ;[1 1 1] Sight Reaction
  (CallFunction|OnSeeReaction Pawn))

(event OnDeath(BP_NPCStats)
  (Class|PawnSensingComponent|SetSensingUpdatesEnabled (Variables|Default|GetPawnSensing) false))

(event OnHearNoise(PawnSensing)
  (params (Instigator :type Pawn%20Object%20Reference) (Location :type Vector%20%28by%20ref%29 :default "0, 0, 0") (Volume :type Float%20%28single-precision%29))
  ;[1 1 1] Hearing Reaction
  (CallFunction|OnHearReaction Instigator Location Volume))

(event EventTick
  (params (DeltaSeconds :type Float%20%28single-precision%29))
  (|CallParentFunction DeltaSeconds))

(fn ConstructionScript
  (|CallParentFunction))

(fn OnHearReaction
  (params (Instigator :type Pawn%20Object%20Reference) (Location :type Vector) (Volume :type Float%20%28single-precision%29))
  (AI|Components|Blackboard|SetValueasVector (Variables|/Script/AIModule.AIController|GetBlackboard (AI|GetAIController self)) (Utilities|Name|MakeLiteralName "LastKnownTargetLocation") Location)
  (Development|PrintString "I Heard something!" true true "(R=1.000000,G=0.000000,B=0.060073,A=1.000000)" 5.0))

(fn OnSeeReaction
  (params (Pawn :type Pawn%20Object%20Reference))
  (Development|PrintString (Utilities|String|Append "Should see." (Utilities|GetDisplayName Pawn)))
  (bind _asbp_character_custom (Utilities|Casting|CastToBP_CharacterCustom Pawn))
  (if (CallFunction|IsEnemyFaction (Variables|/Game/VikingMageProject/Core/Characters/BP_CharacterCustom.BP_CharacterCustom_C|GetFaction _asbp_character_custom))
    (bind _asbp_player_character (Utilities|Casting|CastToBP_PlayerCharacter _asbp_character_custom)
      (:then
        (if (Variables|/Game/VikingMageProject/Core/Characters/Player/BP_PlayerCharacter.BP_PlayerCharacter_C|GetCanBeSeenByAI _asbp_player_character)
          (Utilities|IsValid (AI|Components|Blackboard|GetValueasObject (Variables|/Script/AIModule.AIController|GetBlackboard (AI|GetAIController self)) (Utilities|Name|MakeLiteralName "TargetActor")) :!label _label
            (:Is%20Not%20Valid
              (Development|PrintString "See you!")
              (CallFunction|StartFocusActor _asbp_character_custom)))))
      (:CastFailed
        (goto _label)))))