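; BP_NPCStats tracks an NPC's health, death and a timed finisher window.
; ReceiveDamage clamps health, flags the NPC as finishable at or below a health threshold, restarts the timer on every hit, and fires OnDeath at zero.
; Tick counts the window down; on expiry it clears the flag and sets health to the rounded-up threshold.
; Die, bound to OnDeath, sets the death state; its quest-log kill notification is disconnected.
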(event Custom|execDie
  (CallFunction|Die))

(event EventBeginPlay
  (EventDispatchers|BindEventtoOnDeath (delegate Custom|execDie)))

(event EventTick
  (params (DeltaSeconds :type Float%20%28single-precision%29))
  (CallFunction|UpdateFinishable DeltaSeconds))

(fn ReceiveDamage
  (params (amount :type Float%20%28single-precision%29))
  (Variables|Default|Health|SetcurrHealth (Math|Float|Clamp(Float) (- (Variables|Default|Health|GetcurrHealth) amount) 0.0 (Variables|Default|Health|GetmaxHealth)))
  (Variables|Default|Finisher|SetcanBeFinished (<= (Variables|Default|Health|GetcurrHealth) (* (Variables|Default|Health|GetmaxHealth) (Variables|Default|Finisher|GetfinishThreshold))))
  (CallFunction|StartCanbeFinished)
  (if (and (<= (Variables|Default|Health|GetcurrHealth) 0.0) (not (Variables|Default|Health|GetisDead)))
    (Default|CallOnDeath)))

(fn Die
  (Variables|Default|Health|SetisDead true)
  (Variables|Default|Finisher|SetcanBeFinished false))

(fn UpdateFinishable
  (params (DeltaSeconds :type Float%20%28single-precision%29))
  (if (Variables|Default|Finisher|GetcanBeFinished)
    (bind _output_get (Variables|Default|Finisher|SetRestTimeToFinish (- (Variables|Default|Finisher|GetRestTimeToFinish) DeltaSeconds)))
    (bind _output_get_2 (Variables|Default|Finisher|SetcanBeFinished (not (<= _output_get 0.0))))
    (if (not _output_get_2)
      (Variables|Default|Finisher|SetStartedFinishTime false)
      (Variables|Default|Health|SetcurrHealth (Math|Conversions|ToFloat(Integer) (Math|Float|Ceil (* (Variables|Default|Health|GetmaxHealth) (Variables|Default|Finisher|GetfinishThreshold))))))))

(fn StartCanbeFinished
  (Variables|Default|Finisher|SetStartedFinishTime true)
  (Variables|Default|Finisher|SetRestTimeToFinish (Variables|Default|Finisher|GetMaxTimeToFinish)))