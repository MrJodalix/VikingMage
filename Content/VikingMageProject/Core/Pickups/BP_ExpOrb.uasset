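; Experience orb pickup that homes in on the player and grants experience on contact.
; BeginPlay stores the first player character as the target, and Tick moves the orb straight toward it at MovementSpeed without sweeping.
; On sphere overlap with BP_PlayerCharacter, it adds ExpAmount to that player's BP_PlayerState and destroys itself.
; An Initialize function lets the spawner set ExpAmount.
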(event OnComponentBeginOverlap(Sphere)
  (params (OverlappedComponent :type Primitive%20Component%20Object%20Reference) (OtherActor :type Actor%20Object%20Reference) (OtherComp :type Primitive%20Component%20Object%20Reference) (OtherBodyIndex :type Integer) (bFromSweep :type Boolean) (SweepResult :type Hit%20Result%20Structure%20%28by%20ref%29))
  (bind _asbp_player_character (Utilities|Casting|CastToBP_PlayerCharacter OtherActor))
  (bind _asbp_player_state (Utilities|Casting|CastToBP_PlayerState (Variables|/Script/Engine.Pawn|GetPlayerState _asbp_player_character)))
  (Default|AddExperience _asbp_player_state (Variables|Default|GetexpAmount))
  (Actor|DestroyActor))

(event EventTick
  (params (DeltaSeconds :type Float%20%28single-precision%29))
  (CallFunction|MovetoTarget (Variables|Default|GetmoveTarget) DeltaSeconds (Variables|Default|GetmovementSpeed)))

(event EventBeginPlay
  (Variables|Default|SetmoveTarget (Game|GetPlayerCharacter 0)))

(fn ConstructionScript)

(fn MovetoTarget
  (params (moveTarget :type Actor%20Object%20Reference) (deltaSeconds :type Float%20%28single-precision%29) (speed :type Float%20%28single-precision%29))
  (Transformation|SetActorLocation (+ (* (* (Math|Vector|Normalize (- (Transformation|GetActorLocation moveTarget) (Transformation|GetActorLocation))) deltaSeconds) speed) (Transformation|GetActorLocation)) false false))

(fn Initialize
  (params (expAmount :type Float%20%28single-precision%29))
  (Variables|Default|SetexpAmount expAmount))