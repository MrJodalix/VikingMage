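; Ambient sound manager that switches the playing ambience between day and night sets, following the UDS actor's sunrise and sunset events.
; Add and remove calls maintain reference-counted sound maps, though adds always write to the day map, even for night sounds.
; Each update diffs the current set against active sounds, keeping shared ones playing, fading in new attached sounds and fading out unneeded ones.
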(fn Initialize
  (params (UDS_Actor :type Ultra%20Dynamic%20Sky%20Object%20Reference))
  (bind _time_of_day (Variables|/Game/UltraDynamicSky/Blueprints/Ultra_Dynamic_Sky.Ultra_Dynamic_Sky_C|GetTime%20of%20Day UDS_Actor))
  (Utilities|IsValid UDS_Actor
    (:Is%20Valid
      (Variables|Default|SetDayTime (select (and (< (+ (Variables|/Game/UltraDynamicSky/Blueprints/Ultra_Dynamic_Sky.Ultra_Dynamic_Sky_C|GetDawn%20Time UDS_Actor) (Variables|/Game/UltraDynamicSky/Blueprints/Ultra_Dynamic_Sky.Ultra_Dynamic_Sky_C|GetSunrise%20Event%20Offset UDS_Actor)) _time_of_day) (< _time_of_day (+ (Variables|/Game/UltraDynamicSky/Blueprints/Ultra_Dynamic_Sky.Ultra_Dynamic_Sky_C|GetDusk%20Time UDS_Actor) (Variables|/Game/UltraDynamicSky/Blueprints/Ultra_Dynamic_Sky.Ultra_Dynamic_Sky_C|GetSunset%20Event%20Offset UDS_Actor)))) "NewEnumerator1" "NewEnumerator3"))
      (EventDispatchers|BindEventtoSunrise UDS_Actor (EventDispatchers|CreateEvent :!event SetPlayModeDay))
      (EventDispatchers|BindEventtoSunset UDS_Actor (EventDispatchers|CreateEvent :!event SetPlayModeNight)))
    (:Is%20Not%20Valid
      (Development|PrintString 0 "WARNING: Ambient Sound Manager could not be properly initialized"))))

(fn SetPlayModeDay
  (Variables|Default|SetDayTime "NewEnumerator1")
  (CallFunction|UpdateActiveSounds))

(fn SetPlayModeNight
  (Variables|Default|SetDayTime "NewEnumerator3")
  (CallFunction|UpdateActiveSounds))

(fn AddSoundtoMap
  (params (SoundIn :type Sound%20Base%20Object%20Reference) (Data :type S%20Stored%20Sound%20Data%20Structure) (Sounds :type Map%20of%20Sound%20Base%20Object%20References%20to%20Structs))
  (bind (_value _returnvalue) (Utilities|Map|Find Sounds SoundIn))
  (if _returnvalue
    ;[1 1 1] Increase Ref Counter
    (Utilities|Map|Add (Variables|Default|GetCurrDayTimeSounds) SoundIn (Utilities|Struct|MakeSStoredSoundData (.fadein Data) (.fadeout Data) (.attachmentcomponent Data) (+ (.References (Utilities|Struct|BreakSStoredSoundData _value)) 1)))
    (else
      ;[1 1 1] Add New
      (Utilities|Map|Add (Variables|Default|GetCurrDayTimeSounds) SoundIn Data)))
  (CallFunction|UpdateActiveSounds))

(fn RemoveSoundfromMap
  (params (SoundIn :type Sound%20Base%20Soft%20Object%20Reference) (Data :type S%20Stored%20Sound%20Data%20Structure) (Sounds :type Map%20of%20Sound%20Base%20Object%20References%20to%20Structs))
  (LocalVariables|SetSound (Utilities|ResolveSoftReference SoundIn))
  (if (.ReturnValue (Utilities|Map|Find Sounds (LocalVariables|GetSound)))
    (if (> (- (.References (Utilities|Struct|BreakSStoredSoundData (.Value (Utilities|Map|Find Sounds (LocalVariables|GetSound))))) 1) 0)
      (Utilities|Map|Add Sounds (LocalVariables|GetSound) (Utilities|Struct|MakeSStoredSoundData (.fadein Data) (.fadeout Data) (.attachmentcomponent Data) (- (.References (Utilities|Struct|BreakSStoredSoundData (.Value (Utilities|Map|Find Sounds (LocalVariables|GetSound))))) 1)))
      (else
        (Utilities|Map|Remove Sounds (LocalVariables|GetSound))))
    (CallFunction|UpdateActiveSounds)))

(fn UpdateActiveSounds
  (bind _activesounds (Variables|Default|GetActiveSounds))
  (Utilities|FlowControl|Sequence
    (:then_0
      ;[1 1 1] Cache and clear currently Playing sounds Sounds
      (LocalVariables|SetSoundsToStop _activesounds)
      (Utilities|Map|Clear _activesounds))
    (:then_1
      (switch Utilities|FlowControl|Switch|SwitchonEDayTime (Variables|Default|GetDayTime)
        (:NewEnumerator1
          (LocalVariables|SetSoundsToPlay (Variables|Default|GetCurrDayTimeSounds)))
        (:NewEnumerator3
          (LocalVariables|SetSoundsToPlay (Variables|Default|GetCurrNightTimeSounds))))
      (bind _keys (Utilities|Map|Keys (LocalVariables|GetSoundsToPlay)))
      (for _array_element _keys
        (bind _output_get (LocalVariables|SetCurrSound _array_element))
        (if (.ReturnValue (Utilities|Map|Find (LocalVariables|GetSoundsToStop) _output_get))
          ;[1 1 1] Reuse Existing Sound (keep it playing) (if Audio Component is invalid sound ended, do not restart)
          (Utilities|IsValid (.AudioComponent (Utilities|Struct|BreakSActiveSoundData (.Value (Utilities|Map|Find (LocalVariables|GetSoundsToStop) _output_get))))
            (:Is%20Valid
              (Utilities|Map|Add (Variables|Default|GetActiveSounds) (LocalVariables|GetCurrSound) (Utilities|Struct|MakeSActiveSoundData (.FadeIn (Utilities|Struct|BreakSStoredSoundData (.Value (Utilities|Map|Find (LocalVariables|GetSoundsToPlay) (LocalVariables|GetCurrSound))))) (.FadeOut (Utilities|Struct|BreakSStoredSoundData (.Value (Utilities|Map|Find (LocalVariables|GetSoundsToPlay) (LocalVariables|GetCurrSound))))) (.AudioComponent (Utilities|Struct|BreakSActiveSoundData (.Value (Utilities|Map|Find (LocalVariables|GetSoundsToStop) _output_get))))))
              (Utilities|Map|Remove (LocalVariables|GetSoundsToStop) (LocalVariables|GetCurrSound))))
          (else
            ;[1 1 1] Sound not found => spawn new
            (bind _returnvalue (Audio|SpawnSoundAttached (LocalVariables|GetCurrSound) (.AttachmentComponent (Utilities|Struct|BreakSStoredSoundData (.Value (Utilities|Map|Find (LocalVariables|GetSoundsToPlay) (LocalVariables|GetCurrSound))))) "None" "0, 0, 0" "0, 0, 0" "KeepRelativeOffset" false 1.0 1.0 0.0 0 0))
            (Utilities|Map|Add (Variables|Default|GetActiveSounds) (LocalVariables|GetCurrSound) (Utilities|Struct|MakeSActiveSoundData (.FadeIn (Utilities|Struct|BreakSStoredSoundData (.Value (Utilities|Map|Find (LocalVariables|GetSoundsToPlay) (LocalVariables|GetCurrSound))))) (.FadeOut (Utilities|Struct|BreakSStoredSoundData (.Value (Utilities|Map|Find (LocalVariables|GetSoundsToPlay) (LocalVariables|GetCurrSound))))) _returnvalue))
            (Audio|Components|Audio|FadeIn _returnvalue (.FadeIn (Utilities|Struct|BreakSStoredSoundData (.Value (Utilities|Map|Find (LocalVariables|GetSoundsToPlay) (LocalVariables|GetCurrSound))))) 1.0 0.0 "Linear" :!class /Script/Engine.AudioComponent))))
      ;[1 1 1] All Incoming sounds are playing, stop playing sounds that are no longer needed
      (bind _values (Utilities|Map|Values (LocalVariables|GetSoundsToStop)))
      (for _array_element_2 _values
        (Utilities|IsValid (.AudioComponent (Utilities|Struct|BreakSActiveSoundData _array_element_2))
          (:Is%20Valid
            (Audio|Components|Audio|FadeOut (.AudioComponent (Utilities|Struct|BreakSActiveSoundData _array_element_2)) (.FadeOut (Utilities|Struct|BreakSActiveSoundData _array_element_2)) 0.0 "Linear" :!class /Script/Engine.AudioComponent)))))))

(fn AddAmbientSound
  (params (SoundIn :type Sound%20Base%20Object%20Reference) (DayTime :type EDayTime%20Enum :default "NewEnumerator1") (Data :type S%20Stored%20Sound%20Data%20Structure))
  (switch Utilities|FlowControl|Switch|SwitchonEDayTime DayTime
    (:NewEnumerator1
      (CallFunction|AddSoundtoMap SoundIn Data (Variables|Default|GetCurrDayTimeSounds)))
    (:NewEnumerator3
      (CallFunction|AddSoundtoMap SoundIn Data (Variables|Default|GetCurrNightTimeSounds)))))

(fn RemoveAmbientSound
  (params (SoundIn :type Sound%20Base%20Soft%20Object%20Reference) (DayTime :type EDayTime%20Enum :default "NewEnumerator1") (Data :type S%20Stored%20Sound%20Data%20Structure))
  (switch Utilities|FlowControl|Switch|SwitchonEDayTime DayTime
    (:NewEnumerator1
      (CallFunction|RemoveSoundfromMap SoundIn Data (Variables|Default|GetCurrDayTimeSounds)))
    (:NewEnumerator3
      (CallFunction|RemoveSoundfromMap SoundIn Data (Variables|Default|GetCurrNightTimeSounds)))))