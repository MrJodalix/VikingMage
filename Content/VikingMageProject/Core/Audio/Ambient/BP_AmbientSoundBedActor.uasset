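; Trigger-volume actor that supplies day and night ambient sound beds while the player is inside it.
; On overlap, it async-loads each bed from its AudioPreset and registers it with the GameInstance's AmbientSoundManager, tagged by time of day, with fade times and attachment root.
; Loads that finish after the player leaves are discarded.
; Exit removes both lists from the manager, passing the day tag for night beds too.
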(event OnComponentBeginOverlap(AudioTrigger)
  (params (OverlappedComponent :type Primitive%20Component%20Object%20Reference) (OtherActor :type Actor%20Object%20Reference) (OtherComp :type Primitive%20Component%20Object%20Reference) (OtherBodyIndex :type Integer) (bFromSweep :type Boolean) (SweepResult :type Hit%20Result%20Structure%20%28by%20ref%29))
  (bind _audiopreset (Variables|Default|GetAudioPreset))
  (if (== OtherActor (Game|GetPlayerCharacter 0))
    (Variables|Default|SetOverlapping true)
    (Utilities|FlowControl|Sequence
      (:then_0
        (for _array_element (Variables|/Game/VikingMageProject/Core/Audio/Ambient/BP_AmbientSoundData.BP_AmbientSoundData_C|GetDayTimeAmbientBeds _audiopreset)
          (Utilities|LoadandAddSoundtoManager _array_element "NewEnumerator1")))
      (:then_1
        (for _array_element_2 (Variables|/Game/VikingMageProject/Core/Audio/Ambient/BP_AmbientSoundData.BP_AmbientSoundData_C|GetNightTimeAmbientBeds _audiopreset)
          (Utilities|LoadandAddSoundtoManager _array_element_2 "NewEnumerator3"))))))

(event OnComponentEndOverlap(AudioTrigger)
  (params (OverlappedComponent :type Primitive%20Component%20Object%20Reference) (OtherActor :type Actor%20Object%20Reference) (OtherComp :type Primitive%20Component%20Object%20Reference) (OtherBodyIndex :type Integer))
  (bind _audiopreset (Variables|Default|GetAudioPreset))
  (if (== (Game|GetPlayerCharacter 0) OtherActor)
    (Variables|Default|SetOverlapping false)
    (Utilities|FlowControl|Sequence
      (:then_0
        (for _array_element (Variables|/Game/VikingMageProject/Core/Audio/Ambient/BP_AmbientSoundData.BP_AmbientSoundData_C|GetDayTimeAmbientBeds _audiopreset)
          (Default|RemoveAmbientSound (Variables|/Game/VikingMageProject/Core/Characters/Player/BP_GameInstance.BP_GameInstance_C|GetAmbientSoundManager (.AsBP%20Game%20Instance (Utilities|Casting|CastToBP_GameInstance (Game|GetGameInstance)))) (.AmbientSound (Utilities|Struct|BreakSAmbientSoundBed _array_element)) "NewEnumerator1" (Utilities|Struct|MakeSStoredSoundData (.FadeIn (Utilities|Struct|BreakSAmbientSoundBed _array_element)) (.FadeOut (Utilities|Struct|BreakSAmbientSoundBed _array_element)) (Variables|Default|GetDefaultSceneRoot) 1))))
      (:then_1
        (for _array_element_2 (Variables|/Game/VikingMageProject/Core/Audio/Ambient/BP_AmbientSoundData.BP_AmbientSoundData_C|GetNightTimeAmbientBeds _audiopreset)
          (Default|RemoveAmbientSound (Variables|/Game/VikingMageProject/Core/Characters/Player/BP_GameInstance.BP_GameInstance_C|GetAmbientSoundManager (.AsBP%20Game%20Instance (Utilities|Casting|CastToBP_GameInstance (Game|GetGameInstance)))) (.AmbientSound (Utilities|Struct|BreakSAmbientSoundBed _array_element_2)) "NewEnumerator1" (Utilities|Struct|MakeSStoredSoundData (.FadeIn (Utilities|Struct|BreakSAmbientSoundBed _array_element_2)) (.FadeOut (Utilities|Struct|BreakSAmbientSoundBed _array_element_2)) (Variables|Default|GetDefaultSceneRoot) 1)))))))

(event EventTick
  (params (DeltaSeconds :type Float%20%28single-precision%29)))

(fn ConstructionScript)