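; BP_MusicOptionsArea is a placeable trigger area that changes the music play mode while the player is inside it.
; When a BP_PlayerCharacter begins overlapping the Area component, it sets the MusicManager on BP_GameInstance to the ModeToSet variable.
; When the player stops overlapping, it sets the play mode to None rather than restoring the previous one.
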(event OnComponentBeginOverlap(Area)
  (params (OverlappedComponent :type Primitive%20Component%20Object%20Reference) (OtherActor :type Actor%20Object%20Reference) (OtherComp :type Primitive%20Component%20Object%20Reference) (OtherBodyIndex :type Integer) (bFromSweep :type Boolean) (SweepResult :type Hit%20Result%20Structure%20%28by%20ref%29))
  (if (== (Utilities|GetClass OtherActor) "/Game/VikingMageProject/Core/Characters/Player/BP_PlayerCharacter.BP_PlayerCharacter_C")
    (Default|SetPlayMode (Variables|/Game/VikingMageProject/Core/Characters/Player/BP_GameInstance.BP_GameInstance_C|GetMusicManager (.AsBP%20Game%20Instance (Utilities|Casting|CastToBP_GameInstance (Game|GetGameInstance)))) (Variables|Default|GetModeToSet))))

(event OnComponentEndOverlap(Area)
  (params (OverlappedComponent :type Primitive%20Component%20Object%20Reference) (OtherActor :type Actor%20Object%20Reference) (OtherComp :type Primitive%20Component%20Object%20Reference) (OtherBodyIndex :type Integer))
  (if (== (Utilities|GetClass OtherActor) "/Game/VikingMageProject/Core/Characters/Player/BP_PlayerCharacter.BP_PlayerCharacter_C")
    (Default|SetPlayMode (Variables|/Game/VikingMageProject/Core/Characters/Player/BP_GameInstance.BP_GameInstance_C|GetMusicManager (.AsBP%20Game%20Instance (Utilities|Casting|CastToBP_GameInstance (Game|GetGameInstance)))) "None")))

(event EventBeginPlay)

(event Collision|EventActorBeginOverlap
  (params (OtherActor :type Actor%20Object%20Reference)))

(event EventTick
  (params (DeltaSeconds :type Float%20%28single-precision%29)))

(fn ConstructionScript)