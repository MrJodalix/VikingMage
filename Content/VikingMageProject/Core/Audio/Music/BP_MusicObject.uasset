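; Music object that plays a set of layered tracks whose mix follows the current play mode.
; Play spawns and fades in every layer on an attach component, keeping inactive ones at OffLayerVolume so mode changes only crossfade volumes.
; ShouldLayerPlay picks each layer's per-mode volume, falling back to its default settings for modes no layer defines.
; Stop fades all layers out, then a timer marks it stopped and signals completion.
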(fn Stop
  (if (Utilities|Enum|Equal(Enum) (Variables|Default|GetPlayState) "Playing")
    (bind _values (Utilities|Map|Values (Variables|Default|GetMusic)))
    (for _array_element _values
      (Utilities|IsValid (.SoundComponent (Utilities|Struct|BreakSMusicLayerData _array_element))
        (:Is%20Valid
          (Audio|Components|Audio|FadeOut (.SoundComponent (Utilities|Struct|BreakSMusicLayerData _array_element)) (Variables|Default|GetFadeOutTime) 0.0 "Linear" :!class /Script/Engine.AudioComponent))))
    (Utilities|Time|SetTimerbyFunctionName self "PlayingStopped" (Variables|Default|GetFadeOutTime))
    (Variables|Default|SetPlayState "FadingOut")
    (return true)
    (else
      (return false))))

(fn HasStopped
  (bind _playstate (Variables|Default|GetPlayState))
  (return (or (Utilities|Enum|Equal(Enum) _playstate "Stopped") (Utilities|Enum|Equal(Enum) _playstate "FadingOut"))))

(fn Play
  (params (Mode :type Name :default "None"))
  (bind _music (Variables|Default|GetMusic))
  (Variables|Default|SetCurrentMode Mode)
  (CallFunction|Init)
  (bind _keys (Utilities|Map|Keys _music))
  (for _array_element _keys
    (bind _returnvalue (Audio|SpawnSoundAttached _array_element (Variables|Default|GetAttachComponent) "None" "0, 0, 0" "0, 0, 0" "KeepRelativeOffset" false 1.0 1.0 0.0 0 0))
    (Utilities|Map|Add (Variables|Default|GetMusic) _array_element (Utilities|Struct|MakeSMusicLayerData _returnvalue (.modestoplayin (.Value (Utilities|Map|Find _music _array_element))) (.playbydefault (.Value (Utilities|Map|Find _music _array_element))) (.defaultvolume (.Value (Utilities|Map|Find _music _array_element)))))
    (bind _volume (Utilities|ShouldLayerPlay (.modestoplayin (.Value (Utilities|Map|Find _music _array_element))) (.playbydefault (.Value (Utilities|Map|Find _music _array_element))) (.defaultvolume (.Value (Utilities|Map|Find _music _array_element))))
      (:Play
        (Audio|Components|Audio|FadeIn _returnvalue (Variables|Default|GetFadeInTime) _volume 0.0 "Linear" :!class /Script/Engine.AudioComponent))
      (:DontPlay
        (Audio|Components|Audio|FadeIn _returnvalue (Variables|Default|GetFadeInTime) (Variables|Default|GetOffLayerVolume) 0.0 "Linear" :!class /Script/Engine.AudioComponent)))
    (Audio|Components|Audio|SetVolumeMultiplier _returnvalue (Variables|Default|GetMasterVolume) :!class /Script/Engine.AudioComponent))
  (Variables|Default|SetPlayState "Playing"))

(fn PlayingStopped
  (Variables|Default|SetPlayState "Stopped")
  (Default|CallOnStoppedPlaying))

(fn UpdateLayers
  (bind _offlayervolume (Variables|Default|GetOffLayerVolume))
  (Development|PrintString 0 (Utilities|String|Append "Updating " (Utilities|GetObjectName self)))
  (bind _values (Utilities|Map|Values (Variables|Default|GetMusic)))
  (for _array_element _values
    (Utilities|IsValid (.SoundComponent (Utilities|Struct|BreakSMusicLayerData _array_element))
      (:Is%20Valid
        (bind _volume (Utilities|ShouldLayerPlay (.ModesToPlayIn (Utilities|Struct|BreakSMusicLayerData _array_element)) (.PlayByDefault (Utilities|Struct|BreakSMusicLayerData _array_element)) (.DefaultVolume (Utilities|Struct|BreakSMusicLayerData _array_element)))
          (:Play
            (Audio|Components|Audio|AdjustVolume (.SoundComponent (Utilities|Struct|BreakSMusicLayerData _array_element)) (Variables|Default|GetCrossfadeTime) (Math|Float|Max(Float) _volume _offlayervolume) "Linear" :!class /Script/Engine.AudioComponent))
          (:DontPlay
            (Audio|Components|Audio|AdjustVolume (.SoundComponent (Utilities|Struct|BreakSMusicLayerData _array_element)) (Variables|Default|GetCrossfadeTime) _offlayervolume "Linear" :!class /Script/Engine.AudioComponent)))))))

(fn Init
  (Utilities|FlowControl|DoOnce false
    (:Completed
      (bind _values (Utilities|Map|Values (Variables|Default|GetMusic)))
      (for _array_element _values
        (bind _keys (Utilities|Map|Keys (.ModesToPlayIn (Utilities|Struct|BreakSMusicLayerData _array_element))))
        (for _array_element_2 _keys
          (Utilities|Array|AddUnique (Variables|Default|GetAvailableModes) _array_element_2))))))

(fn SetPlayMode
  (params (Mode :type Name))
  (Variables|Default|SetCurrentMode Mode)
  (CallFunction|UpdateLayers))