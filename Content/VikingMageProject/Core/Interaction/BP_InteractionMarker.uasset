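; BP_InteractionMarker is an overlap trigger that makes a referenced Actor interactable for the player character.
; Entering InteractionRange while active either auto-interacts, optionally only until the first success, or shows a message widget attached to that Actor.
; Interact sends the interact message to the Actor, reports it to player 0's quest log, and returns the result.
; Leaving range destroys any prompt and closes the other inventory.
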(event OnComponentBeginOverlap(InteractionRange)
  (params (OverlappedComponent :type Primitive%20Component%20Object%20Reference) (OtherActor :type Actor%20Object%20Reference) (OtherComp :type Primitive%20Component%20Object%20Reference) (OtherBodyIndex :type Integer) (bFromSweep :type Boolean) (SweepResult :type Hit%20Result%20Structure%20%28by%20ref%29))
  (bind _asbp_player_character (Utilities|Casting|CastToBP_PlayerCharacter OtherActor))
  (if (Variables|Default|GetIsActive)
    (if (Variables|Default|GetAutoInteract)
      (bind _success (CallFunction|Interact _asbp_player_character))
      (Variables|Default|SetAutoInteract (not (and _success (Variables|Default|GetAutoInteractOnlyOnce))))
      (else
        (bind _returnvalue (AddComponent|AddWidgetComponent false))
        (bind _output_get (Variables|Default|SetInteractMessage _returnvalue))
        (Variables|/Game/VikingMageProject/Core/Interaction/WBP_InteractMessage_UI.WBP_InteractMessage_UI_C|SetMessage (.AsWBP%20Interact%20Message%20UI (Utilities|Casting|CastToWBP_InteractMessage_UI (UserInterface|GetWidget _output_get))) (Variables|Default|GetMessage))
        (bind _returnvalue_2 (AddComponent|AddSceneComponent (Variables|Default|GetActor) false))
        (Transformation|AttachComponentToComponent _output_get _returnvalue_2 "None" "KeepRelative" "KeepRelative" "KeepRelative" true)))))

(event OnComponentEndOverlap(InteractionRange)
  (params (OverlappedComponent :type Primitive%20Component%20Object%20Reference) (OtherActor :type Actor%20Object%20Reference) (OtherComp :type Primitive%20Component%20Object%20Reference) (OtherBodyIndex :type Integer))
  (bind _asbp_player_character (Utilities|Casting|CastToBP_PlayerCharacter OtherActor))
  (bind _interactmessage (Variables|Default|GetInteractMessage)
    (:then
      (Components|DestroyComponent _interactmessage)
      (Default|CloseOtherInventory (Variables|/Game/VikingMageProject/Core/Characters/Player/BP_PlayerCharacter.BP_PlayerCharacter_C|GetInventory%20%28InventoryComponent%29 _asbp_player_character)))
    (:else)))

(fn ConstructionScript)

(fn Interact
  (params (Interactor :type BP%20Player%20Character%20Object%20Reference))
  (if (Variables|Default|GetIsActive)
    (bind _success (Class|BPIInteract|Interact(Message) (Variables|Default|GetActor) Interactor))
    (Default|ActorInteractedwith (Variables|/Game/VikingMageProject/Core/Characters/Player/BP_PlayerCharacter.BP_PlayerCharacter_C|GetQuestLog%20%28QuestLogComponent%29 (.AsBP%20Player%20Character (Utilities|Casting|CastToBP_PlayerCharacter (Game|GetPlayerCharacter 0)))) (Variables|Default|GetActor))
    (return _success)))