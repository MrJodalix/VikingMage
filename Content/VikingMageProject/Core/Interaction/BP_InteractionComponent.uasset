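; BP_InteractionComponent is an interaction component for the player character that triggers the closest interaction marker in range.
; On an interact button press, it loops over InteractMarkersInRange and picks the marker whose root is nearest the given player position.
; If that marker is valid, it calls Interact on it, passing the owner cast to BP_PlayerCharacter.
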(event Custom|OnInteractButtonPressed
  (params (PlayerPos :type Vector))
  (bind _marker (CallFunction|GetNearestInteractionMarker PlayerPos))
  (Utilities|IsValid _marker
    (:Is%20Valid
      (Default|Interact _marker (.AsBP%20Player%20Character (Utilities|Casting|CastToBP_PlayerCharacter (Components|GetOwner)))))))

(fn GetNearestInteractionMarker
  (params (PlayerPos :type Vector))
  (for _array_element (Variables|Default|GetInteractMarkersInRange)
    (if (< (Math|Vector|VectorLength (- PlayerPos (Transformation|GetWorldLocation (Variables|/Game/VikingMageProject/Core/Interaction/BP_InteractionMarker.BP_InteractionMarker_C|GetDefaultSceneRoot _array_element)))) (LocalVariables|GetClosestDistance))
      (LocalVariables|SetClosestDistance (Math|Vector|VectorLength (- PlayerPos (Transformation|GetWorldLocation (Variables|/Game/VikingMageProject/Core/Interaction/BP_InteractionMarker.BP_InteractionMarker_C|GetDefaultSceneRoot _array_element)))))
      (LocalVariables|SetClosestMarker _array_element)))
  (return (LocalVariables|GetClosestMarker)))