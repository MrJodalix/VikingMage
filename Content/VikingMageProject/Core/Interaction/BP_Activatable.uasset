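; Base interactable that becomes active when its dependency Activatables are active, optionally also requiring a toggle trigger.
; Tick animates dependency and trigger progress over set times, feeding empty Visualize events meant for child overrides.
; EvaluateActivity updates Active immediately or at animation endpoints and broadcasts ActivityChanged, waking dependents' Tick to form chains; settled endpoints switch Tick off.
; The construction script previews editor progress values and warns about inconsistent setups.
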(event Custom|VisualizeDependenciesProgress
  (params (Progress :type Float%20%28single-precision%29)))

(event Custom|VisualizeTriggeredProgress
  (params (Progress :type Float%20%28single-precision%29)))

(event Custom|DependeciesChanged
  ;[1 1 1] Start Listening for Dependency changes
  (Actor|Tick|SetActorTickEnabled true))

(event EventBeginPlay
  (Utilities|FlowControl|Sequence
    (:then_0
      (CallFunction|InitializeState))
    (:then_1
      ;[1 1 1] Start Listening for Dependency changes
      (for _array_element (Variables|Custom|ActivateDependant|GetDependencies)
        (EventDispatchers|AssignActivityChanged _array_element (delegate Custom|DependeciesChanged))))))

(event EventTick
  (params (DeltaSeconds :type Float%20%28single-precision%29))
  (Utilities|FlowControl|Sequence
    (:then_0
      ;[1 1 1] Auto Activation Behavior
      (bind _out_depprogress (CallFunction|CalcDepProgress))
      (bind _newcurrentprogress (CallFunction|AnimateProgress DeltaSeconds (Variables|Custom|ActivateDependant|GetCurrDepProgress) _out_depprogress (Variables|Custom|ActivateDependant|GetDependantActivationTime)))
      (bind _output_get (Variables|Custom|ActivateDependant|SetCurrDepProgress _newcurrentprogress))
      (CallFunction|VisualizeDependenciesProgress _output_get))
    (:then_1
      ;[1 1 1] Triggered Activation Behavior
      (if (Variables|Custom|ActivateTriggered|GetActivateOnTrigger)
        (bind _output_get_2 (Variables|Custom|ActivateTriggered|SetGoingToActive (and (Variables|Custom|ActivateTriggered|GetGoingToActive) (== (Variables|Custom|ActivateDependant|GetCurrDepProgress) 1.0)))) ; Going active goes false if Dependency Progress isn't enough
        (bind _newcurrentprogress_2 (CallFunction|AnimateProgress DeltaSeconds (Variables|Custom|ActivateTriggered|GetCurrTrigProgress) (Math|Conversions|ToFloat(Boolean) _output_get_2) (Variables|Custom|ActivateTriggered|GetTriggeredActivationTime)))
        (bind _output_get_3 (Variables|Custom|ActivateTriggered|SetCurrTrigProgress _newcurrentprogress_2))
        (CallFunction|VisualizeTriggeredProgress _output_get_3)))
    (:then_2
      (CallFunction|EvaluateActivity))))

(fn ConstructionScript
  (Utilities|FlowControl|Sequence
    (:then_0
      (if (and (== (Utilities|Array|Length (Variables|Custom|ActivateDependant|GetDependencies)) 0) (> (Variables|Custom|ActivateDependant|GetDependantActivationTime) 0.0))
        (Variables|Custom|ActivateDependant|SetDependantActivationTime 0.0)
        (Development|PrintString (Utilities|String|Append (Utilities|GetObjectName self) ": Resetting Activation time, because Dependencies is Empty")))
      (if (Variables|Custom|Editor|GetEnableSnapping)
        (if (Variables|Custom|ActivateTriggered|GetActivateOnTrigger)
          (if (and (> (Variables|Custom|Editor|GetEditorTriggeredProgress) 0.0) (< (Variables|Custom|Editor|GetEditorDependantProgress) 1.0))
            ;[1 0.05267 0] Für EditorProgress [0-1[ sollte ETP = 0 sein,              Für EditorTriggeredProgress ]0 -1] sollte EP = 1 sein.
            (Development|PrintString "EDITORWARNING: EditorProgress should be 1 for EditorTriggeredProgress to work correctly" true false "(R=1.000000,G=0.047707,B=0.000000,A=1.000000)"))
          (CallFunction|VisualizeDependenciesProgress (Variables|Custom|Editor|GetEditorDependantProgress))
          (CallFunction|VisualizeTriggeredProgress (Variables|Custom|Editor|GetEditorTriggeredProgress))
          (else
            (CallFunction|VisualizeTriggeredProgress (Variables|Custom|Editor|GetEditorDependantProgress))))))))

(fn CheckingDependencies
  (for _array_element (Variables|Custom|ActivateDependant|GetDependencies)
    (if (Variables|/Game/VikingMageProject/Gameplay/Triggers/BP_TriggeredMovingActor.BP_TriggeredMovingActor_C|GetActive _array_element)
      (Math|Integer|IncrementInt (LocalVariables|GetDependenciesCount))))
  (return (LocalVariables|GetDependenciesCount)))

(fn CalcDepProgress
  (if (== (Utilities|Array|Length (Variables|Custom|ActivateDependant|GetDependencies)) 0)
    (return 1.0)
    (else
      (bind _activedependencies (CallFunction|CheckingDependencies))
      (return (/ (Math|Conversions|ToFloat(Integer) _activedependencies) (Math|Conversions|ToFloat(Integer) (Utilities|Array|Length (Variables|Custom|ActivateDependant|GetDependencies))))))))

(fn ActivationTriggered
  (if (Variables|Custom|ActivateTriggered|GetActivateOnTrigger)
    (bind _out_depprogress (CallFunction|CalcDepProgress))
    (Variables|Custom|ActivateTriggered|SetGoingToActive (and (Math|Float|NearlyEqual(Float) _out_depprogress 1.0 1e-06) (not (Variables|Custom|ActivateTriggered|GetGoingToActive))))
    (Actor|Tick|SetActorTickEnabled true)
    (else
      (Development|PrintString "WARNING: Trying to activate an Activatable by trigger that cannot be trigger-activated" true true "(R=1.000000,G=0.006970,B=0.000000,A=1.000000)"))))

(fn AnimateProgress
  (params (Delta :type Float%20%28single-precision%29) (CurrentProgress :type Float%20%28single-precision%29) (TargetProgress :type Float%20%28single-precision%29) (AnimationTime :type Float%20%28single-precision%29))
  (if (== AnimationTime 0.0)
    (return TargetProgress)
    (else
      (LocalVariables|SetCurrentTime (* CurrentProgress AnimationTime))
      (LocalVariables|SetTargetTime (* TargetProgress AnimationTime))
      (if (< (LocalVariables|GetCurrentTime) (LocalVariables|GetTargetTime))
        (LocalVariables|SetCurrentTime (Math|Float|Clamp(Float) (+ (LocalVariables|GetCurrentTime) Delta) 0.0 (LocalVariables|GetTargetTime)))
        (else
          (LocalVariables|SetCurrentTime (Math|Float|Clamp(Float) (- (LocalVariables|GetCurrentTime) Delta) (LocalVariables|GetTargetTime) AnimationTime))))
      (return (/ (LocalVariables|GetCurrentTime) AnimationTime)))))

(fn ResetEditorPosition
  (Variables|Custom|Editor|SetEnableSnapping false)
  (CallFunction|InitializeState))

(fn InitializeState
  (if (or (Variables|Custom|ActivateTriggered|GetActivateOnTrigger) (> (Utilities|Array|Length (Variables|Custom|ActivateDependant|GetDependencies)) 0))
    _
    (else
      (Development|PrintString (Utilities|String|Append "WARNING: " (Utilities|GetObjectName self) " can never be Activated") true true "(R=1.000000,G=0.019096,B=0.000000,A=1.000000)")))
  (bind _output_get (Variables|Custom|ActivateTriggered|SetGoingToActive (Variables|Custom|GetActive)))
  (if _output_get
    (Variables|Custom|ActivateDependant|SetCurrDepProgress 1.0)
    (Variables|Custom|ActivateTriggered|SetCurrTrigProgress 1.0)
    (else
      (bind _out_depprogress (CallFunction|CalcDepProgress))
      (Variables|Custom|ActivateDependant|SetCurrDepProgress _out_depprogress)
      (Variables|Custom|ActivateTriggered|SetCurrTrigProgress 0.0)))
  (if (Variables|Custom|ActivateTriggered|GetActivateOnTrigger)
    (CallFunction|VisualizeDependenciesProgress (Variables|Custom|ActivateDependant|GetCurrDepProgress))
    (CallFunction|VisualizeTriggeredProgress (Variables|Custom|ActivateTriggered|GetCurrTrigProgress))
    (else
      (CallFunction|VisualizeTriggeredProgress (Variables|Custom|ActivateDependant|GetCurrDepProgress)))))

(fn EvaluateActivity
  (bind _currtrigprogress (Variables|Custom|ActivateTriggered|GetCurrTrigProgress))
  (bind _currdepprogress (Variables|Custom|ActivateDependant|GetCurrDepProgress))
  (if (Variables|Custom|ActivateTriggered|GetActivateOnTrigger)
    (if (== (Variables|Custom|ActivateDependant|GetCurrDepProgress) 1.0)
      (if (Variables|Custom|ActivateTriggered|GetToggleStateImmediately)
        ;[1 1 1] Immediate switching
        (if (Math|Boolean|NotEqual(Boolean) (Variables|Custom|ActivateTriggered|GetGoingToActive) (Variables|Custom|GetActive))
          (Variables|Custom|SetActive (Variables|Custom|ActivateTriggered|GetGoingToActive))
          (Default|CallActivityChanged))
        (else
          ;[1 1 1] Latent switching
          (if (== _currtrigprogress 1.0)
            (Variables|Custom|SetActive true)
            (Default|CallActivityChanged :!label _label)
            (Actor|Tick|SetActorTickEnabled false)
            (elif (== _currtrigprogress 0.0)
              (Variables|Custom|SetActive false)
              (goto _label))))))
    (elif (== _currdepprogress 1.0)
      (Variables|Custom|SetActive true)
      (Default|CallActivityChanged :!label _label_2)
      (Actor|Tick|SetActorTickEnabled false)
      (elif (== _currdepprogress 0.0)
        (Variables|Custom|SetActive false)
        (goto _label_2)))))