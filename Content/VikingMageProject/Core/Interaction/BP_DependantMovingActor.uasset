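; BP_DependantMovingActor is an interaction actor that moves to reflect the progress of its dependencies.
; Its VisualizeDependenciesProgress event linearly interpolates between InactivePosition and ActivePosition by the incoming Progress value and sets the root component's world location, without sweep or teleport.
; It has no logic of its own on BeginPlay, overlap or construction, so movement depends entirely on that event being called.
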(event EventBeginPlay
  (|CallParentFunction) ; This node is disabled and will not be called.\nDrag off pins to build functionality.
)

(event Collision|EventActorBeginOverlap
  (params (OtherActor :type Actor%20Object%20Reference))
  (|CallParentFunction OtherActor) ; This node is disabled and will not be called.\nDrag off pins to build functionality.
)

(event EventVisualizeDependenciesProgress
  (params (Progress :type Float%20%28single-precision%29))
  (Transformation|SetWorldLocation (Variables|Default|GetDefaultSceneRoot) (Math|Vector|Lerp(Vector) (Variables|Custom|GetInactivePosition) (Variables|Custom|GetActivePosition) Progress) false false))

(fn ConstructionScript
  (|CallParentFunction))