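; Burnable world actor that ignites from fire damage, burns progressively, and can burn up into ash before being destroyed.
; Burn progress and fire origin reach the mesh material through custom primitive data.
; While burning, a box can spread fire damage to overlapping actors on contact or at intervals.
; Niagara fire and ash effects use the mesh as source and take wind from Ultra Dynamic Weather.
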(event OnComponentBeginOverlap(Box)
  (params (OverlappedComponent :type Primitive%20Component%20Object%20Reference) (OtherActor :type Actor%20Object%20Reference) (OtherComp :type Primitive%20Component%20Object%20Reference) (OtherBodyIndex :type Integer) (bFromSweep :type Boolean) (SweepResult :type Hit%20Result%20Structure%20%28by%20ref%29))
  ;[1 1 1] Overlap Box Component
  (if (and (Variables|DamageDealing|GetShouldDealBurnDamage) (!= OtherActor self))
    (if (Variables|DamageDealing|GetDmgOverTime)
      (Utilities|Array|Add (Variables|Default|GetOtherActors) OtherActor)
      (else
        (Game|Damage|ApplyDamage OtherActor (Variables|DamageDealing|GetContactDamage) 0 0 "/Game/VikingMageProject/Core/Characters/Player/Spells/BP_FireDamage.BP_FireDamage_C")))))

(event OnComponentEndOverlap(Box)
  (params (OverlappedComponent :type Primitive%20Component%20Object%20Reference) (OtherActor :type Actor%20Object%20Reference) (OtherComp :type Primitive%20Component%20Object%20Reference) (OtherBodyIndex :type Integer))
  ;[1 1 1] Overlap Box Component
  (Utilities|Array|RemoveItem (Variables|Default|GetotherActors) OtherActor))

(event Custom|BurnHandling)

(event EventBeginPlay
  (bind _returnvalue (Actor|GetActorOfClass "/Game/UltraDynamicSky/Blueprints/Ultra_Dynamic_Weather.Ultra_Dynamic_Weather_C"))
  (Variables|BurnEffect|SetUltraDynamicWeather _returnvalue)
  (Variables|BurnEffect|SetMaxBurnProcess (+ (Math|Conversions|ToFloat(Byte) (Variables|BurnEffect|GetMaxBurnState)) 1.0))
  (bind _output_get (Variables|BurnEffect|SetBurnProcess (Math|Float|Clamp(Float) (Variables|BurnEffect|GetBurnProcess) 0.0 (Variables|BurnEffect|GetMaxBurnProcess))))
  (CallFunction|SetBurnMaterialValues _output_get (Transformation|GetActorLocation))
  (CallFunction|InitParticleEffects)
  (if (not (Variables|BurnEffect|GetIsBurning))
    (Collision|SetCollisionEnabled (Variables|Default|GetBox) "NoCollision")))

(event Game|Damage|EventAnyDamage
  (params (Damage :type Float%20%28single-precision%29) (DamageType :type Damage%20Type%20Object%20Reference) (InstigatedBy :type Controller%20Object%20Reference) (DamageCauser :type Actor%20Object%20Reference))
  (bind _returnvalue (Transformation|GetActorLocation DamageCauser))
  (Development|PrintString "Hello")
  (Utilities|Casting|CastToBP_FireDamage DamageType)
  (Components|Activation|SetActive (Variables|Default|GetParticles) true false)
  (if (not (Variables|BurnEffect|GetIsBurning))
    (Rendering|Material|SetCustomPrimitiveDataVector4 (Variables|Default|GetStaticMesh) (Variables|BurnEffect|GetFireStartPos_CustomPrimitiveIndex) (Math|Vector4|MakeVector4 (.x _returnvalue) (.y _returnvalue) (.z _returnvalue) 1.0))
    (CallFunction|IncreaseBurnProcess (Variables|BurnEffect|GetFirstHitProgress))
    (Collision|SetCollisionEnabled (Variables|Default|GetBox) "QueryAndPhysics")
    (else
      (CallFunction|IncreaseBurnProcess (Variables|BurnEffect|GetHitProgress))))
  (Variables|BurnEffect|SetIsBurning true))

(event EventTick
  (params (DeltaSeconds :type Float%20%28single-precision%29))
  (if (Variables|BurnEffect|GetIsBurning)
    (CallFunction|DealDmgOverTime DeltaSeconds)
    (CallFunction|UpdateParticleWindEffects (Variables|Default|GetParticles))
    (bind _burnprocess (CallFunction|IncreaseBurnProcess (* DeltaSeconds (Variables|BurnEffect|GetBurnSpeed))))
    (Rendering|Material|SetCustomPrimitiveDataFloat (Variables|Default|GetStaticMesh) (Variables|BurnEffect|GetFireProcess_CustomPrimitveIndex) _burnprocess)
    (if (and (>= (Variables|BurnEffect|GetBurnProcess) (Variables|BurnEffect|GetMaxBurnProcess)) (Variables|BurnEffect|GetCanBeDestroyed))
      (CallFunction|PrepareDestruction)
      (Utilities|FlowControl|Delay (Variables|BurnEffect|GetTimeBeforeActorDestruction))
      (Actor|DestroyActor))))

(fn ConstructionScript)

(fn IncreaseBurnProcess
  (params (Progress :type Float%20%28single-precision%29))
  (bind _output_get (Variables|BurnEffect|SetBurnProcess (Math|Float|Min(Float) (+ (Variables|BurnEffect|GetBurnProcess) Progress) (Variables|BurnEffect|GetMaxBurnProcess))))
  (return _output_get))

(fn InitParticleEffects
  (bind _particles (Variables|Default|GetParticles))
  (Utilities|FlowControl|Sequence
    (:then_0
      ;[1 1 1] Fire Particles
      (Class|NiagaraFunctionLibrary|OverrideSystemUserVariableStaticMeshComponent _particles "" (Variables|Default|GetStaticMesh))
      (CallFunction|UpdateParticleWindEffects (Variables|Default|GetParticles))
      (Components|Activation|SetActive _particles (Variables|BurnEffect|GetIsBurning) false))
    (:then_1
      ;[1 1 1] AshParticles
      (Class|NiagaraFunctionLibrary|OverrideSystemUserVariableStaticMeshComponent (Variables|Default|GetAshParticles) "" (Variables|Default|GetStaticMesh)))))

(fn UpdateParticleWindEffects
  (params (ParticleSystem :type Niagara%20Component%20Object%20Reference))
  (bind _ultradynamicweather (Variables|BurnEffect|GetUltraDynamicWeather))
  (Utilities|IsValid _ultradynamicweather
    (:Is%20Valid
      (Niagara|SetNiagaraVariable(Vector3) ParticleSystem "WindSpeed" (Class|KismetMathLibrary|CreateVectorfromYawPitch (Variables|/Game/UltraDynamicSky/Blueprints/Ultra_Dynamic_Weather.Ultra_Dynamic_Weather_C|GetCurrent%20Wind%20Direction _ultradynamicweather) 0.0 1.0))
      (Niagara|SetNiagaraVariable(Float) ParticleSystem "WindSpeedScale" (* (Variables|/Game/UltraDynamicSky/Blueprints/Ultra_Dynamic_Weather.Ultra_Dynamic_Weather_C|GetCurrent%20Wind%20Intensity _ultradynamicweather) (Variables|BurnEffect|GetWindScaleMultiplier))))))

(fn DealDmgOverTime
  (params (DeltaSeconds :type Float%20%28single-precision%29))
  (Utilities|FlowControl|Sequence
    (:then_0
      (if (and (and (<= (Variables|DamageDealing|GetdmgSecondsLeft) 0.0) (Variables|DamageDealing|GetDmgOverTime)) (> (Utilities|Array|Length (Variables|Default|GetotherActors)) 0))
        (for _array_element (Variables|Default|GetotherActors)
          (Game|Damage|ApplyDamage _array_element (Variables|DamageDealing|GetContactDamage) 0 0 "/Game/VikingMageProject/Core/Characters/Player/Spells/BP_FireDamage.BP_FireDamage_C"))
        (Variables|DamageDealing|SetdmgSecondsLeft (Variables|DamageDealing|GetDmgFrequency))))
    (:then_1
      (if (> (Variables|DamageDealing|GetdmgSecondsLeft) 0.0)
        (Variables|DamageDealing|SetdmgSecondsLeft (- (Variables|DamageDealing|GetdmgSecondsLeft) DeltaSeconds))))))

(fn SetBurnMaterialValues
  (params (BurnProcess :type Float%20%28single-precision%29) (FireStartPosition :type Vector))
  (bind _staticmesh (Variables|Default|GetStaticMesh))
  (Rendering|Material|SetCustomPrimitiveDataFloat _staticmesh 0 BurnProcess)
  (Rendering|Material|SetCustomPrimitiveDataVector4 _staticmesh 1 (Math|Vector4|MakeVector4 (.x FireStartPosition) (.y FireStartPosition) (.z FireStartPosition) 1.0)))

(fn PrepareDestruction
  (bind _ashparticles (Variables|Default|GetAshParticles))
  ;[1 1 1] Initialize
  (Components|Activation|SetActive _ashparticles true false)
  (CallFunction|UpdateParticleWindEffects _ashparticles)
  ;[1 1 1] Hide Mesh
  (Rendering|SetVisibility (Variables|Default|GetStaticMesh) false false)
  (Collision|SetCollisionEnabled (Variables|Default|GetStaticMesh) "NoCollision")
  ;[1 1 1] Disable Fire Particles
  (Components|Activation|SetActive (Variables|Default|GetParticles) false false)
  ;[1 1 1] Clean Up Damage Dealing
  (Collision|SetCollisionEnabled (Variables|Default|GetBox) "NoCollision")
  (Utilities|Array|Clear (Variables|Default|GetOtherActors)))