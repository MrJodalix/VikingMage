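; Destroyable world actor that records its destruction in the player's save game.
; On Destroyed, it checks IsNetStartupActor so that only actors loaded with the level are saved, not runtime spawns.
; SaveAsDestroyedActor passes itself and the current level name to PlayerSaveGame on BP_GameInstance, then prints a debug message.
; RemoveFromInstancedActors is an empty stub.
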(event EventDestroyed
  (if (Class|ActorBlueprintFunctionLibrary|IsNetStatupActor self)
    (CallFunction|SaveasDestroyedActor)))

(fn ConstructionScript)

(fn SaveasDestroyedActor
  (bind _returnvalue (Game|GetCurrentLevelName true))
  (Default|SaveDestroyedActor (Variables|/Game/VikingMageProject/Core/Characters/Player/BP_GameInstance.BP_GameInstance_C|GetPlayerSaveGame (.AsBP%20Game%20Instance (Utilities|Casting|CastToBP_GameInstance (Game|GetGameInstance)))) self _returnvalue)
  (Development|PrintString (Utilities|String|Append "Saved To Level: " _returnvalue)))

(fn RemovefromInstancedActors)