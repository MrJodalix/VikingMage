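; BP_DestructiveEnvironment is an actor that attaches to a parent actor and makes it destructible through a Health value.
; Any damage lowers Health, unless OnlyDamagedByType is set and the damage type's class differs.
; At zero Health it destroys the parent, and a binding to the parent's OnDestroyed made at BeginPlay removes this actor too.
; Non-lethal hits print a debug string and call DamagedEnvironment.
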(event Custom|Die
  (Actor|DestroyActor (Actor|GetAttachParentActor)))

(event Custom|Destroy
  (params (DestroyedActor :type Actor%20Object%20Reference))
  ;[1 1 1] Destroy this too, when parent is destroyed
  (Actor|DestroyActor))

(event Game|Damage|EventAnyDamage
  (params (Damage :type Float%20%28single-precision%29) (DamageType :type Damage%20Type%20Object%20Reference) (InstigatedBy :type Controller%20Object%20Reference) (DamageCauser :type Actor%20Object%20Reference))
  (if (!= (Variables|Default|GetOnlyDamagedByType) 0)
    (if (== (Variables|Default|GetOnlyDamagedByType) (Utilities|GetClass DamageType))
      (Variables|Default|SetHealth (- (Variables|Default|GetHealth) Damage))
      (if (<= (Variables|Default|GetHealth) 0.0) :!label _label
        (CallFunction|Die)
        (else
          (Development|PrintString "Damage no death" true true "(R=1.000000,G=0.029223,B=0.000000,A=1.000000)")
          (Default|CallDamagedEnvironment))))
    (else
      (Variables|Default|SetHealth (- (Variables|Default|GetHealth) Damage))
      (goto _label))))

(event EventBeginPlay
  ;[1 1 1] Destroy this too, when parent is destroyed
  (Game|BindEventtoOnDestroyed (Actor|GetAttachParentActor) (delegate Custom|Destroy)))

(fn ConstructionScript)