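; BP_Information is a world trigger actor that shows an on-screen info message when BP_PlayerCharacter overlaps it.
; On overlap begin it creates a WBP_Info widget with its text, applies alignment, color and font, then adds it to the viewport after a delay.
; On overlap end it removes the widget and, if DestroyActor is set, destroys itself.
; Debug prints report creation and destruction.
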(event Collision|EventActorBeginOverlap
  (params (OtherActor :type Actor%20Object%20Reference))
  (Utilities|Casting|CastToBP_PlayerCharacter OtherActor)
  (bind _returnvalue (UserInterface|CreateWidget "/Game/VikingMageProject/Core/UI/Infos/WBP_Info.WBP_Info_C" 0 (Variables|Default|GetText)))
  (bind _output_get (Variables|Default|SetWidget _returnvalue))
  (Default|ChangeTextAlignment _output_get (Variables|Default|GetTextHeightOverActor))
  (Default|ChangeFontColor (Variables|Default|GetWidget) (Variables|Default|GetFontColor))
  (Default|ChangeFont (Variables|Default|GetWidget) (Variables|Default|GetSlate%20Font%20Info))
  (Utilities|FlowControl|Delay (Variables|Default|GetTimeUntilInfoShown))
  (UserInterface|Viewport|AddtoViewport (Variables|Default|GetWidget) 0)
  (Widget|SetVisibility (Variables|Default|GetWidget) "HitTestInvisible")
  (Development|PrintString "Information Created" true true "(R=1.000000,G=0.000000,B=0.065193,A=1.000000)"))

(event Collision|EventActorEndOverlap
  (params (OtherActor :type Actor%20Object%20Reference))
  (Utilities|Casting|CastToBP_PlayerCharacter OtherActor)
  (bind _widget (Variables|Default|GetWidget)
    (:then
      (Widget|RemovefromParent _widget)
      (if (Variables|Default|GetDestroyActor)
        (Actor|DestroyActor)
        (Development|PrintString "Destroyed Info" true true "(R=1.000000,G=0.000000,B=0.110300,A=1.000000)")))
    (:else)))

(fn ConstructionScript)