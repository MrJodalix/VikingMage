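; BP_DamageAreaEffect is a box-trigger area that damages actors inside it, either once on entry or periodically while they stay.
; With DamageOverTime on, overlapping actors are tracked in OtherActors and removed when they leave.
; Tick counts DmgSecondsLeft down and, when it expires, damages every tracked actor and resets it to DmgEachSeconds.
; Otherwise, each begin overlap applies Damage immediately.
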(event OnComponentBeginOverlap(Box)
  (params (OverlappedComponent :type Primitive%20Component%20Object%20Reference) (OtherActor :type Actor%20Object%20Reference) (OtherComp :type Primitive%20Component%20Object%20Reference) (OtherBodyIndex :type Integer) (bFromSweep :type Boolean) (SweepResult :type Hit%20Result%20Structure%20%28by%20ref%29))
  (if (Variables|Default|GetdamageOverTime)
    (Utilities|Array|Add (Variables|Default|GetotherActors) OtherActor)
    (else
      (Game|Damage|ApplyDamage OtherActor (Variables|Default|Getdamage) 0 0))))

(event OnComponentEndOverlap(Box)
  (params (OverlappedComponent :type Primitive%20Component%20Object%20Reference) (OtherActor :type Actor%20Object%20Reference) (OtherComp :type Primitive%20Component%20Object%20Reference) (OtherBodyIndex :type Integer))
  (Utilities|Array|RemoveItem (Variables|Default|GetotherActors) OtherActor))

(event EventBeginPlay)

(event EventTick
  (params (DeltaSeconds :type Float%20%28single-precision%29))
  (Utilities|FlowControl|Sequence
    (:then_0
      (if (and (and (<= (Variables|Default|GetdmgSecondsLeft) 0.0) (Variables|Default|GetdamageOverTime)) (> (Utilities|Array|Length (Variables|Default|GetotherActors)) 0))
        (for _array_element (Variables|Default|GetotherActors)
          (Game|Damage|ApplyDamage _array_element (Variables|Default|Getdamage) 0 0))
        (Variables|Default|SetdmgSecondsLeft (Variables|Default|GetdmgEachSeconds))))
    (:then_1
      (if (> (Variables|Default|GetdmgSecondsLeft) 0.0)
        (Variables|Default|SetdmgSecondsLeft (- (Variables|Default|GetdmgSecondsLeft) DeltaSeconds))))))

(fn ConstructionScript)