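; BP_MovementPathSpline is a world actor holding a spline, apparently a movement path, that it flattens onto a horizontal plane at BeginPlay.
; A first pass caches each point's world location and tangent, replacing height with the root component's Z and zeroing the tangent's Z.
; A second pass writes the cached values back to the spline in world space, preserving the horizontal positions and tangent components.
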(event EventBeginPlay
  (bind _spline (Variables|Default|GetSpline))
  (for _index (range 0 (- (Spline|GetNumberOfSplinePoints (Variables|Default|GetSpline)) 1))
    (Utilities|Array|Add (Variables|Default|GetNewSplinePointInfo) (Utilities|Struct|MakeSSplinePointInfo (Math|Vector|MakeVector (.X (Math|Vector|BreakVector (.Location (Spline|GetLocationandTangentatSplinePoint (Variables|Default|GetSpline) _index "World")))) (.Y (Math|Vector|BreakVector (.Location (Spline|GetLocationandTangentatSplinePoint (Variables|Default|GetSpline) _index "World")))) (.z (Transformation|GetWorldLocation (Variables|Default|GetDefaultSceneRoot)))) (Math|Vector|MakeVector (.X (Math|Vector|BreakVector (.Tangent (Spline|GetLocationandTangentatSplinePoint (Variables|Default|GetSpline) _index "World")))) (.Y (Math|Vector|BreakVector (.Tangent (Spline|GetLocationandTangentatSplinePoint (Variables|Default|GetSpline) _index "World")))) 0.0))))
  (for (_array_element _array_index) (Variables|Default|GetNewSplinePointInfo)
    (Spline|SetLocationatSplinePoint _spline _array_index (.pointposition _array_element) "World" true)
    (Spline|SetTangentatSplinePoint _spline _array_index (.pointtangent _array_element) "World" true)))

(event Collision|EventActorBeginOverlap
  (params (OtherActor :type Actor%20Object%20Reference)))

(event EventTick
  (params (DeltaSeconds :type Float%20%28single-precision%29)))

(fn ConstructionScript)