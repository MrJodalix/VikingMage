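; Trigger zone that lets the player character switch between two movement splines, A and B.
; Sphere overlap registers the zone on the player and shows a styled WBP_Info transition prompt, both cleared on exit.
; With AutoSwitch on, entry immediately calls the player's SwitchSpline.
; Toggle swaps the player's spline and prompt text, while ToggleCheckButtonUsage gates it so button presses only work in manual zones.
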(event OnComponentEndOverlap(Sphere)
  (params (OverlappedComponent :type Primitive%20Component%20Object%20Reference) (OtherActor :type Actor%20Object%20Reference) (OtherComp :type Primitive%20Component%20Object%20Reference) (OtherBodyIndex :type Integer))
  (bind _widgetinfotext (Variables|Custom|TransitionText|GetWidgetInfoText))
  (bind _asbp_player_character (Utilities|Casting|CastToBP_PlayerCharacter OtherActor))
  (Variables|/Game/VikingMageProject/Core/Characters/Player/BP_PlayerCharacter.BP_PlayerCharacter_C|SetSplineTransitionRef _asbp_player_character 0)
  (Variables|Custom|SetisOverlappingPlayer false)
  (Utilities|IsValid _widgetinfotext
    (:Is%20Valid
      (Widget|RemovefromParent _widgetinfotext)
      (Variables|Custom|SetplayerBPRef 0))))

(event OnComponentBeginOverlap(Sphere)
  (params (OverlappedComponent :type Primitive%20Component%20Object%20Reference) (OtherActor :type Actor%20Object%20Reference) (OtherComp :type Primitive%20Component%20Object%20Reference) (OtherBodyIndex :type Integer) (bFromSweep :type Boolean) (SweepResult :type Hit%20Result%20Structure%20%28by%20ref%29))
  (bind _returnvalue (Game|GetPlayerController 0))
  (bind _asbp_player_character (Utilities|Casting|CastToBP_PlayerCharacter OtherActor))
  (Variables|Custom|SetisOverlappingPlayer true)
  (bind _output_get (Variables|Custom|SetplayerBPRef _asbp_player_character))
  (Variables|/Game/VikingMageProject/Core/Characters/Player/BP_PlayerCharacter.BP_PlayerCharacter_C|SetSplineTransitionRef _output_get self)
  (Utilities|FlowControl|Sequence
    (:then_0
      ;[1 1 1] Show Text
      (if (and (== (Variables|/Game/VikingMageProject/Core/Characters/BP_CharacterCustom.BP_CharacterCustom_C|GetMovementSpline _asbp_player_character) (Variables|Custom|GetmovementSplineA)) (not (Variables|Custom|GetAutoSwitch)))
        (bind _returnvalue_2 (UserInterface|CreateWidget "/Game/VikingMageProject/Core/UI/Infos/WBP_Info.WBP_Info_C" _returnvalue (Variables|Custom|TransitionText|GetTextTransitToMSB)))
        (bind _output_get_2 (Variables|Custom|TransitionText|SetWidgetInfoText _returnvalue_2))
        (else
          (bind _returnvalue_3 (UserInterface|CreateWidget "/Game/VikingMageProject/Core/UI/Infos/WBP_Info.WBP_Info_C" _returnvalue (Variables|Custom|TransitionText|GetTextTransitToMSA)))
          (bind _output_get_3 (Variables|Custom|TransitionText|SetWidgetInfoText _returnvalue_3))))
      (Default|ChangeTextAlignment _output_get_2 (Variables|Custom|TransitionText|GetTextYAlignment))
      (Default|ChangeFontColor (Variables|Custom|TransitionText|GetWidgetInfoText) (Variables|Custom|TransitionText|GetTextColor))
      (Default|ChangeFont (Variables|Custom|TransitionText|GetWidgetInfoText) (Variables|Custom|TransitionText|GetSlate%20Font%20Info))
      (UserInterface|Viewport|AddtoViewport (Variables|Custom|TransitionText|GetWidgetInfoText) 0))
    (:then_1
      (if (and (Variables|Custom|GetAutoSwitch) (Utilities|IsValid (Variables|Custom|GetplayerBPRef)))
        (Default|SwitchSpline (Variables|Custom|GetplayerBPRef) false)))))

(event EventBeginPlay)

(event EventTick
  (params (DeltaSeconds :type Float%20%28single-precision%29)))

(fn ConstructionScript)

(fn Toggle
  (bind _playerbpref (Variables|Custom|GetplayerBPRef))
  (if (== (Variables|/Game/VikingMageProject/Core/Characters/BP_CharacterCustom.BP_CharacterCustom_C|GetMovementSpline (Variables|Custom|GetplayerBPRef)) (Variables|Custom|GetmovementSplineA))
    (Variables|/Game/VikingMageProject/Core/Characters/BP_CharacterCustom.BP_CharacterCustom_C|SetMovementSpline _playerbpref (Variables|Custom|GetmovementSplineB))
    (Variables|/Game/VikingMageProject/Core/UI/Infos/WBP_Info.WBP_Info_C|SetText (Variables|Custom|TransitionText|GetWidgetInfoText) (Variables|Custom|TransitionText|GetTextTransitToMSA))
    (else
      (Variables|/Game/VikingMageProject/Core/Characters/BP_CharacterCustom.BP_CharacterCustom_C|SetMovementSpline _playerbpref (Variables|Custom|GetmovementSplineA))
      (Variables|/Game/VikingMageProject/Core/UI/Infos/WBP_Info.WBP_Info_C|SetText (Variables|Custom|TransitionText|GetWidgetInfoText) (Variables|Custom|TransitionText|GetTextTransitToMSB)))))

(fn ToggleCheckButtonUsage
  (params (ButtonUsed :type Boolean))
  (if (Math|Boolean|NotEqual(Boolean) ButtonUsed (Variables|Custom|GetAutoSwitch))
    (CallFunction|Toggle)))