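; Checkpoint actor that sets the player's respawn point on activation-capsule overlap and opens a player HUD menu on interaction.
; Until activated, its rune stone glows brighter through a dynamic material as the player nears, using curve-shaped horizontal distance within a proximity capsule.
; First activation locks full glow and spawns a lightning effect.
; Rune meshes show or hide according to the spells stored in the HUD's checkpoint widget.
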(event OnComponentBeginOverlap(ActivationCapsule)
  (params (OverlappedComponent :type Primitive%20Component%20Object%20Reference) (OtherActor :type Actor%20Object%20Reference) (OtherComp :type Primitive%20Component%20Object%20Reference) (OtherBodyIndex :type Integer) (bFromSweep :type Boolean) (SweepResult :type Hit%20Result%20Structure%20%28by%20ref%29))
  (Utilities|Casting|CastToBP_PlayerCharacter OtherActor)
  (if (Variables|Custom|GetIsActive)
    (CallFunction|SetRespawnPoint)
    (else
      (CallFunction|Activate)
      (Development|PrintString "Activating Checkpoint"))))

(event OnComponentBeginOverlap(ProximityCapsule)
  (params (OverlappedComponent :type Primitive%20Component%20Object%20Reference) (OtherActor :type Actor%20Object%20Reference) (OtherComp :type Primitive%20Component%20Object%20Reference) (OtherBodyIndex :type Integer) (bFromSweep :type Boolean) (SweepResult :type Hit%20Result%20Structure%20%28by%20ref%29))
  (Utilities|Casting|CastToBP_PlayerCharacter OtherActor)
  (if (not (Variables|Custom|GetIsActive))
    (Variables|Custom|SetIsPlayerNearby true)))

(event OnComponentEndOverlap(ProximityCapsule)
  (params (OverlappedComponent :type Primitive%20Component%20Object%20Reference) (OtherActor :type Actor%20Object%20Reference) (OtherComp :type Primitive%20Component%20Object%20Reference) (OtherBodyIndex :type Integer))
  (Utilities|Casting|CastToBP_PlayerCharacter OtherActor)
  (Variables|Custom|SetIsPlayerNearby false)
  (if (Variables|Custom|GetIsActive)
    (Components|DestroyComponent (Variables|Default|GetProximityCapsule))))

(event Custom|SpellsInCheckpointUpdated
  (params (Spells :type Array%20of%20BP%20Spell%20Class%20References))
  (for _array_element (Variables|Custom|GetRuneMeshes)
    (Utilities|IsValid (.runemesh _array_element)
      (:Is%20Valid
        (Rendering|SetVisibility (Variables|/Script/Engine.StaticMeshActor|GetStaticMeshComponent (.runemesh _array_element)) (Utilities|Array|ContainsItem Spells (.spell _array_element)) false)))))

(event EventTick
  (params (DeltaSeconds :type Float%20%28single-precision%29))
  (bind _returnvalue (Game|GetPlayerCharacter 0))
  (bind _proximitycapsule (Variables|Default|GetProximityCapsule))
  (bind _returnvalue_2 (Transformation|GetWorldLocation _proximitycapsule))
  (bind _returnvalue_3 (Transformation|GetActorLocation _returnvalue))
  (if (and (Utilities|IsValid (Variables|Custom|GetRuneStoneMaterial)) (Variables|Custom|GetIsPlayerNearby))
    (Rendering|Material|SetScalarParameterValue (Variables|Custom|GetRuneStoneMaterial) "Emission" (Math|Float|Lerp (Variables|Custom|GetMinGlow) (Variables|Custom|GetMaxGlow) (Math|Curves|GetFloatValue (Variables|Custom|GetGlowupCurve) (+ (* -1 (/ (Math|Vector|VectorLength (- (Math|Vector|MakeVector (.x _returnvalue_3) (.y _returnvalue_3) 0.0) (Math|Vector|MakeVector (.x _returnvalue_2) (.y _returnvalue_2) 0.0))) (Components|Capsule|GetScaledCapsuleRadius _proximitycapsule))) 1.0))) :!class /Script/Engine.MaterialInstanceDynamic)))

(event EventBeginPlay
  (bind _runestone (Variables|Custom|GetRuneStone))
  (Utilities|IsValid _runestone
    (:Is%20Valid
      (bind _returnvalue (Rendering|Material|CreateDynamicMaterialInstance (Variables|/Script/Engine.StaticMeshActor|GetStaticMeshComponent _runestone) 1 0 "None" :!class /Script/Engine.PrimitiveComponent))
      (bind _output_get (Variables|Custom|SetRuneStoneMaterial _returnvalue))
      (Rendering|Material|SetScalarParameterValue _output_get "Emission" (Variables|Custom|GetMinGlow) :!class /Script/Engine.MaterialInstanceDynamic)
      (Rendering|Material|SetVectorParameterValue _output_get "Color" (Variables|Custom|GetGlowColor) :!class /Script/Engine.MaterialInstanceDynamic))
    (:Is%20Not%20Valid
      _))
  ;[1 1 1] Vielleicht reicht auch ohne Delay
  (Utilities|FlowControl|Delay 0.02)
  (bind _output_get_2 (Variables|Custom|SetWBP%20Check%20Point (Variables|/Game/VikingMageProject/Core/UI/WBP_PlayerHUD.WBP_PlayerHUD_C|GetWBP_CheckPoint (Variables|/Game/VikingMageProject/Core/Characters/Player/BP_PlayerCharacter.BP_PlayerCharacter_C|GetWBP_PlayerHUD (.AsBP%20Player%20Character (Utilities|Casting|CastToBP_PlayerCharacter (Game|GetPlayerCharacter 0)))))))
  (CallFunction|SpellsinCheckpointUpdated (Variables|/Game/VikingMageProject/Core/UI/CheckPoint/WBP_CheckPoint.WBP_CheckPoint_C|GetStoredSpells _output_get_2))
  (EventDispatchers|AssignStoredSpellsChanged (Variables|Custom|GetWBP%20Check%20Point) (EventDispatchers|CreateEvent :!event Custom|SpellsInCheckpointUpdated)))

(fn ConstructionScript
  (bind _activationcapsule (Variables|Default|GetActivationCapsule))
  (bind (_outradius _outhalfheight) (Class|CapsuleComponent|GetUnscaledCapsuleSize _activationcapsule))
  (Components|Capsule|SetCapsuleSize (Variables|Default|GetProximityCapsule) (* (Variables|Custom|GetRadiusFactor) _outradius) (* _outhalfheight (* 2 (Variables|Custom|GetHeightFactor))) true)
  (bind _returnvalue (Rendering|Material|CreateDynamicMaterialInstance (Variables|/Script/Engine.StaticMeshActor|GetStaticMeshComponent (Variables|Custom|GetRuneStone)) 1 0 "None" :!class /Script/Engine.PrimitiveComponent))
  (bind _output_get (Variables|Custom|SetRuneStoneMaterial _returnvalue))
  (Rendering|Material|SetScalarParameterValue _output_get "Emission" (Variables|Custom|GetMinGlow) :!class /Script/Engine.MaterialInstanceDynamic)
  (Rendering|Material|SetVectorParameterValue _output_get "Color" (Variables|Custom|GetGlowColor) :!class /Script/Engine.MaterialInstanceDynamic))

(fn Activate
  (bind _returnvalue (Math|Float|MakeLiteralFloat 0.61))
  (bind _runestone (Variables|Custom|GetRuneStone))
  (bind _runestonematerial (Variables|Custom|GetRuneStoneMaterial))
  (Variables|Custom|SetIsActive true)
  (Variables|Custom|SetIsPlayerNearby false)
  (Utilities|IsValid _runestonematerial
    (:Is%20Valid
      (Rendering|Material|SetScalarParameterValue _runestonematerial "Emission" (Variables|Custom|GetMaxGlow) :!class /Script/Engine.MaterialInstanceDynamic))
    (:Is%20Not%20Valid
      _))
  (Utilities|IsValid _runestone
    (:Is%20Valid
      (Effects|SpawnEmitteratLocation "/Game/Luos8Elements/Particles/Lightning/Par_4E_LightningStrike_01.Par_4E_LightningStrike_01" (Transformation|GetWorldLocation (Variables|/Script/Engine.Actor|GetRootComponent _runestone)) "0, 0, 0" (Math|Vector|MakeVector _returnvalue _returnvalue _returnvalue)))
    (:Is%20Not%20Valid
      _))
  (CallFunction|SetRespawnPoint))

(fn SetRespawnPoint
  (Default|SetNewRespawnInfo (.AsBP%20Player%20Character (Utilities|Casting|CastToBP_PlayerCharacter (Game|GetPlayerCharacter 0))) (Variables|Custom|GetRespawnPosition)))

(fn Interact
  (params (Interactor :type BP%20Player%20Character%20Object%20Reference))
  ;[1 1 1] CheckPoint Menü öffnen
  (Default|TriggerMenu (Variables|/Game/VikingMageProject/Core/Characters/Player/BP_PlayerCharacter.BP_PlayerCharacter_C|GetWBP_PlayerHUD (.AsBP%20Player%20Character (Utilities|Casting|CastToBP_PlayerCharacter (Game|GetPlayerCharacter 0)))) "NewEnumerator3" false)
  (return true))