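; Quest log component that tracks active and completed quests and the currently pursued quest.
; Gameplay events for locations, kills, interactions, dialog choices and collected items are forwarded to every active quest, queuing completed ones.
; A shared update then refreshes the objectives UI, moves queued quests to the completed list and picks a new pursued quest if needed.
; Quests are added as per-log instances, with queries for quest and objective state.
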(event Custom|EnemyKilled
  (params (Enemy :type Actor%20Object%20Reference))
  (for _array_element (Variables|Default|GetActiveQuests)
    (Class|QuestAsset|EnemyKilled _array_element Enemy)
    (Development|PrintString (Utilities|String|Append "Is Quest " (Utilities|GetDisplayName _array_element) " complete: " (Utilities|String|ToString(Boolean) (Variables|/Script/QuestAsset.QuestAsset|GetIsComplete _array_element))) true true "(R=0.915362,G=1.000000,B=0.000000,A=1.000000)" 5.0)
    (if (Variables|/Script/QuestAsset.QuestAsset|GetIsComplete _array_element)
      (Utilities|Array|Add (Variables|Default|GetToBeMoved) _array_element)))
  (CallFunction|UpdateActiveQuests))

(event Custom|ActorInteractedWith
  (params (Actor :type Actor%20Object%20Reference))
  (for _array_element (Variables|Default|GetActiveQuests)
    (Class|QuestAsset|Interactedwith _array_element Actor)
    (if (Variables|/Script/QuestAsset.QuestAsset|GetIsComplete _array_element)
      (Utilities|Array|Add (Variables|Default|GetToBeMoved) _array_element)))
  (CallFunction|UpdateActiveQuests))

(event Custom|LocationReached
  (params (LocationReached :type BP%20Location%20Marker%20Object%20Reference))
  (for _array_element (Variables|Default|GetActiveQuests)
    (Class|QuestAsset|LocationVisited _array_element LocationReached)
    (if (Variables|/Script/QuestAsset.QuestAsset|GetIsComplete _array_element)
      (Utilities|Array|Add (Variables|Default|GetToBeMoved) _array_element)))
  (CallFunction|UpdateActiveQuests))

(event Custom|ItemCollected
  (params (ItemID :type Integer) (ItemAmount :type Integer))
  (for _array_element (Variables|Default|GetActiveQuests)
    (Class|QuestAsset|ItemCollected _array_element ItemID ItemAmount)
    (if (Variables|/Script/QuestAsset.QuestAsset|GetIsComplete _array_element)
      (Utilities|Array|Add (Variables|Default|GetToBeMoved) _array_element)))
  (CallFunction|UpdateActiveQuests))

(event Custom|DialogOptionChosen
  (params (InteractionID :type Name))
  (for _array_element (Variables|Default|GetActiveQuests)
    (Class|QuestAsset|TriggeredInteractionID _array_element InteractionID)
    (if (Variables|/Script/QuestAsset.QuestAsset|GetIsComplete _array_element)
      (Utilities|Array|Add (Variables|Default|GetToBeMoved) _array_element)))
  (CallFunction|UpdateActiveQuests))

(fn AddQuesttoLog
  (params (Quest :type Quest%20Asset%20Object%20Reference) (activateQuest :type Boolean))
  (bind _returnvalue (Class|QuestAsset|CreateInstanceOf Quest self))
  (Development|PrintString (Utilities|String|Append (Utilities|String|ToString(Integer) (Utilities|Array|Length (Class|QuestAsset|GetObjectives Quest))) "vs " (Utilities|String|ToString(Integer) (Utilities|Array|Length (Class|QuestAsset|GetObjectives _returnvalue)))) true true "(R=1.000000,G=0.977579,B=0.000000,A=1.000000)" 5e+01)
  (Utilities|Array|AddUnique (Variables|Default|GetActiveQuests) _returnvalue)
  (if activateQuest
    (Variables|Default|SetPursuedQuest _returnvalue)
    (Default|CallPursuedQuestChanged)))

(fn UpdateActiveQuests
  (Default|UpdateObjectives (Variables|Default|GetObjectivesUI))
  (for _array_element (Variables|Default|GetToBeMoved)
    (Utilities|Array|Add (Variables|Default|GetCompletedQuests) _array_element)
    (Utilities|Array|RemoveItem (Variables|Default|GetActiveQuests) _array_element))
  (Utilities|Array|Clear (Variables|Default|GetToBeMoved))
  ;[1 1 1] Die aktuelle aktive Quest wird nicht mehr verfolgt (abgeschlossen oder aufgegeben)
  (if (not (Utilities|Array|ContainsItem (Variables|Default|GetActiveQuests) (Variables|Default|GetPursuedQuest)))
    (if (> (Utilities|Array|Length (Variables|Default|GetActiveQuests)) 0)
      (Variables|BP_QuestLogComponent_C|SetPursuedQuest self (Utilities|Array|Get(acopy) (Variables|Default|GetActiveQuests)))
      (else
        (Variables|BP_QuestLogComponent_C|SetPursuedQuest self 0)))
    (Default|CallPursuedQuestChanged)))

(fn HasQuest
  (params (QuestID :type Name))
  (bind _outcontains (CallFunction|ContainsQuest QuestID (Variables|Default|GetActiveQuests)))
  (return _outcontains))

(fn HasCompletedQuest
  (params (QuestID :type Name))
  (bind _outcontains (CallFunction|ContainsQuest QuestID (Variables|Default|GetCompletedQuests)))
  (return _outcontains))

(fn ContainsQuest
  (params (QuestID :type Name) (Array :type Array%20of%20Quest%20Asset%20Object%20References))
  (for _array_element Array
    (if (Utilities|Name|Equal(Name) (Variables|/Script/QuestAsset.QuestAsset|GetID _array_element) QuestID)
      (return true)))
  (return false))

(fn IsObjectiveActive
  (params (QuestID :type Name) (ObjectiveID :type Name))
  (for _array_element (Variables|Default|GetActiveQuests)
    (if (Utilities|Name|Equal(Name) (Variables|/Script/QuestAsset.QuestAsset|GetID _array_element) QuestID)
      (bind _returnvalue (Class|QuestAsset|IsObjectiveVisible _array_element ObjectiveID))
      (return _returnvalue)))
  (return false))

(fn IsObjectiveComplete
  (params (QuestID :type Name) (ObjectiveID :type Name))
  (for _array_element (Variables|Default|GetActiveQuests)
    (if (Utilities|Name|Equal(Name) (Variables|/Script/QuestAsset.QuestAsset|GetID _array_element) QuestID)
      (bind _returnvalue (Class|QuestAsset|IsObjectiveComplete _array_element ObjectiveID))
      (return _returnvalue)))
  (return false))