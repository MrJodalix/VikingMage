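; BP_BurningTree_Lightning is a one-shot scripted trigger that stages a lightning strike on a two-part tree.
; When the player overlaps its box, it fires only if their spell inventory contains the Fireball spell.
; It applies fire damage to the lower half, enables physics on the upper half, and plays lightning and hit Niagara effects, thunder and camera shake.
; It then gives the upper half a lifespan and destroys itself.
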(event OnComponentBeginOverlap(BoxTrigger)
  (params (OverlappedComponent :type Primitive%20Component%20Object%20Reference) (OtherActor :type Actor%20Object%20Reference) (OtherComp :type Primitive%20Component%20Object%20Reference) (OtherBodyIndex :type Integer) (bFromSweep :type Boolean) (SweepResult :type Hit%20Result%20Structure%20%28by%20ref%29))
  (bind _asbp_player_character (Utilities|Casting|CastToBP_PlayerCharacter OtherActor))
  (bind _wassuccessful (CallFunction|TriggerLightning _asbp_player_character))
  (if _wassuccessful
    (Actor|SetLifeSpan (Variables|Default|GetUpperHalf) 3e+01)
    (Actor|DestroyActor)))

(event EventBeginPlay)

(event Collision|EventActorBeginOverlap
  (params (OtherActor :type Actor%20Object%20Reference)))

(event EventTick
  (params (DeltaSeconds :type Float%20%28single-precision%29)))

(fn ConstructionScript)

(fn TriggerLightning
  (params (PlayerCharacter :type BP%20Player%20Character%20Object%20Reference))
  (bind _lightning (Variables|Default|GetLightning))
  (bind _returnvalue (Transformation|GetActorLocation _lightning))
  (bind _array_element (Utilities|Array|ForEachLoopwithBreak (Variables|/Game/VikingMageProject/Core/Characters/Player/Spells/BP_SpellComponent.BP_SpellComponent_C|GetSpellInventory (Variables|/Game/VikingMageProject/Core/Characters/Player/BP_PlayerCharacter.BP_PlayerCharacter_C|GetCharacter%20Spells%20%28SpellComponent%29 PlayerCharacter)) :!label _label)
    (:LoopBody
      (bind _output_get (LocalVariables|SetSuccessfulTrigger (== (Utilities|GetClass _array_element) "/Game/VikingMageProject/Core/Characters/Player/Spells/BP_Spell_Fireball.BP_Spell_Fireball_C")))
      (if _output_get
        (goto _label Break)))
    (:Completed
      (if (LocalVariables|GetSuccessfulTrigger)
        (Game|Damage|ApplyDamage (Variables|Default|GetLowerHalf) 5e+01 0 (Variables|Default|GetLightning) "/Game/VikingMageProject/Core/Characters/Player/Spells/BP_FireDamage.BP_FireDamage_C")
        (Physics|SetSimulatePhysics (Actor|GetComponentbyClass (Variables|Default|GetUpperHalf) "/Script/Engine.StaticMeshComponent") true)
        (Components|Activation|SetActive (Variables|/Script/Niagara.NiagaraActor|GetNiagaraComponent _lightning) true false)
        (Audio|PlaySoundatLocation "/Game/UltraDynamicSky/Sound/Close_Thunder/CloseThunder_2.CloseThunder_2" _returnvalue "0, 0, 0" 1.0 1.0 0.0 0 0 0)
        (Camera|PlayWorldCameraShake "/Game/VikingMageProject/Cinematics/BP_LightningShake.BP_LightningShake_C" _returnvalue 0.0 1e+03 0.0)
        (Components|Activation|SetActive (Variables|/Script/Niagara.NiagaraActor|GetNiagaraComponent (Variables|Default|GetHitParticles)) true false)
        (return (LocalVariables|GetSuccessfulTrigger))
        (else
          (return (LocalVariables|GetSuccessfulTrigger)))))))