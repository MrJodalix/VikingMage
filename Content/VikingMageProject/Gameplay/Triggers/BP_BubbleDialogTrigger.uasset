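; Trigger actor that plays a dialogue as speech bubbles over characters when the player overlaps it, ignoring retriggers while one is active.
; It starts the dialogue with default participants and passes each node to the active speaker's SaySomeDialog.
; ForwardDialog always picks the first option, ending early if the next speaker cannot bubble-talk.
; Ending unbinds the bubble's finished-talking events and optionally destroys the trigger if the dialogue completed.
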(event Custom|ForwardDialog
  (bind _activecontext (Variables|Default|GetActiveContext))
  (bind _activecontext_2 (Variables|Default|GetActiveContext)
    (:then
      (bind _returnvalue (Class|DlgContext|ChooseOption _activecontext_2))
      (if _returnvalue
        ;[1 1 1] Dialog is still active, let next person talk
        (bind _asbp_character_custom (Utilities|Casting|CastToBP_CharacterCustom (Class|DlgContext|GetActiveNodeParticipant _activecontext)))
        (if (Default|CanBubbleTalk _asbp_character_custom)
          (Default|SaySomeDialog _asbp_character_custom (Class|DlgContext|GetMutableActiveNode _activecontext) self)
          (else
            (CallFunction|EndSpeechBubbleDialog false)))
        (else
          (CallFunction|EndSpeechBubbleDialog true))))
    (:else)))

(event EventBeginPlay)

(event Collision|EventActorBeginOverlap
  (params (OtherActor :type Actor%20Object%20Reference))
  (bind _dialogue (Variables|Default|GetDialogue))
  (if (not (Utilities|IsValid (Variables|Default|GetActiveContext))) ; Do not retrigger
    (Utilities|IsValid _dialogue
      (:Is%20Valid
        (Utilities|Casting|CastToBP_PlayerCharacter OtherActor)
        (bind _returnvalue (Class|DlgManager|StartDialoguewithDefaultParticipants _dialogue))
        (Utilities|IsValid _returnvalue
          (:Is%20Valid
            (bind _output_get (Variables|Default|SetActiveContext _returnvalue))
            (bind _asbp_character_custom (Utilities|Casting|CastToBP_CharacterCustom (Class|DlgContext|GetActiveNodeParticipant _output_get))
              (:then
                (Default|SaySomeDialog _asbp_character_custom (Class|DlgContext|GetMutableActiveNode _output_get) self))
              (:CastFailed
                (Development|PrintString "Invalid Participant"))))
          (:Is%20Not%20Valid
            (Development|PrintString "Dialogue could not be started"))))
      (:Is%20Not%20Valid
        (Development|PrintString "WARNING: No Dialog to start" true true "(R=1.000000,G=0.007958,B=0.000000,A=1.000000)")))))

(fn ConstructionScript)

(fn EndSpeechBubbleDialog
  (params (HasEnded :type Boolean))
  (bind _activecontext (Variables|Default|GetActiveContext)
    (:then
      (EventDispatchers|UnbindallEventsfromFinishedTalking (Variables|/Game/VikingMageProject/Core/Characters/BP_CharacterCustom.BP_CharacterCustom_C|GetBP_SpeechBubbleComponent (.AsBP%20Character%20Custom (Utilities|Casting|CastToBP_CharacterCustom (Class|DlgContext|GetActiveNodeParticipant _activecontext)))))
      (Variables|Default|SetActiveContext 0)
      (if (and (Variables|Default|GetDisappearOnFinished) HasEnded)
        (Actor|DestroyActor)))
    (:else)))